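; Puzzle actor that plays the entrance cinematic when triggered through SwitchInteraction, then opens the boss portal.
; The trigger creates a level sequence player, waits briefly, plays it, broadcasts OnOpenPortalSequence, flags the player as in-sequence and hides the linked switches.
; When the sequence finishes, it spawns BP_BossPortal at its own transform and reverses those states.
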(event Custom|Event%20EntranceSequence%20End
  (Game|SpawnActorfromClass "/Game/Interaction_Objects/BP_BossPortal.BP_BossPortal_C" (Transformation|GetActorTransform) "AlwaysSpawn" "MultiplyWithRoot" 0 0)
  (EventDispatchers|UnbindEventfromOnFinished (stale EventSwitchInteraction _returnvalue) (delegate Custom|Event%20EntranceSequence%20End))
  (Default|CallOnOpenPortalSequence false)
  (Default|PlayerinSequence (Variables|Default|GetBP_Player) false)
  (for _array_element (Variables|Default|GetBP_Switches)
    (Rendering|SetActorHiddenInGame _array_element false)))

(event EventBeginPlay
  (|CallParentFunction)
  (bind _asbp_third_person_character (Utilities|Casting|CastToBP_ThirdPersonCharacter (Game|GetPlayerCharacter 0)))
  (Variables|Default|SetBP_Player _asbp_third_person_character))

(event EventSwitchInteraction
  (bind _returnvalue (Sequencer|Player|CreateLevelSequencePlayer (Variables|Default|GetEntranceSequence)))
  (EventDispatchers|BindEventtoOnFinished _returnvalue (delegate Custom|Event%20EntranceSequence%20End))
  (Utilities|FlowControl|Delay 2.0)
  (Sequencer|Player|Play _returnvalue :!class /Script/MovieScene.MovieSceneSequencePlayer)
  (Default|CallOnOpenPortalSequence true)
  (Default|PlayerinSequence (Variables|Default|GetBP_Player) true)
  (for _array_element (Variables|Default|GetBP_Switches)
    (Rendering|SetActorHiddenInGame _array_element true)))

(fn ConstructionScript
  (|CallParentFunction))