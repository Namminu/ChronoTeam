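; BP_FirePuzzle is a puzzle object that catches fire when an actor tagged FIRE overlaps its Box.
; Igniting sets IsFire, shows the fire particle effect, adds the FIRE tag to itself so it can light others, and calls Operation, which is defined outside this file.
; BeginPlay hides the point light, sets IsPlural, syncs the fire state and calls Operation if it starts lit.
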(event OnComponentBeginOverlap(Box)
  (params (OverlappedComponent :type Primitive%20Component%20Object%20Reference) (OtherActor :type Actor%20Object%20Reference) (OtherComp :type Primitive%20Component%20Object%20Reference) (OtherBodyIndex :type Integer) (bFromSweep :type Boolean) (SweepResult :type Hit%20Result%20Structure%20%28by%20ref%29))
  (if (and (Actor|ActorHasTag OtherActor "FIRE") (not (Variables|Default|GetIsFire)))
    (Variables|Default|SetIsFire true)
    (CallFunction|IsFireAttach)
    (CallFunction|Operation)))

(event EventBeginPlay
  (Development|SetHiddeninGame (Variables|Default|GetPointLight) true false)
  (CallFunction|IsFireAttach)
  (Variables|Default|SetIsPlural true)
  (if (Variables|Default|GetIsFire)
    (CallFunction|Operation)))

(fn ConstructionScript)

(fn IsFireAttach
  (if (Variables|Default|GetIsFire)
    (Development|SetHiddeninGame (Variables|Default|GetPS_FX_fire_dungeon_01) false false)
    (Utilities|Array|Add (Variables|Default|GetTags) "FIRE")
    (else
      (Development|SetHiddeninGame (Variables|Default|GetPS_FX_fire_dungeon_01) true false))))