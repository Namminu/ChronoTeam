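; Switch-driven puzzle pillar that adds a glow response to the switch behavior inherited from its parent Blueprint.
; BeginPlay creates a dynamic material on element 1 of the wall mesh.
; SwitchInteraction plays one timeline forward to raise the glow intensity, while SwitchInteractionEnd plays a second in reverse to dim it.
; Both events start their timeline, then call the parent implementation.
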(event EventBeginPlay
  (bind _mod_wall_01_m_straight_large_half_r (Variables|Default|GetMOD_Wall_01_M_straight_large_half_R))
  (bind _returnvalue (Rendering|Material|CreateDynamicMaterialInstance _mod_wall_01_m_straight_large_half_r 1 (Rendering|Material|GetMaterial _mod_wall_01_m_straight_large_half_r 1) "None" :!class /Script/Engine.PrimitiveComponent))
  (Variables|Default|SetGlow%20MT _returnvalue))

(event EventSwitchInteraction
  (Utilities|FlowControl|Sequence
    (:then_0
      (bind _새_트랙_0 (Timeline|타임라인_0 PlayFromStart)
        (:Update
          (Rendering|Material|SetScalarParameterValue (Variables|Default|GetGlow%20MT) "Glow Instense" (Math|Float|Lerp 1.0 2e+01 _새_트랙_0) :!class /Script/Engine.MaterialInstanceDynamic))))
    (:then_1
      (|CallParentFunction))))

(event EventSwitchInteractionEnd
  (Utilities|FlowControl|Sequence
    (:then_0
      (bind _새_트랙_0 (Timeline|타임라인_1 ReverseFromEnd)
        (:Update
          (Rendering|Material|SetScalarParameterValue (Variables|Default|GetGlow%20MT) "Glow Instense" (Math|Float|Lerp 1.0 2e+01 _새_트랙_0) :!class /Script/Engine.MaterialInstanceDynamic))))
    (:then_1
      (|CallParentFunction))))

(fn ConstructionScript)