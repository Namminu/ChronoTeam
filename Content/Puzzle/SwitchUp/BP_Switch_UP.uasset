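; Puzzle switch Blueprint that slides its UPSwitch component from a start marker to an end marker when operated, then resets after a delay.
; Operation raises the glow on a dynamic material and plays a timeline that lerps the position.
; When the forward move finishes, a SwitchTime timer calls NoOperation, which dims the glow, calls the parent and reverses the timeline.
; The IsOperation flag stops the return move from restarting the timer.
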(event EventBeginPlay
  (bind _upswitch (Variables|Default|GetUPSwitch))
  (|CallParentFunction)
  (Transformation|SetWorldLocation (Variables|Default|GetUPSwitch) (Transformation|GetWorldLocation (Variables|Default|GetSwitchStart)) false false)
  (bind _returnvalue (Rendering|Material|CreateDynamicMaterialInstance _upswitch 0 (Rendering|Material|GetMaterial _upswitch 0) "None" :!class /Script/Engine.PrimitiveComponent))
  (Variables|Default|SetGLowMT _returnvalue))

(event EventOperation
  (Variables|Default|SetIsOperation true)
  (Rendering|Material|SetScalarParameterValue (Variables|Default|GetGLowMT) "Glow Instense" 2e+01 :!class /Script/Engine.MaterialInstanceDynamic)
  (bind _새_트랙_0 (Timeline|타임라인 PlayFromStart)
    (:Update
      (Transformation|SetWorldLocation (Variables|Default|GetUPSwitch) (Math|Vector|Lerp(Vector) (Transformation|GetWorldLocation (Variables|Default|GetSwitchStart)) (Transformation|GetWorldLocation (Variables|Default|GetSwitchEnd)) _새_트랙_0) false false))
    (:Finished
      (if (Variables|Default|GetIsOperation)
        (Utilities|Time|SetTimerbyFunctionName 0 "NoOperation" (Variables|Default|GetSwitchTime))))))

(event EventNoOperation
  (Variables|Default|SetIsOperation false)
  (Rendering|Material|SetScalarParameterValue (Variables|Default|GetGLowMT) "Glow Instense" 1.0 :!class /Script/Engine.MaterialInstanceDynamic)
  (|CallParentFunction)
  (bind _새_트랙_0 (Timeline|타임라인 ReverseFromEnd)
    (:Update
      (Transformation|SetWorldLocation (Variables|Default|GetUPSwitch) (Math|Vector|Lerp(Vector) (Transformation|GetWorldLocation (Variables|Default|GetSwitchStart)) (Transformation|GetWorldLocation (Variables|Default|GetSwitchEnd)) _새_트랙_0) false false))
    (:Finished
      (if (Variables|Default|GetIsOperation)
        (Utilities|Time|SetTimerbyFunctionName 0 "NoOperation" (Variables|Default|GetSwitchTime))))))

(fn ConstructionScript)