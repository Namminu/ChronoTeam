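; BP_DissolveFootBoard is a switch-driven puzzle footboard that becomes collidable or non-collidable through a dissolve effect.
; The construction script creates a dynamic material instance, and BeginPlay applies the initial dissolve value with collision disabled.
; Switch interaction start and end play one timeline forward or in reverse to animate the Dissolve parameter.
; Each event stores a target collision type, which is applied only when the timeline finishes.
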(event EventBeginPlay
  (|CallParentFunction)
  (Rendering|Material|SetScalarParameterValue (Variables|Default|GetMaterialParameter) "Dissolve" (Variables|Default|GetDissolveValue) :!class /Script/Engine.MaterialInstanceDynamic)
  (Collision|SetCollisionEnabled (Variables|Default|GetStaticMesh) "NoCollision"))

(event EventSwitchInteraction
  (Variables|Default|SetNew%20Type "QueryAndPhysics")
  (bind _새_트랙_0 (Timeline|타임라인_0 PlayFromStart)
    (:Update
      (Rendering|Material|SetScalarParameterValue (Variables|Default|GetMaterialParameter) "Dissolve" (Math|Float|Lerp 0.0 1.0 _새_트랙_0) :!class /Script/Engine.MaterialInstanceDynamic))
    (:Finished
      (Collision|SetCollisionEnabled (Variables|Default|GetStaticMesh) (Variables|Default|GetNew%20Type)))))

(event EventSwitchInteractionEnd
  (Variables|Default|SetNew%20Type "NoCollision")
  (bind _새_트랙_0 (Timeline|타임라인_0 ReverseFromEnd)
    (:Update
      (Rendering|Material|SetScalarParameterValue (Variables|Default|GetMaterialParameter) "Dissolve" (Math|Float|Lerp 0.0 1.0 _새_트랙_0) :!class /Script/Engine.MaterialInstanceDynamic))
    (:Finished
      (Collision|SetCollisionEnabled (Variables|Default|GetStaticMesh) (Variables|Default|GetNew%20Type)))))

(fn ConstructionScript
  (bind _returnvalue (Rendering|Material|CreateDynamicMaterialInstance (Variables|Default|GetStaticMesh) 0 0 "None" :!class /Script/Engine.PrimitiveComponent))
  (bind _output_get (Variables|Default|SetMaterialParameter _returnvalue))
  (Rendering|Material|SetScalarParameterValue _output_get "Dissolve" 0.98 :!class /Script/Engine.MaterialInstanceDynamic))