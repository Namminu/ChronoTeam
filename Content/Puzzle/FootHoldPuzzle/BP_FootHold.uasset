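; Foothold switch for a puzzle that the player activates by stepping on its box, signalling the switch and raising the material's Glow.
; Leaving the box starts a timed fade that calls NoOperation when it finishes, with the second timeline seeked to 100 minus SwitchTime for an adjustable duration.
; Once MultipleGimicSuccess is set, overlaps are ignored and Operation stops the fade and replays the glow.
; The construction script creates the colored dynamic material and sets IsPlural.
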(event OnComponentBeginOverlap(Box)
  (params (OverlappedComponent :type Primitive%20Component%20Object%20Reference) (OtherActor :type Actor%20Object%20Reference) (OtherComp :type Primitive%20Component%20Object%20Reference) (OtherBodyIndex :type Integer) (bFromSweep :type Boolean) (SweepResult :type Hit%20Result%20Structure%20%28by%20ref%29))
  (if (== OtherActor (Game|GetPlayerCharacter 0))
    (if (not (Variables|Default|GetMultipleGimicSuccess))
      (Variables|Default|SetIsOperation true)
      (if (not (Variables|Default|GetIsGimic))
        (bind _output_get (Variables|Default|SetIsGimic true))
        (Default|CallBeginSwitch _output_get)
        (bind _새_트랙_0 (Timeline|타임라인 PlayFromStart)
          (:Update
            (Rendering|Material|SetScalarParameterValue (Variables|Default|GetMeshInstance) "Glow" (Math|Float|Lerp 1.0 (Variables|Default|GetGlow) _새_트랙_0) :!class /Script/Engine.MaterialInstanceDynamic)))
        (else
          (Timeline|타임라인 PlayFromStart))))))

(event OnComponentEndOverlap(Box)
  (params (OverlappedComponent :type Primitive%20Component%20Object%20Reference) (OtherActor :type Actor%20Object%20Reference) (OtherComp :type Primitive%20Component%20Object%20Reference) (OtherBodyIndex :type Integer))
  (if (not (Variables|Default|GetMultipleGimicSuccess))
    (CallFunction|Operation)
    (Actor|Tick|SetActorTickEnabled true)))

(event EventBeginPlay)

(event Collision|EventActorBeginOverlap
  (params (OtherActor :type Actor%20Object%20Reference))
  (|CallParentFunction OtherActor) ; 지금 이 노드는 비활성 상태입니다. \n핀을 끌어서 다른 노드를 연결하면 활성화됩니다.
)

(event EventTick
  (params (DeltaSeconds :type Float%20%28single-precision%29))
  (|CallParentFunction DeltaSeconds) ; 지금 이 노드는 비활성 상태입니다. \n핀을 끌어서 다른 노드를 연결하면 활성화됩니다.
)

(event EventOperation
  (if (not (Variables|Default|GetMultipleGimicSuccess))
    (Utilities|FlowControl|Sequence
      (:then_0
        (bind _새_트랙_0 (Timeline|타임라인_0 SetNewTime)
          (:Update
            (Rendering|Material|SetScalarParameterValue (Variables|Default|GetMeshInstance) "Glow" (Math|Float|Lerp (Variables|Default|GetGlow) 1.0 (/ (- _새_트랙_0 (- 1e+02 (Variables|Default|GetSwitchTime))) (Variables|Default|GetSwitchTime))) :!class /Script/Engine.MaterialInstanceDynamic))
          (:Finished
            (if (not (Variables|Default|GetMultipleGimicSuccess))
              (CallFunction|NoOperation)))))
      (:then_1
        (Timeline|타임라인_0 Play)))
    (else
      (Variables|Default|SetIsOperation false)
      (Utilities|FlowControl|Sequence
        (:then_0
          (Timeline|타임라인_0 Stop))
        (:then_1
          (bind _새_트랙_0_2 (Timeline|타임라인 PlayFromStart)
            (:Update
              (Rendering|Material|SetScalarParameterValue (Variables|Default|GetMeshInstance) "Glow" (Math|Float|Lerp 1.0 (Variables|Default|GetGlow) _새_트랙_0_2) :!class /Script/Engine.MaterialInstanceDynamic))))))))

(fn ConstructionScript
  (|CallParentFunction)
  (bind _returnvalue (Rendering|Material|CreateDynamicMaterialInstance (Variables|Default|GetStaticMesh) 0 0 "None" :!class /Script/Engine.PrimitiveComponent))
  (bind _output_get (Variables|Default|SetMeshInstance _returnvalue))
  (Rendering|Material|SetVectorParameterValue _output_get "BaseColor" (Variables|Default|GetValueColor) :!class /Script/Engine.MaterialInstanceDynamic)
  (Variables|Default|SetIsPlural true))