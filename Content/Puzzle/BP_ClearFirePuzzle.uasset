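; Puzzle actor for a clear-fire puzzle that shows or hides a dungeon fire effect and its point light.
; The FIreOnOff event takes a boolean and toggles hidden-in-game on the particle and light components.
; BeginPlay calls it with false, so the fire starts unlit.
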(event Custom|FIreOnOff
  (params (NewParam :type Boolean))
  (if NewParam
    (Development|SetHiddeninGame (Variables|Default|GetPS_FX_fire_dungeon_01) false false)
    (Development|SetHiddeninGame (Variables|Default|GetPointLight) false false)
    (else
      (Development|SetHiddeninGame (Variables|Default|GetPS_FX_fire_dungeon_01) true false)
      (Development|SetHiddeninGame (Variables|Default|GetPointLight) true false))))

(event EventBeginPlay
  (CallFunction|FIreonOff false))

(event Collision|EventActorBeginOverlap
  (params (OtherActor :type Actor%20Object%20Reference)))

(event EventTick
  (params (DeltaSeconds :type Float%20%28single-precision%29)))

(fn ConstructionScript)