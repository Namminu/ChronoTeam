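; BP_Puzzle_DistanceDoor is a puzzle door whose position follows the player's distance from a Center component.
; BeginPlay caches the player as BP_ThirdPersonCharacter.
; Each Tick, while that distance is between the minimum and maximum, the door mesh lerps from DoorEnd (near) to DoorStart (far).
; The door holds its last position outside that band or while the character's E skill is active.
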(event EventBeginPlay
  (bind _asbp_third_person_character (Utilities|Casting|CastToBP_ThirdPersonCharacter (Game|GetPlayerCharacter 0)))
  (Variables|Default|SetAs%20BP%20Third%20Person%20Character _asbp_third_person_character))

(event Collision|EventActorBeginOverlap
  (params (OtherActor :type Actor%20Object%20Reference)))

(event EventTick
  (params (DeltaSeconds :type Float%20%28single-precision%29))
  (bind _returnvalue (Game|GetPlayerCharacter 0))
  (bind _center (Variables|Default|GetCenter))
  (bind _minimumdistance (Variables|Default|GetMinimumDistance))
  (bind _returnvalue_2 (Transformation|GetActorLocation _returnvalue))
  (bind _returnvalue_3 (Transformation|GetWorldLocation _center))
  (bind _returnvalue_4 (Math|Vector|Distance(Vector) _returnvalue_3 _returnvalue_2))
  (Variables|Default|GetAs%20BP%20Third%20Person%20Character
    (:then
      (if (Math|Boolean|ANDBoolean (> _returnvalue_4 (Variables|Default|GetMinimumDistance)) (< _returnvalue_4 (Variables|Default|GetMaximumDistance)) (not (Variables|/Script/TeamChrono.TeamChronoCharacter|GetIsESkillDoing (Variables|Default|GetAs%20BP%20Third%20Person%20Character))))
        (Transformation|SetWorldLocation (Variables|Default|GetMOD_Gateway_Door_01_med_01_door) (Math|Vector|Lerp(Vector) (Transformation|GetWorldLocation (Variables|Default|GetDoor_End)) (Transformation|GetWorldLocation (Variables|Default|GetDoor_Start)) (/ (- _returnvalue_4 _minimumdistance) (- (Variables|Default|GetMaximumDistance) _minimumdistance))) false false)))
    (:else)))

(fn ConstructionScript)