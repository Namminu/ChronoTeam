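; BP_Switch_UP is a timed puzzle switch that extends a parent switch Blueprint and moves its UPSwitch component when operated.
; Operation plays a timeline that lerps UPSwitch from the SwitchStart location to SwitchEnd.
; When the timeline finishes while still operating, a timer calls NoOperation after SwitchTime.
; NoOperation clears the operating flag, calls the parent logic and reverses the timeline to return the switch.
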(event EventBeginPlay
  (|CallParentFunction)
  (Transformation|SetWorldLocation (Variables|Default|GetUPSwitch) (Transformation|GetWorldLocation (Variables|Default|GetSwitchStart)) false false))

(event EventOperation
  (Variables|Default|SetIsOperation true)
  (bind _새_트랙_0 (Timeline|타임라인 PlayFromStart)
    (:Update
      (Transformation|SetWorldLocation (Variables|Default|GetUPSwitch) (Math|Vector|Lerp(Vector) (Transformation|GetWorldLocation (Variables|Default|GetSwitchStart)) (Transformation|GetWorldLocation (Variables|Default|GetSwitchEnd)) _새_트랙_0) false false))
    (:Finished
      (if (Variables|Default|GetIsOperation)
        (Utilities|Time|SetTimerbyFunctionName 0 "NoOperation" (Variables|Default|GetSwitchTime))))))

(event EventNoOperation
  (Variables|Default|SetIsOperation false)
  (|CallParentFunction)
  (bind _새_트랙_0 (Timeline|타임라인 ReverseFromEnd)
    (:Update
      (Transformation|SetWorldLocation (Variables|Default|GetUPSwitch) (Math|Vector|Lerp(Vector) (Transformation|GetWorldLocation (Variables|Default|GetSwitchStart)) (Transformation|GetWorldLocation (Variables|Default|GetSwitchEnd)) _새_트랙_0) false false))
    (:Finished
      (if (Variables|Default|GetIsOperation)
        (Utilities|Time|SetTimerbyFunctionName 0 "NoOperation" (Variables|Default|GetSwitchTime))))))

(fn ConstructionScript)