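; A fire pillar hazard that sweeps its flame back and forth and damages the player inside it.
; Two timelines endlessly alternate FireObject between Start and End rotations with brief pauses, playing only their last TurnTime seconds to make sweep duration configurable.
; Capsule overlap starts and clears a looping timer that applies damage to the player character.
; The construction script offsets End by RotationArea and scales particles and capsule by FireLength.
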(event OnComponentBeginOverlap(Capsule)
  (params (OverlappedComponent :type Primitive%20Component%20Object%20Reference) (OtherActor :type Actor%20Object%20Reference) (OtherComp :type Primitive%20Component%20Object%20Reference) (OtherBodyIndex :type Integer) (bFromSweep :type Boolean) (SweepResult :type Hit%20Result%20Structure%20%28by%20ref%29))
  (if (== OtherActor (Variables|Default|GetBP%20Player))
    (bind _returnvalue (Utilities|Time|SetTimerbyEvent (delegate Custom|TakeDamage) 0.2 true))
    (Variables|Default|SetNewVar _returnvalue)))

(event OnComponentEndOverlap(Capsule)
  (params (OverlappedComponent :type Primitive%20Component%20Object%20Reference) (OtherActor :type Actor%20Object%20Reference) (OtherComp :type Primitive%20Component%20Object%20Reference) (OtherBodyIndex :type Integer))
  (if (== OtherActor (Variables|Default|GetBP%20Player))
    (Utilities|Time|ClearandInvalidateTimerbyHandle (Variables|Default|GetNewVar))))

(event Custom|TakeDamage
  (Game|Damage|ApplyDamage (Variables|Default|GetBP%20Player) 1.0 0 0))

(event EventBeginPlay
  (bind _asbp_third_person_character (Utilities|Casting|CastToBP_ThirdPersonCharacter (Game|GetPlayerCharacter 0)))
  (Variables|Default|SetBP%20Player _asbp_third_person_character)
  (Utilities|FlowControl|Sequence :!label _label
    (:then_0
      (bind _새_트랙_0 (Timeline|타임라인 SetNewTime)
        (:Update
          (Transformation|SetWorldRotation (Variables|Default|GetFire_Object) (Math|Rotator|Lerp(Rotator) (Transformation|GetWorldRotation (Variables|Default|GetStart)) (Transformation|GetWorldRotation (Variables|Default|GetEnd)) (/ (- _새_트랙_0 (- 1e+02 (Variables|Default|GetTurnTime))) (Variables|Default|GetTurnTime))) false false))
        (:Finished
          (Utilities|FlowControl|Delay 0.3)
          (Utilities|FlowControl|Sequence
            (:then_0
              (bind _새_트랙_0_2 (Timeline|타임라인_0 SetNewTime)
                (:Update
                  (Transformation|SetWorldRotation (Variables|Default|GetFire_Object) (Math|Rotator|Lerp(Rotator) (Transformation|GetWorldRotation (Variables|Default|GetEnd)) (Transformation|GetWorldRotation (Variables|Default|GetStart)) (/ (- _새_트랙_0_2 (- 1e+02 (Variables|Default|GetTurnTime))) (Variables|Default|GetTurnTime))) false false))
                (:Finished
                  (Utilities|FlowControl|Delay 0.3)
                  (goto _label))))
            (:then_1
              (Timeline|타임라인_0 Play))))))
    (:then_1
      (Timeline|타임라인 Play))))

(fn ConstructionScript
  (Transformation|AddWorldRotation (Variables|Default|GetEnd) (Math|Rotator|MakeRotator 0.0 0.0 (Variables|Default|GetRotationArea)) false false)
  (Transformation|SetWorldScale3D (Variables|Default|GetParticleSystem) (Math|Vector|MakeVector (Variables|Default|GetFireLength) 1.0 1.0))
  (Transformation|SetWorldScale3D (Variables|Default|GetCapsule) (Math|Vector|MakeVector 1.0 1.0 (Variables|Default|GetFireLength))))