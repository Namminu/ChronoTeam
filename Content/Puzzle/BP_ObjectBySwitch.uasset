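; Puzzle object that moves a mesh between Start and End transforms in response to switch interaction.
; In plural mode it binds to its switches and counts active ones, lighting one BPClearFire per count as progress indicators.
; When all switches are active, it flags and operates each one, then plays a timeline lerping location and rotation.
; SwitchInteractionEnd reverses that timeline.
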(event Custom|SwitchInteractionEnd
  (bind _새_트랙_0 (Timeline|타임라인 ReverseFromEnd)
    (:Update
      (Transformation|SetWorldLocationAndRotation (Variables|Default|GetMove_StaticMesh) (Math|Vector|Lerp(Vector) (Transformation|GetWorldLocation (Variables|Default|GetStart)) (Transformation|GetWorldLocation (Variables|Default|GetEnd)) _새_트랙_0) (Math|Rotator|Lerp(Rotator) (Transformation|GetWorldRotation (Variables|Default|GetStart)) (Transformation|GetWorldRotation (Variables|Default|GetEnd)) _새_트랙_0) false false))))

(event Custom|SwitchInteraction
  (bind _새_트랙_0 (Timeline|타임라인 PlayFromStart)
    (:Update
      (Transformation|SetWorldLocationAndRotation (Variables|Default|GetMove_StaticMesh) (Math|Vector|Lerp(Vector) (Transformation|GetWorldLocation (Variables|Default|GetStart)) (Transformation|GetWorldLocation (Variables|Default|GetEnd)) _새_트랙_0) (Math|Rotator|Lerp(Rotator) (Transformation|GetWorldRotation (Variables|Default|GetStart)) (Transformation|GetWorldRotation (Variables|Default|GetEnd)) _새_트랙_0) false false))))

(event Custom|IsBeginSwitch
  (params (IsGimic :type Boolean))
  (if IsGimic
    (Math|Integer|IncrementInt (Variables|Default|GetSwitchOperationNum)
      (:%20%20
        _))
    (else
      (Math|Integer|DecrementInt (Variables|Default|GetSwitchOperationNum)
        (:%20%20
          _))))
  (CallFunction|IsGimicSuccess)
  (for (_array_element _array_index) (Variables|Default|GetBP_ClearFire)
    (Default|FIreonOff _array_element (> (Variables|Default|GetSwitchOperationNum) _array_index))))

(event EventBeginPlay
  (Transformation|SetWorldLocation (Variables|Default|GetMove_StaticMesh) (Transformation|GetWorldLocation (Variables|Default|GetStart)) false false)
  (if (Variables|Default|GetIsPlural)
    (Variables|Default|SetSwitchOperationNum 0)
    (for _array_element (Variables|Default|GetBP_Switches)
      (EventDispatchers|BindEventtoBeginSwitch _array_element (delegate Custom|IsBeginSwitch)))))

(fn ConstructionScript)

(fn IsGimicSuccess
  (if (== (Utilities|Array|Length (Variables|Default|GetBP_Switches)) (Variables|Default|GetSwitchOperationNum))
    (for _array_element (Variables|Default|GetBP_Switches)
      (Variables|/Game/Puzzle/BP_BaseSwitch.BP_BaseSwitch_C|SetMultipleGimicSuccess _array_element true)
      (Default|Operation _array_element))
    (CallFunction|SwitchInteraction)))