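; BP_Switch_Down is a puzzle switch that moves between Start and End points and glows brighter while operated, extending a parent's Operation and NoOperation events.
; Operation disables the Box collision, raises glow on a dynamic material and plays a timeline that lerps the switch to End.
; If IsOperation is set when the timeline finishes, a timer calls NoOperation after SwitchTime to restore collision, dim the glow and reverse the movement.
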(event EventBeginPlay
  (bind _downswitch (Variables|Default|GetDownSwitch))
  (|CallParentFunction)
  (Transformation|SetWorldLocation (Variables|Default|GetDownSwitch) (Transformation|GetWorldLocation (Variables|Default|GetStart)) false false)
  (bind _returnvalue (Rendering|Material|CreateDynamicMaterialInstance _downswitch 0 (Rendering|Material|GetMaterial _downswitch 0) "None" :!class /Script/Engine.PrimitiveComponent))
  (Variables|Default|SetGlow%20MT _returnvalue))

(event EventOperation
  (|CallParentFunction)
  (Collision|SetCollisionEnabled (Variables|Default|GetBox) "NoCollision")
  (Utilities|Time|ClearandInvalidateTimerbyHandle (Variables|Default|GetNoOperation%20Timer))
  (Rendering|Material|SetScalarParameterValue (Variables|Default|GetGlow%20MT) "Glow Instense" 2e+01 :!class /Script/Engine.MaterialInstanceDynamic)
  (bind _새_트랙_0 (Timeline|타임라인 PlayFromStart)
    (:Update
      (Transformation|SetWorldLocation (Variables|Default|GetDownSwitch) (Math|Vector|Lerp(Vector) (Transformation|GetWorldLocation (Variables|Default|GetStart)) (Transformation|GetWorldLocation (Variables|Default|GetEnd)) _새_트랙_0) false false))
    (:Finished
      (if (Variables|Default|GetIsOperation)
        (bind _returnvalue (Utilities|Time|SetTimerbyFunctionName 0 "NoOperation" (Variables|Default|GetSwitchTime)))
        (Variables|Default|SetNoOperation%20Timer _returnvalue)))))

(event EventNoOperation
  (|CallParentFunction)
  (Collision|SetCollisionEnabled (Variables|Default|GetBox) "QueryOnly")
  (Variables|Default|SetIsOperation false)
  (Rendering|Material|SetScalarParameterValue (Variables|Default|GetGlow%20MT) "Glow Instense" 1.0 :!class /Script/Engine.MaterialInstanceDynamic)
  (bind _새_트랙_0 (Timeline|타임라인 ReverseFromEnd)
    (:Update
      (Transformation|SetWorldLocation (Variables|Default|GetDownSwitch) (Math|Vector|Lerp(Vector) (Transformation|GetWorldLocation (Variables|Default|GetStart)) (Transformation|GetWorldLocation (Variables|Default|GetEnd)) _새_트랙_0) false false))
    (:Finished
      (if (Variables|Default|GetIsOperation)
        (bind _returnvalue (Utilities|Time|SetTimerbyFunctionName 0 "NoOperation" (Variables|Default|GetSwitchTime)))
        (Variables|Default|SetNoOperation%20Timer _returnvalue)))))

(fn ConstructionScript)

(fn GetIsOperation
  (return (Variables|Default|GetIsOperation)))