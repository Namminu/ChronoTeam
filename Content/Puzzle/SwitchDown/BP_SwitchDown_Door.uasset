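; BP_SwitchDown_Door is a puzzle door Blueprint that responds to switch interaction, requiring one or several switches.
; When IsPlural is false, SwitchInteraction runs the parent's behavior directly.
; Otherwise it counts switches in BPSwitches with IsGimic set and proceeds only when all are set.
; It then flags each switch with MultipleGimicSuccess, calls its Operation, and runs the parent interaction once per switch inside that loop.
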(event EventBeginPlay)

(event Collision|EventActorBeginOverlap
  (params (OtherActor :type Actor%20Object%20Reference)))

(event EventTick
  (params (DeltaSeconds :type Float%20%28single-precision%29)))

(event EventSwitchInteraction
  (if (not (Variables|Default|GetIsPlural))
    (|CallParentFunction)
    (else
      (Variables|Default|SetSwitchOperationNum 0)
      (for _array_element (Variables|Default|GetBP_Switches)
        (if (Variables|/Game/Puzzle/SwitchDown/BP_Switch_Down.BP_Switch_Down_C|GetIsGimic _array_element)
          (Math|Integer|IncrementInt (Variables|Default|GetSwitchOperationNum))))
      (if (== (Utilities|Array|Length (Variables|Default|GetBP_Switches)) (Variables|Default|GetSwitchOperationNum))
        (for _array_element_2 (Variables|Default|GetBP_Switches)
          (Variables|/Game/Puzzle/SwitchDown/BP_Switch_Down.BP_Switch_Down_C|SetMultipleGimicSuccess _array_element_2 true)
          (Default|Operation _array_element_2)
          (|CallParentFunction))))))

(fn ConstructionScript
  (|CallParentFunction))