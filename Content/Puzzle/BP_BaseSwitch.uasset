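; Base puzzle switch that triggers when damaged and drives a list of linked objects.
; A hit latches the switch, calls SwitchInteraction on each object and broadcasts BeginSwitch unless the multi-switch gimmick has succeeded.
; NoOperation re-arms it, either ending the linked interactions or, in plural mode, broadcasting an off state.
; While enabled, Tick copies changes in the switch's CustomTimeDilation to the linked objects.
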(event Custom|OnTakeAnyDamage_이벤트
  (params (DamagedActor :type Actor%20Object%20Reference) (Damage :type Float%20%28single-precision%29) (DamageType :type Damage%20Type%20Object%20Reference) (InstigatedBy :type Controller%20Object%20Reference) (DamageCauser :type Actor%20Object%20Reference))
  (if (not (Variables|Default|GetHiting))
    (Variables|Default|SetHiting true)
    (CallFunction|Operation)
    (CallFunction|HitFunction)
    (Actor|Tick|SetActorTickEnabled true)))

(event Custom|Operation
  (if (and (Variables|Default|GetIsPlural) (not (Variables|Default|GetMultipleGimicSuccess)))
    (Variables|Default|SetIsOperation true)
    (else
      (Variables|Default|SetIsOperation false)
      (CallFunction|NoneTick)))
  (if (not (Variables|Default|GetMultipleGimicSuccess))
    (bind _output_get (Variables|Default|SetIsGimic true))
    (Default|CallBeginSwitch _output_get)))

(event Custom|NoOperation
  (Variables|Default|SetHiting false)
  (if (not (Variables|Default|GetIsPlural))
    (for _array_element (Variables|Default|GetBP_Objectbys)
      (Default|SwitchInteractionEnd _array_element))
    (Utilities|FlowControl|Delay 2.0)
    (Actor|Tick|SetActorTickEnabled false)
    (else
      (bind _output_get (Variables|Default|SetIsGimic false))
      (Default|CallBeginSwitch _output_get))))

(event Custom|NoneTick
  (Actor|Tick|SetActorTickEnabled false))

(event EventBeginPlay
  (EventDispatchers|AssignOnTakeAnyDamage (delegate Custom|OnTakeAnyDamage_이벤트)))

(event Collision|EventActorBeginOverlap
  (params (OtherActor :type Actor%20Object%20Reference)))

(event EventTick
  (params (DeltaSeconds :type Float%20%28single-precision%29))
  (if (!= (Variables|Default|GetCustomTimeDilation) (Variables|Default|GetByCostomTime))
    (for _array_element (Variables|Default|GetBP_Objectbys)
      (Variables|/Script/Engine.Actor|SetCustomTimeDilation _array_element (Variables|Default|GetCustomTimeDilation)))
    (Variables|Default|SetByCostomTime (Variables|Default|GetCustomTimeDilation))))

(fn ConstructionScript)

(fn HitFunction
  (for _array_element (Variables|Default|GetBP_Objectbys)
    (Default|SwitchInteraction _array_element)))