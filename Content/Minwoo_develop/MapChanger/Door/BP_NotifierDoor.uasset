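; Door actor that slides open and closed, chains those calls to a linked NextDoor, and resets encounters when the player dies.
; A timeline lerps the mesh between closed and open markers, playing forward or in reverse.
; TempInitialize binds to the player's death, whose handler reinitializes the spawner array, unbinds, then reopens the doors after a delay.
; It also forwards an E-skill transform fix to the player.
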(event Custom|Event_PlayerDieSoInitialize
  (if (!= 0 (Utilities|Array|Length (Variables|Default|GetSpawnerArray)))
    (Variables|Default|SetisGetWorked false)
    (for _array_element (Variables|Default|GetSpawnerArray)
      (Class|MonsterSpawner|InitFunc _array_element))
    (EventDispatchers|UnbindEventfromOnPlayerDie (Variables|Default|GetBP_Player) (delegate Custom|Event_PlayerDieSoInitialize))
    (Utilities|FlowControl|Delay 3.0)
    (Class|NotifierDoor|SetOpenDoor)
    (bind _nextdoor (Variables|Default|GetNextDoor)
      (:then
        (Class|DoorNextDoor|SetOpenDoor _nextdoor))
      (:else))))

(event EventBeginPlay
  (bind _asbp_third_person_character (Utilities|Casting|CastToBP_ThirdPersonCharacter (Game|GetPlayerCharacter 0)))
  (Variables|Default|SetBP_Player _asbp_third_person_character))

(event EventInitFuncPlayerDie
  (Variables|Default|SetisGetWorked false)
  (Class|NotifierDoor|SetOpenDoor)
  (bind _nextdoor (Variables|Default|GetNextDoor)
    (:then
      (Class|DoorNextDoor|SetOpenDoor _nextdoor)
      (for _array_element (Variables|Default|GetSpawnerArray)
        (Class|MonsterSpawner|InitFunc _array_element)))
    (:else)))

(event EventSetCloseDoor
  (bind _nextdoor (Variables|Default|GetNextDoor)
    (:then
      (Class|DoorNextDoor|SetCloseDoor _nextdoor)
      (bind _새_트랙_0 (Timeline|타임라인 ReverseFromEnd)
        (:Update
          (Transformation|SetWorldLocation (Variables|Default|GetMOD_Gateway_Door_01_med_01_door) (Math|Vector|Lerp(Vector) (Transformation|GetWorldLocation (Variables|Default|GetDoor_Close)) (Transformation|GetWorldLocation (Variables|Default|GetDoor_Open)) _새_트랙_0) false false))))
    (:else
      (Timeline|타임라인 ReverseFromEnd))))

(event EventSetOpenDoor
  (EventDispatchers|UnbindEventfromOnPlayerDie (Variables|Default|GetBP_Player) (EventDispatchers|CreateEvent :!event Custom|Event_PlayerDieSoInitialize))
  (bind _nextdoor (Variables|Default|GetNextDoor)
    (:then
      (Class|DoorNextDoor|SetOpenDoor _nextdoor)
      (bind _새_트랙_0 (Timeline|타임라인 PlayFromStart)
        (:Update
          (Transformation|SetWorldLocation (Variables|Default|GetMOD_Gateway_Door_01_med_01_door) (Math|Vector|Lerp(Vector) (Transformation|GetWorldLocation (Variables|Default|GetDoor_Close)) (Transformation|GetWorldLocation (Variables|Default|GetDoor_Open)) _새_트랙_0) false false))))
    (:else
      (Timeline|타임라인 PlayFromStart))))

(event EventSetPlayerESkillLocation
  (Default|EskillTransFormFix (Variables|Default|GetBP_Player)))

(event EventTempInitialize
  (EventDispatchers|BindEventtoOnPlayerDie (Variables|Default|GetBP_Player) (delegate Custom|Event_PlayerDieSoInitialize)))

(fn ConstructionScript)