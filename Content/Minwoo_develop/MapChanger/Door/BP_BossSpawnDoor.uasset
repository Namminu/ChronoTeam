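; Boss arena door that, when the player overlaps it, plays an optional intro sequence once, closes via a timeline lerp and spawns the configured boss.
; Player death reinitializes the boss, reopens the door and re-arms the trigger after a delay.
; Boss death reopens the door and plays an optional end sequence, which fades and loads the next level when finished.
; Dispatchers broadcast entrance and player-or-boss death.
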(event Custom|Door%20Close
  (bind _새_트랙_0 (Timeline|Change%20Door%20State%20TImeline PlayFromStart)
    (:Update
      (Transformation|SetWorldLocation (Variables|Default|GetMOD_Gateway_Door_01_med_01_door) (Math|Vector|Lerp(Vector) (Transformation|GetWorldLocation (Variables|Default|GetDoor_Open)) (Transformation|GetWorldLocation (Variables|Default|GetDoor_Close)) _새_트랙_0) false false))))

(event Custom|Door%20Open
  (bind _새_트랙_0 (Timeline|Change%20Door%20State%20TImeline ReverseFromEnd)
    (:Update
      (Transformation|SetWorldLocation (Variables|Default|GetMOD_Gateway_Door_01_med_01_door) (Math|Vector|Lerp(Vector) (Transformation|GetWorldLocation (Variables|Default|GetDoor_Open)) (Transformation|GetWorldLocation (Variables|Default|GetDoor_Close)) _새_트랙_0) false false))))

(event Custom|Spawn%20MyBoss
  (bind _returnvalue (Game|SpawnActorfromClass (Variables|Default|GetMyBossClass) (Math|Transform|MakeTransform (.location (Transformation|GetWorldTransform (Variables|Default|GetArrow))) "0, 0, 0" "1.000000,1.000000,1.000000") "AdjustIfPossibleButDontSpawnIfColliding" "MultiplyWithRoot" 0 0))
  (Variables|Default|SetBossRef _returnvalue)
  (Actor|Tick|SetActorTickEnabled true)
  (EventDispatchers|BindEventtoBossMonsterDie (Variables|Default|GetBossRef) (delegate Custom|Boss%20Die%20Event))
  (Default|CallOnBossDoorEntrance false))

(event Custom|Temp_EndSequencer%20Event
  (EventDispatchers|UnbindEventfromOnFinished (stale Custom|Boss%20Die%20Event _returnvalue) (delegate Custom|Temp_EndSequencer%20Event))
  (Default|PlayerinSequence (Variables|Player|GetBP_Player) false)
  (bind _returnvalue (UserInterface|CreateWidget "/Game/Minwoo_develop/UI/BossUI/WZ_Fade_InOut.WZ_Fade_InOut_C"))
  (UserInterface|Viewport|AddtoViewport _returnvalue 0)
  (Utilities|FlowControl|Delay 0.6)
  (Game|OpenLevel(byName) (Variables|Default|GetNext%20Level)))

(event Custom|Boss%20Die%20Event
  (bind _bossref (Variables|Default|GetBossRef))
  (bind _bossendsequence (Variables|Default|GetBossEndSequence))
  (Actor|Tick|SetActorTickEnabled false)
  (Utilities|FlowControl|Delay (Variables|/Script/TeamChrono.Base_Boss|GetfBossDeathTime _bossref))
  (Default|CallOnPlayerorBossDie false)
  (Class|BaseBoss|ClearMyBoss _bossref)
  (Utilities|IsValid _bossendsequence
    (:Is%20Valid
      (bind _returnvalue (Sequencer|Player|CreateLevelSequencePlayer _bossendsequence))
      (EventDispatchers|BindEventtoOnFinished _returnvalue (delegate Custom|Temp_EndSequencer%20Event))
      (Sequencer|Player|Play _returnvalue :!class /Script/MovieScene.MovieSceneSequencePlayer))
    (:Is%20Not%20Valid
      _))
  (CallFunction|DoorOpen)
  (Default|PlayerinSequence (Variables|Player|GetBP_Player) true))

(event Custom|Player%20Die%20Event
  (Class|BaseBoss|InitFunc (Variables|Default|GetBossRef) (Transformation|GetWorldLocation (Variables|Default|GetArrow)))
  (Default|CallOnPlayerorBossDie true)
  (Utilities|FlowControl|Delay 4.0)
  (Variables|CheckPP|SetIsOverlap false)
  (Transformation|SetWorldLocation (Variables|Default|GetMOD_Gateway_Door_01_med_01_door) (Transformation|GetWorldLocation (Variables|Default|GetDoor_Open)) false true)
  (EventDispatchers|UnbindEventfromOnPlayerDie (Variables|Player|GetBP_Player) (EventDispatchers|CreateEvent :!event Custom|Player%20Die%20Event)))

(event Custom|BeginSequencer%20Finish%20Event
  (bind _bossref (Variables|Default|GetBossRef))
  (EventDispatchers|UnbindEventfromOnFinished (stale Collision|EventActorBeginOverlap _returnvalue) (delegate Custom|BeginSequencer%20Finish%20Event))
  (Default|PlayerinSequence (Variables|Player|GetBP_Player) false)
  (CallFunction|DoorClose)
  (CallFunction|SpawnMyBoss)
  (Utilities|IsValid _bossref
    (:Is%20Valid
      (Variables|/Script/TeamChrono.Base_Boss|SetbIsBeginSequencer _bossref true)
      (Rendering|SetActorHiddenInGame _bossref false))))

(event EventBeginPlay
  (bind _asbp_third_person_character (Utilities|Casting|CastToBP_ThirdPersonCharacter (Game|GetPlayerCharacter 0)))
  (Variables|Player|SetBP_Player _asbp_third_person_character))

(event Collision|EventActorBeginOverlap
  (params (OtherActor :type Actor%20Object%20Reference))
  (bind _bossbeginsequence (Variables|Default|GetBossBeginSequence))
  (bind _bossref (Variables|Default|GetBossRef))
  (if (Actor|ActorHasTag OtherActor "PLAYER")
    (EventDispatchers|BindEventtoOnPlayerDie (Variables|Player|GetBP_Player) (EventDispatchers|CreateEvent :!event Custom|Player%20Die%20Event))
    (if (not (Variables|CheckPP|GetIsOverlap))
      (Variables|CheckPP|SetIsOverlap true)
      (if (Variables|CheckPP|GetIsSequencer)
        (CallFunction|DoorClose :!label _label)
        (CallFunction|SpawnMyBoss)
        (Variables|/Script/TeamChrono.Base_Boss|SetbIsBeginSequencer _bossref true)
        (Rendering|SetActorHiddenInGame _bossref false)
        (else
          (Utilities|IsValid _bossbeginsequence
            (:Is%20Valid
              (bind _returnvalue (Sequencer|Player|CreateLevelSequencePlayer _bossbeginsequence))
              (EventDispatchers|BindEventtoOnFinished _returnvalue (delegate Custom|BeginSequencer%20Finish%20Event))
              (Sequencer|Player|Play _returnvalue :!class /Script/MovieScene.MovieSceneSequencePlayer)
              (Variables|CheckPP|SetIsSequencer true)
              (Default|PlayerinSequence (Variables|Player|GetBP_Player) true)
              (Default|CallOnBossDoorEntrance true))
            (:Is%20Not%20Valid
              (goto _label))))))))

(fn ConstructionScript)