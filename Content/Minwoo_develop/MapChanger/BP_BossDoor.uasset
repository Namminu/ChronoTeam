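; Boss room door actor that shuts once the player has passed through and reopens when its linked boss dies.
; A player-tagged actor ending overlap enables Tick and, the first time only, closes the door.
; Tick polls MyBoss.IsDie, then switches itself off and opens the door.
; One timeline, played forward or reversed, lerps the door mesh's world location between DoorClose and DoorOpen marker components.
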(event Custom|Door%20Open
  (bind _새_트랙_0 (Timeline|타임라인 PlayFromStart)
    (:Update
      (Transformation|SetWorldLocation (Variables|Default|GetMOD_Gateway_Door_01_med_01_door) (Math|Vector|Lerp(Vector) (Transformation|GetWorldLocation (Variables|Default|GetDoor_Close)) (Transformation|GetWorldLocation (Variables|Default|GetDoor_Open)) _새_트랙_0) false false))))

(event Custom|Door%20Close
  (bind _새_트랙_0 (Timeline|타임라인 ReverseFromEnd)
    (:Update
      (Transformation|SetWorldLocation (Variables|Default|GetMOD_Gateway_Door_01_med_01_door) (Math|Vector|Lerp(Vector) (Transformation|GetWorldLocation (Variables|Default|GetDoor_Close)) (Transformation|GetWorldLocation (Variables|Default|GetDoor_Open)) _새_트랙_0) false false))))

(event Collision|EventActorEndOverlap
  (params (OtherActor :type Actor%20Object%20Reference))
  (if (Actor|ActorHasTag OtherActor "PLAYER")
    (Actor|Tick|SetActorTickEnabled true)
    (if (not (Variables|Default|GetIsOverlap))
      (CallFunction|DoorClose)
      (Variables|Default|SetIsOverlap true))))

(event EventTick
  (params (DeltaSeconds :type Float%20%28single-precision%29))
  (if (Variables|/Script/TeamChrono.Base_Boss|GetbIsDie (Variables|Default|GetMyBoss))
    (Actor|Tick|SetActorTickEnabled false)
    (CallFunction|DoorOpen)))

(fn ConstructionScript)