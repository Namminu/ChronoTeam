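; Map-changer Blueprint providing player transition helper events; the file itself contains no movement logic.
; Fadein stores the third-person character, shows a fade widget and disables camera lag, then removes the widget and restores lag after a short delay.
; ChangeOrb calls EskillTransFormFix on that stored player.
; DamagetoActor applies minimal damage to a given actor and prints its name.
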(event EventChangeOrb
  (Default|EskillTransFormFix (Variables|Default|GetPlayer)))

(event EventBeginPlay)

(event EventDamagetoActor
  (params (DamagedActor :type Actor%20Object%20Reference))
  (Game|Damage|ApplyDamage DamagedActor 1.0 0 0)
  (Development|PrintString (Utilities|GetDisplayName DamagedActor)))

(event EventFadein
  (params (player :type Actor%20Object%20Reference))
  (bind _asbp_third_person_character (Utilities|Casting|CastToBP_ThirdPersonCharacter player))
  (Variables|Default|SetPlayer _asbp_third_person_character)
  (bind _returnvalue (UserInterface|CreateWidget "/Game/Minwoo_develop/UI/BossUI/WZ_Fade_InOut.WZ_Fade_InOut_C"))
  (bind _output_get (Variables|Default|SetFade%20WZ _returnvalue))
  (UserInterface|Viewport|AddtoViewport _output_get 0)
  (Utilities|FlowControl|Sequence
    (:then_0
      (Variables|/Script/Engine.SpringArmComponent|SetbEnableCameraLag (Variables|/Script/TeamChrono.TeamChronoCharacter|GetCameraBoom (Variables|Default|GetPlayer)) false))
    (:then_1
      (Default|Fadein (Variables|Default|GetFade%20WZ)))
    (:then_2
      (Utilities|FlowControl|Delay 0.5)
      (Widget|RemovefromParent (Variables|Default|GetFade%20WZ))
      (Variables|/Script/Engine.SpringArmComponent|SetbEnableCameraLag (Variables|/Script/TeamChrono.TeamChronoCharacter|GetCameraBoom (Variables|Default|GetPlayer)) true))))

(fn ConstructionScript)