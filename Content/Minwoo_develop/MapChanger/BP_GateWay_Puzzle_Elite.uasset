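; BP_GateWay_Puzzle_Elite is a gateway door that opens when its assigned monster, MyOneMonster, dies.
; Tick polls the monster's IsMonsterLive flag, then fires MyMonsterDied once and disables actor tick.
; A timeline moves the door mesh by lerping between the world locations of the DoorClose and DoorOpen markers.
; A loop over a MyMonsters array is left unconnected, so only the single monster gates the door.
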(event Custom|My%20Monster%20Died
  (bind _새_트랙_0 (Timeline|타임라인 PlayFromStart)
    (:Update
      (Transformation|SetWorldLocation (Variables|Default|GetMOD_Gateway_Door_01_med_01_door) (Math|Vector|Lerp(Vector) (Transformation|GetWorldLocation (Variables|Default|GetDoor_Close)) (Transformation|GetWorldLocation (Variables|Default|GetDoor_Open)) _새_트랙_0) false false))))

(event EventBeginPlay)

(event EventTick
  (params (DeltaSeconds :type Float%20%28single-precision%29))
  (bind _myonemonster (Variables|Default|GetMyOneMonster)
    (:then
      (if (not (Variables|/Script/TeamChrono.BaseMonster|GetisMonsterLive _myonemonster))
        (CallFunction|MyMonsterDied)
        (Actor|Tick|SetActorTickEnabled false)))
    (:else)))

(fn ConstructionScript)