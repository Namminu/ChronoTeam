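; BP_TestRenderVolume is a test volume that shows the static meshes inside it only while the player is in it.
; On BeginPlay it stores the StaticMeshActors overlapping its Box and hides them in game.
; When an actor tagged PLAYER begins overlapping, it unhides that cached list, and it hides the list again when the overlap ends.
; The list is gathered only once, so later changes to what the box contains are not tracked.
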(event EventBeginPlay
  (bind _output_get (Variables|Default|SetArray (Collision|GetOverlappingActors (Variables|Default|GetBox) "/Script/Engine.StaticMeshActor" :!class /Script/Engine.PrimitiveComponent)))
  (for _array_element _output_get
    (Rendering|SetActorHiddenInGame _array_element true)))

(event Collision|EventActorBeginOverlap
  (params (OtherActor :type Actor%20Object%20Reference))
  (if (Actor|ActorHasTag OtherActor "PLAYER")
    (for _array_element (Variables|Default|GetArray)
      (Rendering|SetActorHiddenInGame _array_element false))))

(event Collision|EventActorEndOverlap
  (params (OtherActor :type Actor%20Object%20Reference))
  (if (Actor|ActorHasTag OtherActor "PLAYER")
    (for _array_element (Variables|Default|GetArray)
      (Rendering|SetActorHiddenInGame _array_element true))))

(fn ConstructionScript)