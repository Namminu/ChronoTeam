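; BP_NotifierDoor is a map-changer door that opens and closes, passing each command along to an optional linked NextDoor.
; A timeline lerps the door mesh's world location between DoorClose and DoorOpen markers, playing forward to open and in reverse to close.
; A separate event calls EskillTransFormFix on the player's BP_ThirdPersonCharacter to fix the E-skill transform.
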(event EventTick
  (params (DeltaSeconds :type Float%20%28single-precision%29)))

(event EventSetCloseDoor
  (bind _nextdoor (Variables|Default|GetNextDoor)
    (:then
      (Class|DoorNextDoor|SetCloseDoor _nextdoor)
      (bind _새_트랙_0 (Timeline|타임라인 ReverseFromEnd)
        (:Update
          (Transformation|SetWorldLocation (Variables|Default|GetMOD_Gateway_Door_01_med_01_door) (Math|Vector|Lerp(Vector) (Transformation|GetWorldLocation (Variables|Default|GetDoor_Close)) (Transformation|GetWorldLocation (Variables|Default|GetDoor_Open)) _새_트랙_0) false false))))
    (:else
      (Timeline|타임라인 ReverseFromEnd))))

(event EventSetOpenDoor
  (bind _nextdoor (Variables|Default|GetNextDoor)
    (:then
      (Class|DoorNextDoor|SetOpenDoor _nextdoor)
      (bind _새_트랙_0 (Timeline|타임라인 PlayFromStart)
        (:Update
          (Transformation|SetWorldLocation (Variables|Default|GetMOD_Gateway_Door_01_med_01_door) (Math|Vector|Lerp(Vector) (Transformation|GetWorldLocation (Variables|Default|GetDoor_Close)) (Transformation|GetWorldLocation (Variables|Default|GetDoor_Open)) _새_트랙_0) false false))))
    (:else
      (Timeline|타임라인 PlayFromStart))))

(event EventSetPlayerESkillLocation
  (bind _asbp_third_person_character (Utilities|Casting|CastToBP_ThirdPersonCharacter (Game|GetPlayerCharacter 0)))
  (Default|EskillTransFormFix _asbp_third_person_character))

(fn ConstructionScript)