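; Gateway door that opens once every monster in its MyMonsters list is dead.
; With IsSameDoor set (entrance doubles as exit), it starts open and closes the first time the player character leaves its overlap; otherwise box collision is disabled.
; Tick prunes dead monsters and counts them against the initial total, then opens the door and disables itself.
; One timeline lerps the mesh between DoorClose and DoorOpen, reversed for closing.
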(event Custom|My%20Monster%20Died
  (bind _새_트랙_0 (Timeline|타임라인 PlayFromStart)
    (:Update
      (Transformation|SetWorldLocation (Variables|Default|GetMOD_Gateway_Door_01_med_01_door) (Math|Vector|Lerp(Vector) (Transformation|GetWorldLocation (Variables|Default|GetDoor_Close)) (Transformation|GetWorldLocation (Variables|Default|GetDoor_Open)) _새_트랙_0) false false))))

(event Custom|Door%20Closer
  (bind _새_트랙_0 (Timeline|타임라인 ReverseFromEnd)
    (:Update
      (Transformation|SetWorldLocation (Variables|Default|GetMOD_Gateway_Door_01_med_01_door) (Math|Vector|Lerp(Vector) (Transformation|GetWorldLocation (Variables|Default|GetDoor_Close)) (Transformation|GetWorldLocation (Variables|Default|GetDoor_Open)) _새_트랙_0) false false))))

(event EventBeginPlay
  (bind _box (Variables|Default|GetBox))
  (Variables|Default|SetInitArraySize (Utilities|Array|Length (Variables|Default|GetMyMonsters)))
  (if (Variables|Door|GetIsSameDoor)
    (Collision|SetCollisionEnabled _box "QueryOnly") ; 출입구가 같을 경우
    (Transformation|SetWorldLocation (Variables|Default|GetMOD_Gateway_Door_01_med_01_door) (Transformation|GetWorldLocation (Variables|Default|GetDoor_Open)) false false)
    (else
      (Collision|SetCollisionEnabled _box "NoCollision") ; 출입구가 다를 경우
    )))

(event EventTick
  (params (DeltaSeconds :type Float%20%28single-precision%29))
  (bind _mymonsters (Variables|Default|GetMyMonsters))
  (Utilities|FlowControl|Sequence
    (:then_0
      (for (_array_element _array_index) _mymonsters
        (Utilities|IsValid _array_element
          (:Is%20Valid
            (if (not (Variables|/Script/TeamChrono.BaseMonster|GetisMonsterLive _array_element))
              (Utilities|Array|RemoveIndex _mymonsters _array_index)
              (Variables|Default|SetDiedMonsterCount (+ 1 (Variables|Default|GetDiedMonsterCount))))))))
    (:then_1
      (if (== (Variables|Default|GetDiedMonsterCount) (Variables|Default|GetInitArraySize))
        (Utilities|FlowControl|DoOnce false
          (:Completed
            (CallFunction|MyMonsterDied)
            (Actor|Tick|SetActorTickEnabled false)))))))

(event Collision|EventActorEndOverlap
  (params (OtherActor :type Actor%20Object%20Reference))
  (if (Variables|Door|GetIsSameDoor)
    (Utilities|Casting|CastToBP_ThirdPersonCharacter OtherActor)
    (if (not (Variables|Default|GetIsOverlapped))
      (CallFunction|DoorCloser)
      (Variables|Default|SetIsOverlapped true))))

(fn ConstructionScript)