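; BP_TextPrinter is a trigger actor that shows tutorial text while the player stands inside its Box.
; On BeginPlay it passes NewText to the TutorialWZ user widget and hides TextWidget through a dynamic material's Opacity parameter.
; Player overlap begin and end drive a single timeline, reversed to fade in and played forward to fade out.
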(event OnComponentBeginOverlap(Box)
  (params (OverlappedComponent :type Primitive%20Component%20Object%20Reference) (OtherActor :type Actor%20Object%20Reference) (OtherComp :type Primitive%20Component%20Object%20Reference) (OtherBodyIndex :type Integer) (bFromSweep :type Boolean) (SweepResult :type Hit%20Result%20Structure%20%28by%20ref%29))
  (if (== OtherActor (Variables|Default|GetBP_Player))
    (CallFunction|TextFadein)))

(event OnComponentEndOverlap(Box)
  (params (OverlappedComponent :type Primitive%20Component%20Object%20Reference) (OtherActor :type Actor%20Object%20Reference) (OtherComp :type Primitive%20Component%20Object%20Reference) (OtherBodyIndex :type Integer))
  (if (== OtherActor (Variables|Default|GetBP_Player))
    (CallFunction|TextFadeOut)))

(event Custom|Text%20FadeIn
  (bind _새_트랙_0 (Timeline|타임라인 ReverseFromEnd)
    (:Update
      (Rendering|Material|SetScalarParameterValue (Variables|Default|GetTextMT) "Opacity" (Math|Float|Lerp 1.0 0.0 _새_트랙_0) :!class /Script/Engine.MaterialInstanceDynamic))))

(event Custom|Text%20FadeOut
  (bind _새_트랙_0 (Timeline|타임라인 PlayFromStart)
    (:Update
      (Rendering|Material|SetScalarParameterValue (Variables|Default|GetTextMT) "Opacity" (Math|Float|Lerp 1.0 0.0 _새_트랙_0) :!class /Script/Engine.MaterialInstanceDynamic))))

(event EventBeginPlay
  (bind _returnvalue (Rendering|Material|CreateDynamicMaterialInstance (Variables|Default|GetTextWidget) 0 0 "None" :!class /Script/Engine.PrimitiveComponent))
  (bind _output_get (Variables|Default|SetTextMT _returnvalue))
  (Rendering|Material|SetScalarParameterValue _output_get "Opacity" 0.0 :!class /Script/Engine.MaterialInstanceDynamic)
  (bind _asbp_third_person_character (Utilities|Casting|CastToBP_ThirdPersonCharacter (Game|GetPlayerCharacter 0)))
  (Variables|Default|SetBP_Player _asbp_third_person_character)
  (bind _astutorial_wz (Utilities|Casting|CastToTutorialWZ (UserInterface|GetUserWidgetObject (Variables|Default|GetTextWidget))))
  (bind _output_get_2 (Variables|Default|SetTutoWZ _astutorial_wz))
  (bind _newparam (CallFunction|SetWidgetText))
  (Default|InteractionText _output_get_2 _newparam))

(fn ConstructionScript)

(fn SetWidgetText
  (return (Variables|Default|GetnewText)))