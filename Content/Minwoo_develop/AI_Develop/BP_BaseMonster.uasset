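; Base monster Blueprint that provides a damage flash effect by temporarily changing the emissive look of the skeletal mesh.
; On BeginPlay it creates a dynamic material instance on the mesh's first material slot and caches the original emissive color and multiplier.
; The DamageFlash event applies the flash color and intensity, waits for the flash duration, then restores the cached values.
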(event EventBeginPlay
  (bind _returnvalue (Actor|GetComponentbyClass "/Script/Engine.SkeletalMeshComponent"))
  (Utilities|IsValid _returnvalue
    (:Is%20Valid
      (bind _returnvalue_2 (Rendering|Material|CreateDynamicMaterialInstance _returnvalue 0 0 "None" :!class /Script/Engine.PrimitiveComponent))
      (Variables|Default|SetFlash%20MTI _returnvalue_2)
      (bind _returnvalue_3 (Rendering|Material|GetVectorParameterValue (Variables|Default|GetFlash%20MTI) "EmissiveColor" :!class /Script/Engine.MaterialInstanceDynamic))
      (Variables|Default|SetInit%20Emissive%20Color _returnvalue_3)
      (bind _returnvalue_4 (Rendering|Material|GetScalarParameterValue (Variables|Default|GetFlash%20MTI) "EmissiveMutiplier" :!class /Script/Engine.MaterialInstanceDynamic))
      (Variables|Default|SetInit%20Emissive%20Mutiplier _returnvalue_4))))

(event EventDamageFlash
  (bind _flash_mti (Variables|Default|GetFlash%20MTI))
  (bind _flash_mti_2 (Variables|Default|GetFlash%20MTI))
  (Rendering|Material|SetVectorParameterValue _flash_mti_2 "EmissiveColor" (Variables|Default|GetFlash%20Color) :!class /Script/Engine.MaterialInstanceDynamic)
  (Rendering|Material|SetScalarParameterValue _flash_mti_2 "EmissiveMutiplier" (Variables|Default|GetFlash%20Intensity) :!class /Script/Engine.MaterialInstanceDynamic)
  (Utilities|FlowControl|Delay (Variables|Default|GetFlash%20Duration))
  (Rendering|Material|SetVectorParameterValue _flash_mti "EmissiveColor" (Variables|Default|GetInit%20Emissive%20Color) :!class /Script/Engine.MaterialInstanceDynamic)
  (Rendering|Material|SetScalarParameterValue _flash_mti "EmissiveMutiplier" (Variables|Default|GetInit%20Emissive%20Mutiplier) :!class /Script/Engine.MaterialInstanceDynamic)
  (Utilities|FlowControl|Delay (Variables|Default|GetFlash%20Duration)))

(fn ConstructionScript)