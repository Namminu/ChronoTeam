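; Chase-type monster Blueprint that attaches a sword on BeginPlay and handles its visual feedback and a melee hit check.
; DamageFlash briefly overrides the material's emissive color and multiplier, then restores cached values, forwarding the flash to the weapon.
; ChangeOpacity fades weapon and body materials, using timelines to mark the monster born after appearing or destroy it after disappearing.
; TempAttack sphere-traces between mesh sockets and damages hit components tagged PLAYER.
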(event EventBeginPlay
  (bind _fst_mti (Variables|Default|GetFst_MTI))
  ;[1 1 1] Begin Play
  (Class|BaseMonster|AttachWeapon "/Game/Minwoo_develop/AI_Develop/BP_Monster/Weapon/BP_Weapon_Sword.BP_Weapon_Sword_C" "Weapon_Sword")
  (Utilities|IsValid _fst_mti
    (:Is%20Valid
      (bind _returnvalue (Rendering|Material|GetVectorParameterValue _fst_mti "EmissiveColor" :!class /Script/Engine.MaterialInstanceDynamic))
      (Variables|DAMAGEFLASH|SetFst_Init_Color _returnvalue)
      (bind _returnvalue_2 (Rendering|Material|GetScalarParameterValue _fst_mti "EmissiveMutiplier" :!class /Script/Engine.MaterialInstanceDynamic))
      (Variables|DAMAGEFLASH|SetFst_Init_Multiplier _returnvalue_2))))

(event EventDamageFlash
  (bind _fst_mti (Variables|Default|GetFst_MTI))
  (bind _fst_mti_2 (Variables|Default|GetFst_MTI))
  ;[1 1 1] Damage Flash
  (Class|MonsterWeapon|DamageFlash (Variables|Default|GetWeaponInstance))
  (Rendering|Material|SetVectorParameterValue _fst_mti_2 "EmissiveColor" (Variables|DAMAGEFLASH|GetFlash%20Color) :!class /Script/Engine.MaterialInstanceDynamic)
  (Rendering|Material|SetScalarParameterValue _fst_mti_2 "EmissiveMutiplier" (Variables|DAMAGEFLASH|GetFlash%20Intensity) :!class /Script/Engine.MaterialInstanceDynamic)
  (Utilities|FlowControl|Delay (Variables|DAMAGEFLASH|GetFlash%20Duration))
  (Rendering|Material|SetVectorParameterValue _fst_mti "EmissiveColor" (Variables|DAMAGEFLASH|GetFst_Init_Color) :!class /Script/Engine.MaterialInstanceDynamic)
  (Rendering|Material|SetScalarParameterValue _fst_mti "EmissiveMutiplier" (Variables|DAMAGEFLASH|GetFst_Init_Multiplier) :!class /Script/Engine.MaterialInstanceDynamic)
  (Utilities|FlowControl|Delay (Variables|DAMAGEFLASH|GetFlash%20Duration)))

(event EventChangeOpacity
  (params (StartAlpha :type Float%20%28single-precision%29) (EndAlpha :type Float%20%28single-precision%29))
  ;[1 1 1] Change Opacity
  (Class|MonsterWeapon|ChangeOpacity (Variables|Default|GetWeaponInstance) StartAlpha EndAlpha)
  (if (> StartAlpha EndAlpha)
    ;;[1 1 1] IF (Opacity : Disappear)
    (bind _새_트랙_0 (Timeline|Disappear Play)
      (:Update
        (for _array_element (Variables|Default|GetMTIArray)
          (Rendering|Material|SetScalarParameterValue _array_element "Opacity" (Math|Float|Lerp StartAlpha EndAlpha _새_트랙_0) :!class /Script/Engine.MaterialInstanceDynamic)))
      (:Finished
        (Class|BaseMonster|MonDestroy)))
    (else
      ;;[1 1 1] IF (Opacity : Appear)
      (bind _새_트랙_0_2 (Timeline|Appear Play)
        (:Update
          (for _array_element_2 (Variables|Default|GetMTIArray)
            (Rendering|Material|SetScalarParameterValue _array_element_2 "Opacity" (Math|Float|Lerp StartAlpha EndAlpha _새_트랙_0_2) :!class /Script/Engine.MaterialInstanceDynamic)))
        (:Finished
          (Variables|Default|SetisMonsterBorn true))))))

(event EventTempAttack
  (bind _mesh (Variables|Character|GetMesh))
  ;[1 1 1] Attack Check Func
  (bind (_outhit _returnvalue) (Collision|SphereTraceForObjects (Transformation|GetSocketLocation _mesh "AttackStart") (Transformation|GetSocketLocation _mesh "AttackEnd") 5e+01 (Utilities|Array|MakeArray "ObjectTypeQuery3") false 0 "None"))
  (if _returnvalue
    (if (Components|ComponentHasTag (.HitComponent (Collision|BreakHitResult _outhit)) "PLAYER")
      (Game|Damage|ApplyDamage (.HitActor (Collision|BreakHitResult _outhit)) 1.0 0 0 "/Script/Engine.DamageType"))))

(fn ConstructionScript)