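; Elite magician monster that carries a staff, fires magic balls and casts a big attack spawned attached to the player.
; It begins invincible until a short birth delay ends and collects MAGIC_SPAWN-tagged spawners.
; Damage flashes mesh emissive and staff, while barrier hits briefly swap the shell effect.
; Timelines lift the body on death and fade opacity out; the fade-in branch is disconnected and only prints.
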(event EventBeginPlay
  ;[1 1 1] Begin Play
  (Utilities|FlowControl|Sequence
    (:then_0
      (Class|BaseMonster|AttachWeapon "/Game/Minwoo_develop/AI_Develop/BP_Monster/Weapon/BP_Weapon_Staff.BP_Weapon_Staff_C" "Weapon_Staff")
      (Variables|Default|SetInitBarrierEffect (Variables|Default|GetSpecificEffect)))
    (:then_1
      (Utilities|FlowControl|Delay 1.5)
      (Variables|Default|SetisInvincible false)
      (Variables|Default|SetisMonsterBorn true))
    (:then_2
      (bind _새_트랙_0 (Timeline|타임라인 Play)
        (:Update
          (Transformation|SetActorTransform (Math|Transform|MakeTransform (+ _새_트랙_0 (.location (Transformation|GetActorTransform))) "0, 0, 0" (Transformation|GetActorScale3D))))))))

(event EventChangeOpacity
  (params (StartAlpha :type Float%20%28single-precision%29) (EndAlpha :type Float%20%28single-precision%29))
  ;[1 1 1] Change Opacity
  (if (> StartAlpha EndAlpha)
    (Development|PrintString "Call Change IOpacity for Monster Died")
    ;;[1 1 1] IF (Opacity : Disappear)
    (Class|MonsterWeapon|ChangeOpacity (Variables|Default|GetWeaponInstance) StartAlpha EndAlpha)
    (bind _새_트랙_0 (Timeline|타임라인_1 Play)
      (:Update
        (for _array_element (Variables|Default|GetMTIArray)
          (Rendering|Material|SetScalarParameterValue _array_element "Opacity" (Math|Float|Lerp StartAlpha EndAlpha _새_트랙_0) :!class /Script/Engine.MaterialInstanceDynamic))))
    (else
      (Development|PrintString "Call Change Opacity For Monster born"))))

(event EventBeforeGimic
  ;[1 1 1] Before Gimic
  (Components|Activation|Activate (Variables|Default|GetSpecificEffect) false))

(event EventBarrierFlash
  ;[1 1 1] Barrier Damage Flash
  (Class|NiagaraComponent|SetAsset (Variables|Default|GetSpecificEffect) "/Game/All_Asset/BuffLoop/NS/Vfx_MagicShell_Magician.Vfx_MagicShell_Magician" true)
  (Utilities|FlowControl|Delay 0.5)
  (Class|NiagaraComponent|SetAsset (Variables|Default|GetSpecificEffect) "/Game/All_Asset/BuffLoop/NS/Vfx_MagicShell.Vfx_MagicShell" true))

(event EventWhyOnlyUGetDown
  (bind _returnvalue (Transformation|GetActorLocation))
  (bind _returnvalue_2 (Transformation|GetActorLocation))
  ;[1 1 1] Set Location : Z up for Not Digging in Ground When Magician Death
  (bind _move_magician_to_up (Timeline|타임라인_2 Play)
    (:Update
      (Transformation|SetActorLocation (Math|Vector|MakeVector (.x _returnvalue_2) (.y _returnvalue_2) (Math|Float|Lerp (.z _returnvalue) (+ (.z _returnvalue) 1.0) _move_magician_to_up)) false false))))

(event EventChangeMTI
  (bind _mesh (Variables|Character|GetMesh))
  (bind _mesh_2 (Variables|Character|GetMesh))
  (if (Variables|Default|GetisMTI)
    (Development|PrintString "Die")
    (Rendering|Material|SetMaterial _mesh 0 (Variables|Default|GetFst_MTI))
    (Rendering|Material|SetMaterial _mesh 1 (Variables|Default|GetSnd_MTI))
    (Variables|Default|SetisMTI false)
    (else
      (Development|PrintString "Born")
      (Rendering|Material|SetMaterial _mesh_2 0 "/Game/All_Asset/ToonSkeletonArmy/Characters/Materials/MI_ToonSkeleton_Magician_Opaque.MI_ToonSkeleton_Magician_Opaque")
      (Rendering|Material|SetMaterial _mesh_2 1 "/Game/All_Asset/ToonSkeletonArmy/Characters/Materials/MI_ToonSkeleton_Opaque.MI_ToonSkeleton_Opaque")
      (Variables|Default|SetisMTI true))))

(event EventSetFlashMTI
  ;[1 1 1] Flash MTI 설정
  (bind _returnvalue (Rendering|Material|CreateDynamicMaterialInstance (Variables|Character|GetMesh) 0 0 "None" :!class /Script/Engine.PrimitiveComponent))
  (Variables|Default|SetFst_FlashMTI _returnvalue)
  (bind _returnvalue_2 (Rendering|Material|CreateDynamicMaterialInstance (Variables|Character|GetMesh) 1 0 "None" :!class /Script/Engine.PrimitiveComponent))
  (Variables|Default|SetSnd_FlashMTI _returnvalue_2)
  (Utilities|IsValid (Variables|Default|GetFst_FlashMTI)
    (:Is%20Valid
      (bind _returnvalue_3 (Rendering|Material|GetVectorParameterValue (Variables|Default|GetFst_FlashMTI) "EmissiveColor" :!class /Script/Engine.MaterialInstanceDynamic))
      (Variables|DAMAGEFLASH|SetFst_Init_Color _returnvalue_3)
      (bind _returnvalue_4 (Rendering|Material|GetScalarParameterValue (Variables|Default|GetFst_FlashMTI) "EmissiveMutiplier" :!class /Script/Engine.MaterialInstanceDynamic))
      (Variables|DAMAGEFLASH|SetFst_Init_Multiplier _returnvalue_4)
      (Utilities|IsValid (Variables|Default|GetSnd_FlashMTI)
        (:Is%20Valid
          (bind _returnvalue_5 (Rendering|Material|GetVectorParameterValue (Variables|Default|GetSnd_FlashMTI) "EmissiveColor" :!class /Script/Engine.MaterialInstanceDynamic))
          (Variables|DAMAGEFLASH|SetSnd_Init_Color _returnvalue_5)
          (bind _returnvalue_6 (Rendering|Material|GetScalarParameterValue (Variables|Default|GetSnd_FlashMTI) "EmissiveMutiplier" :!class /Script/Engine.MaterialInstanceDynamic))
          (Variables|DAMAGEFLASH|SetSnd_Init_Multiplier _returnvalue_6))))))

(event EventBigAttackFunc
  ;[1 1 1] Attack Algorithm
  (if (Variables|Default|GetisBigAck)
    (Animation|PlayAnimMontage (Variables|Default|GetBigAtkMontage_Fst) 1.0 "None") ; Big Attack
    (else
      (Animation|PlayAnimMontage (Variables|Default|GetAtkMontage) 1.2 "None") ; Normal Atttack
    )))

(event EventMakeBigAttack
  (bind _player (Variables|Default|Getplayer))
  ;[1 1 1] Attack Algorithm
  ;;[1 1 1] Big Attack : SPawn BigAttack
  (bind _returnvalue (Game|SpawnActorfromClass "/Game/Minwoo_develop/AI_Develop/BP_Monster/Weapon/BP_Magician_BigAttack.BP_Magician_BigAttack_C" (Transformation|GetActorTransform _player) "Undefined" "MultiplyWithRoot" 0 0))
  (bind _output_get (Variables|Default|SetBigAttackBP _returnvalue))
  (Transformation|AttachActorToActor _output_get _player "None" "SnapToTarget" "SnapToTarget" "SnapToTarget" true))

(event EventSpawnMagicBall
  ;[1 1 1] Attack Algorithm
  ;;[1 1 1] Nromal Attack : Spawn Magic_Ball
  (Game|SpawnActorfromClass "/Game/Minwoo_develop/AI_Develop/BP_Monster/Weapon/BP_MagicBall.BP_MagicBall_C" (Math|Transform|MakeTransform (Transformation|GetSocketLocation (Variables|Character|GetMesh) "Weapon_MagicBall") (Transformation|GetActorRotation) "1.000000,1.000000,1.000000") "Undefined" "MultiplyWithRoot" 0 0))

(event EventDamageFlash
  (bind _fst_flashmti (Variables|Default|GetFst_FlashMTI))
  (bind _snd_flashmti (Variables|Default|GetSnd_FlashMTI))
  (bind _fst_flashmti_2 (Variables|Default|GetFst_FlashMTI))
  (bind _snd_flashmti_2 (Variables|Default|GetSnd_FlashMTI))
  ;[1 1 1] Damage Flash
  (Utilities|FlowControl|Sequence
    (:then_0
      (Rendering|Material|SetVectorParameterValue _fst_flashmti_2 "EmissiveColor" (Variables|DAMAGEFLASH|GetFlash%20Color) :!class /Script/Engine.MaterialInstanceDynamic)
      (Rendering|Material|SetScalarParameterValue _fst_flashmti_2 "EmissiveMutiplier" (Variables|DAMAGEFLASH|GetFlash%20Intensity) :!class /Script/Engine.MaterialInstanceDynamic)
      (Utilities|FlowControl|Delay (Variables|DAMAGEFLASH|GetFlash%20Duration))
      (Rendering|Material|SetVectorParameterValue _fst_flashmti "EmissiveColor" (Variables|DAMAGEFLASH|GetFst_Init_Color) :!class /Script/Engine.MaterialInstanceDynamic)
      (Rendering|Material|SetScalarParameterValue _fst_flashmti "EmissiveMutiplier" (Variables|DAMAGEFLASH|GetFst_Init_Multiplier) :!class /Script/Engine.MaterialInstanceDynamic))
    (:then_1
      (Rendering|Material|SetVectorParameterValue _snd_flashmti_2 "EmissiveColor" (Variables|DAMAGEFLASH|GetFlash%20Color) :!class /Script/Engine.MaterialInstanceDynamic)
      (Rendering|Material|SetScalarParameterValue _snd_flashmti_2 "EmissiveMutiplier" (Variables|DAMAGEFLASH|GetFlash%20Intensity) :!class /Script/Engine.MaterialInstanceDynamic)
      (Utilities|FlowControl|Delay (Variables|DAMAGEFLASH|GetFlash%20Duration))
      (Rendering|Material|SetVectorParameterValue _snd_flashmti "EmissiveColor" (Variables|DAMAGEFLASH|GetSnd_Init_Color) :!class /Script/Engine.MaterialInstanceDynamic)
      (Rendering|Material|SetScalarParameterValue _snd_flashmti "EmissiveMutiplier" (Variables|DAMAGEFLASH|GetSnd_Init_Multiplier) :!class /Script/Engine.MaterialInstanceDynamic))
    (:then_2
      (Class|MonsterWeapon|DamageFlash (Variables|Default|GetWeaponInstance)))))

(event EventAssgintoArray
  ;[1 1 1] Assgin Spawner to Array
  (bind _outactors (Actor|GetAllActorsOfClass "/Script/TeamChrono.MonsterSpawner"))
  (for _array_element _outactors
    (if (Actor|ActorHasTag _array_element "MAGIC_SPAWN")
      (Utilities|Array|Add (Variables|Default|GetSpawnerArray) _array_element))))

(fn ConstructionScript)