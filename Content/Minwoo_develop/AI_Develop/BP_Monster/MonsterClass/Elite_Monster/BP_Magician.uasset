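; BP_Magician is an elite skeleton magician monster that attaches a staff at BeginPlay and drops invincibility after three seconds.
; ChangeOpacity fades body materials and staff, calling ChangeMTI before disappearing and setting IsMonsterBorn once appearing finishes.
; ChangeMTI toggles IsMTI, but both branches apply the same opaque materials.
; BigAttackFunc's hardcoded true condition always plays the normal attack montage, leaving the big-attack montage unreachable.
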(event EventBeginPlay
  (Utilities|FlowControl|Sequence
    (:then_0
      (Class|BaseMonster|AttachWeapon "/Game/Minwoo_develop/AI_Develop/BP_Monster/Weapon/BP_Weapon_Staff.BP_Weapon_Staff_C" "Weapon_Staff"))
    (:then_1
      (Utilities|FlowControl|Delay 3.0)
      (Class|BaseEliteMonster|ChangeMTI)
      (Variables|Default|SetisInvincible false))))

(event EventBigAttackFunc
  (if true
    (Animation|PlayAnimMontage (Variables|Default|GetAtkMontage) 1.2 "None")
    (else
      (Animation|PlayAnimMontage (Variables|Default|GetBigAtkMontage_Fst) 1.0 "None"))))

(event EventChangeMTI
  (bind _mesh (Variables|Character|GetMesh))
  (bind _mesh_2 (Variables|Character|GetMesh))
  (if (Variables|Default|GetisMTI)
    (Rendering|Material|SetMaterial _mesh 0 "/Game/All_Asset/ToonSkeletonArmy/Characters/Materials/MI_ToonSkeleton_Magician_Opaque.MI_ToonSkeleton_Magician_Opaque")
    (Rendering|Material|SetMaterial _mesh 1 "/Game/All_Asset/ToonSkeletonArmy/Characters/Materials/MM_ToonSkeleton_Opaque.MM_ToonSkeleton_Opaque")
    (Variables|Default|SetisMTI false)
    (else
      (Rendering|Material|SetMaterial _mesh_2 0 "/Game/All_Asset/ToonSkeletonArmy/Characters/Materials/MI_ToonSkeleton_Magician_Opaque.MI_ToonSkeleton_Magician_Opaque")
      (Rendering|Material|SetMaterial _mesh_2 1 "/Game/All_Asset/ToonSkeletonArmy/Characters/Materials/MM_ToonSkeleton_Opaque.MM_ToonSkeleton_Opaque")
      (Variables|Default|SetisMTI true)))
  (Utilities|FlowControl|DoOnce false))

(event EventChangeOpacity
  (params (StartAlpha :type Float%20%28single-precision%29) (EndAlpha :type Float%20%28single-precision%29))
  ;[1 1 1] Change Opacity
  (if (> StartAlpha EndAlpha)
    (Class|BaseEliteMonster|ChangeMTI)
    ;;[1 1 1] IF (Opacity : Disappear)
    (Class|MonsterWeapon|ChangeOpacity (Variables|Default|GetWeaponInstance) StartAlpha EndAlpha)
    (bind _새_트랙_0 (Timeline|타임라인_0 Play)
      (:Update
        (for _array_element (Variables|Default|GetMTIArray)
          (Rendering|Material|SetScalarParameterValue _array_element "Opacity" (Math|Float|Lerp StartAlpha EndAlpha _새_트랙_0) :!class /Script/Engine.MaterialInstanceDynamic))))
    (else
      ;;[1 1 1] IF (Opacity : Appear)
      (Class|MonsterWeapon|ChangeOpacity (Variables|Default|GetWeaponInstance) StartAlpha EndAlpha)
      (bind _새_트랙_0_2 (Timeline|타임라인 Play)
        (:Update
          (for _array_element_2 (Variables|Default|GetMTIArray)
            (Rendering|Material|SetScalarParameterValue _array_element_2 "Opacity" (Math|Float|Lerp StartAlpha EndAlpha _새_트랙_0_2) :!class /Script/Engine.MaterialInstanceDynamic)))
        (:Finished
          (Variables|Default|SetisMonsterBorn true))))))

(fn ConstructionScript)