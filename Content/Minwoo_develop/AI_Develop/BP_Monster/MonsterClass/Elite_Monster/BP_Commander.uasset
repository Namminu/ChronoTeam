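; Elite Commander monster that fights with a blade and shield and has a shield-barrier gimmick.
; Turns toward the player and follows three normal attacks with a two-montage heavy attack, using sphere-trace functions to apply damage.
; Barrier functions pause a montage, outline the shield and manage a timer that clears the first-damaged flag.
; Shield material swaps and dynamic material parameters drive damage flashes and timeline-based appear/disappear fades across body and weapons.
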(event Custom|RotateToPlayer
  (bind _returnvalue (Transformation|GetActorRotation))
  ;[1 1 1] Rotate To Player : Called When Before Attack
  (bind _rotate_monster (Timeline|타임라인 PlayFromStart)
    (:Update
      (Transformation|SetActorRotation (Math|Rotator|MakeRotator (.roll _returnvalue) (.pitch _returnvalue) (.yaw (Math|Rotator|Lerp(Rotator) (Math|Rotator|MakeRotator 0.0 0.0 (.yaw _returnvalue)) (Math|Rotator|MakeRotator 0.0 0.0 (.yaw (Math|Rotator|FindLookatRotation (Transformation|GetActorLocation) (Transformation|GetActorLocation (Game|GetPlayerCharacter 0))))) _rotate_monster)))))
    (:Finished
      (AI|Components|Blackboard|SetValueasVector (AI|GetBlackboard 0) (Variables|Default|GetBBKey_TargetLocation) (Transformation|GetActorLocation)))))

(event Custom|Set%20Bool%20Return
  ;[1 1 1] Timer Func
  (Variables|Default|SetisGimicFirstDamaged false))

(event EventBeginPlay
  (bind _snd_mti (Variables|Default|GetSnd_MTI))
  (bind _fst_mti (Variables|Default|GetFst_MTI))
  ;[1 1 1] Begin Play
  (Utilities|FlowControl|Sequence
    (:then_0
      ;;[1 1 1] 무기 부착
      (Class|BaseMonster|AttachWeapon "/Game/Minwoo_develop/AI_Develop/BP_Monster/Weapon/BP_Weapon_SSShield.BP_Weapon_SSShield_C" "Weapon_Shield")
      (Variables|Default|SetShieldMT (Rendering|Material|GetMaterial (Variables|/Script/TeamChrono.Monster_Weapon|GetWeapon (Variables|Default|GetWeaponInstance)) 0))
      (Class|BaseEliteMonster|AttachMoreWeapon "/Game/Minwoo_develop/AI_Develop/BP_Monster/Weapon/BP_Weapon_Blade.BP_Weapon_Blade_C" "Weapon_Blade")
      (Transformation|SetActorRelativeScale3D (Variables|Default|GetWeaponInstance2) "1.000000,1.000000,2.000000")
      ;;[1 1 1] Flash MTI 설정
      (Utilities|IsValid _fst_mti
        (:Is%20Valid
          (bind _returnvalue (Rendering|Material|GetVectorParameterValue _fst_mti "EmissiveColor" :!class /Script/Engine.MaterialInstanceDynamic))
          (Variables|DAMAGEFLASH|SetFst_Init_Color _returnvalue)
          (bind _returnvalue_2 (Rendering|Material|GetScalarParameterValue _fst_mti "EmissiveMutiplier" :!class /Script/Engine.MaterialInstanceDynamic))
          (Variables|DAMAGEFLASH|SetFst_Init_Multiplier _returnvalue_2)
          (Utilities|IsValid _snd_mti
            (:Is%20Valid
              (bind _returnvalue_3 (Rendering|Material|GetVectorParameterValue _snd_mti "EmissiveColor" :!class /Script/Engine.MaterialInstanceDynamic))
              (Variables|DAMAGEFLASH|SetSnd_Init_Color _returnvalue_3)
              (bind _returnvalue_4 (Rendering|Material|GetScalarParameterValue _snd_mti "EmissiveMutiplier" :!class /Script/Engine.MaterialInstanceDynamic))
              (Variables|DAMAGEFLASH|SetSnd_Init_Multiplier _returnvalue_4))))))
    (:then_1
      (Utilities|FlowControl|Delay 3.0)
      (CallFunction|MTIFunc)
      (Variables|Default|SetisInvincible false)
      (Components|Activation|Deactivate (Variables|Default|GetSpecificEffect)))))

(event EventChangeOpacity
  (params (StartAlpha :type Float%20%28single-precision%29) (EndAlpha :type Float%20%28single-precision%29))
  ;[1 1 1] Change Opacity
  (if (> StartAlpha EndAlpha)
    (CallFunction|MTIFunc)
    ;;[1 1 1] IF (Opacity : Disappear)
    (Class|MonsterWeapon|ChangeOpacity (Variables|Default|GetWeaponInstance) StartAlpha EndAlpha)
    (bind _새_트랙_0 (Timeline|Disappear Play)
      (:Update
        (for _array_element (Variables|Default|GetMTIArray)
          (Rendering|Material|SetScalarParameterValue _array_element "Opacity" (Math|Float|Lerp StartAlpha EndAlpha _새_트랙_0) :!class /Script/Engine.MaterialInstanceDynamic))))
    (else
      ;;[1 1 1] IF (Opacity : Appear)
      (Class|MonsterWeapon|ChangeOpacity (Variables|Default|GetWeaponInstance) StartAlpha EndAlpha)
      (bind _새_트랙_0_2 (Timeline|Apeear Play)
        (:Update
          (for _array_element_2 (Variables|Default|GetMTIArray)
            (Rendering|Material|SetScalarParameterValue _array_element_2 "Opacity" (Math|Float|Lerp StartAlpha EndAlpha _새_트랙_0_2) :!class /Script/Engine.MaterialInstanceDynamic)))
        (:Finished
          (Variables|Default|SetisMonsterBorn true))))))

(event EventBeforeGimic
  (bind _gimic_montage (Variables|Default|GetGimic_Montage))
  ;[1 1 1] Before Gimic Activate
  (Rendering|SetRenderCustomDepth (Variables|/Script/TeamChrono.Monster_Weapon|GetWeapon (Variables|Default|GetWeaponInstance)) true)
  (Animation|PlayAnimMontage _gimic_montage 1.0 "None")
  (Class|AnimInstance|MontagePause (Components|SkeletalMesh|GetAnimInstance (Variables|Character|GetMesh)) _gimic_montage)
  (Audio|PlaySoundatLocation "/Game/Minwoo_develop/MonsterSound/EliteMonster/Commander_ShieldMake_Sound.Commander_ShieldMake_Sound" (Transformation|GetActorLocation) "0, 0, 0" 1.0 1.0 0.0 "/Game/Minwoo_develop/MonsterSound/Attenuation/SKMonsterSoundAttenuation.SKMonsterSoundAttenuation" 0 0 0))

(event EventTempBigAttack
  (bind _mesh (Variables|Character|GetMesh))
  (bind _returnvalue (Transformation|GetSocketLocation _mesh "AttackStart"))
  ;[1 1 1] Big Attack Check Func
  (bind (_outhit _returnvalue_2) (Collision|SphereTraceForObjects _returnvalue _returnvalue 2.8e+02 (Utilities|Array|MakeArray "ObjectTypeQuery3") false 0 "None"))
  (if _returnvalue_2
    (if (Components|ComponentHasTag (.HitComponent (Collision|BreakHitResult _outhit)) "PLAYER")
      (Game|Damage|ApplyDamage (.HitActor (Collision|BreakHitResult _outhit)) 2.0 0 0 "/Script/Engine.DamageType"))))

(event EventTempAttack
  (bind _mesh (Variables|Character|GetMesh))
  ;[1 1 1] Attack Check Func
  (bind (_outhit _returnvalue) (Collision|SphereTraceForObjects (Transformation|GetSocketLocation _mesh "AttackStart") (Transformation|GetSocketLocation _mesh "Commander_AttackEnd") 5e+01 (Utilities|Array|MakeArray "ObjectTypeQuery3") false 0 "None"))
  (if _returnvalue
    (if (Components|ComponentHasTag (.HitComponent (Collision|BreakHitResult _outhit)) "PLAYER")
      (Game|Damage|ApplyDamage (.HitActor (Collision|BreakHitResult _outhit)) (Math|Conversions|ToFloat(Integer) (Variables|Default|GetmonAtk)) 0 0 "/Script/Engine.DamageType"))))

(event EventDamageFlash
  (bind _snd_mti (Variables|Default|GetSnd_MTI))
  (bind _fst_mti (Variables|Default|GetFst_MTI))
  (bind _snd_mti_2 (Variables|Default|GetSnd_MTI))
  (bind _fst_mti_2 (Variables|Default|GetFst_MTI))
  ;[1 1 1] Damage Flash / Shield Flash
  (Utilities|FlowControl|Sequence
    (:then_0
      (Rendering|Material|SetVectorParameterValue _fst_mti_2 "EmissiveColor" (Variables|DAMAGEFLASH|GetFlash%20Color) :!class /Script/Engine.MaterialInstanceDynamic)
      (Rendering|Material|SetScalarParameterValue _fst_mti_2 "EmissiveMutiplier" (Variables|DAMAGEFLASH|GetFlash%20Intensity) :!class /Script/Engine.MaterialInstanceDynamic)
      (Utilities|FlowControl|Delay (Variables|DAMAGEFLASH|GetFlash%20Duration))
      (Rendering|Material|SetVectorParameterValue _fst_mti "EmissiveColor" (Variables|DAMAGEFLASH|GetFst_Init_Color) :!class /Script/Engine.MaterialInstanceDynamic)
      (Rendering|Material|SetScalarParameterValue _fst_mti "EmissiveMutiplier" (Variables|DAMAGEFLASH|GetFst_Init_Multiplier) :!class /Script/Engine.MaterialInstanceDynamic))
    (:then_1
      (Rendering|Material|SetVectorParameterValue _snd_mti "EmissiveColor" (Variables|DAMAGEFLASH|GetFlash%20Color) :!class /Script/Engine.MaterialInstanceDynamic)
      (Rendering|Material|SetScalarParameterValue _snd_mti "EmissiveMutiplier" (Variables|DAMAGEFLASH|GetFlash%20Intensity) :!class /Script/Engine.MaterialInstanceDynamic)
      (Utilities|FlowControl|Delay (Variables|DAMAGEFLASH|GetFlash%20Duration))
      (Rendering|Material|SetVectorParameterValue _snd_mti_2 "EmissiveColor" (Variables|DAMAGEFLASH|GetSnd_Init_Color) :!class /Script/Engine.MaterialInstanceDynamic)
      (Rendering|Material|SetScalarParameterValue _snd_mti_2 "EmissiveMutiplier" (Variables|DAMAGEFLASH|GetSnd_Init_Multiplier) :!class /Script/Engine.MaterialInstanceDynamic))
    (:then_2
      (Class|MonsterWeapon|DamageFlash (Variables|Default|GetWeaponInstance2))
      (Class|MonsterWeapon|DamageFlash (Variables|Default|GetWeaponInstance)))))

(event EventBigAttackFunc
  ;[1 1 1] 공격 메커니즘
  (CallFunction|RotatetoPlayer)
  (if (< (Variables|Default|GetcurrentAtkCount) 3)
    ;;[1 1 1] 일반 공격
    (Animation|PlayAnimMontage (Variables|Default|GetAtkMontage) 1.0 "None")
    (Variables|Default|SetcurrentAtkCount (+ (Variables|Default|GetcurrentAtkCount) 1))
    (else
      ;;[1 1 1] 강한 공격
      (Animation|PlayAnimMontage (Variables|Default|GetBigAtkMontage_Fst) 0.5 "None")
      (Utilities|FlowControl|Delay 1.3)
      (Animation|PlayAnimMontage (Variables|Default|GetBigAtkMontage_Snd) 2.0 "None")
      (Utilities|FlowControl|Delay 0.1)
      (Components|Activation|Activate (Variables|Default|GetNiagaraAttackEffect) false)
      (Variables|Default|SetcurrentAtkCount 0))))

(event EventPlayShieldBreakSound
  (Audio|PlaySoundatLocation "/Game/Minwoo_develop/MonsterSound/EliteMonster/Commander_ShieldBreak_Sound.Commander_ShieldBreak_Sound" (Transformation|GetActorLocation) "0, 0, 0" 2.0 1.0 0.0 "/Game/Minwoo_develop/MonsterSound/Attenuation/SKMonsterSoundAttenuation.SKMonsterSoundAttenuation" 0 0 0))

(event EventPlayShieldHitSound
  (Audio|PlaySoundatLocation "/Game/Minwoo_develop/MonsterSound/EliteMonster/Commander_ShieldHitted_Sound.Commander_ShieldHitted_Sound" (Transformation|GetActorLocation) "0, 0, 0" 2.0 1.0 0.0 "/Game/Minwoo_develop/MonsterSound/Attenuation/SKMonsterSoundAttenuation.SKMonsterSoundAttenuation" 0 0 0))

(event EventDamageWeaponFlash
  ;[1 1 1] Damage Flash / Shield Flash
  (Class|MonsterWeapon|DamageFlash (Variables|Default|GetWeaponInstance)))

(event EventSetGimicTimer
  ;[1 1 1] Timer Func
  (bind _returnvalue (Utilities|Time|SetTimerbyFunctionName 0 "Set Bool Return" (Variables|Default|GetBarrierHpTime))))

(event EventReSetTimer
  ;[1 1 1] Timer Func
  (Utilities|Time|ClearandInvalidateTimerbyHandle (stale EventSetGimicTimer _returnvalue))
  (Rendering|SetRenderCustomDepth (Variables|/Script/TeamChrono.Monster_Weapon|GetWeapon (Variables|Default|GetWeaponInstance)) false))

(event EventChangeMTI
  ;[1 1 1] Change MTI for OutLiner N DamageFlash
  (if (Variables|Default|GetisMTI)
    (Rendering|Material|SetMaterial (Variables|/Script/TeamChrono.Monster_Weapon|GetWeapon (Variables|Default|GetWeaponInstance)) 0 (Variables|Default|GetShieldMT)) ; change material to first MT
    (Variables|Default|SetisMTI false)
    (else
      (Rendering|Material|SetMaterial (Variables|/Script/TeamChrono.Monster_Weapon|GetWeapon (Variables|Default|GetWeaponInstance)) 0 "/Game/All_Asset/ToonSkeletonArmy/Weapons/Materials/MM_Change_Shield.MM_Change_Shield") ; change material for flash
      (Variables|Default|SetisMTI true))))

(fn ConstructionScript)

(fn MTIFunc
  (Class|BaseEliteMonster|ChangeMTI)
  (Utilities|FlowControl|DoOnce false
    (:Completed
      (Class|MonsterWeapon|SetFlashMTI (Variables|Default|GetWeaponInstance)))))