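; BP_SwordMonster is a sword monster Blueprint that extends its parent's damage flash to a second material instance, SndMTI.
; BeginPlay caches that material's initial emissive color and multiplier when it is valid.
; DamageFlash runs the parent flash, applies the flash color and intensity to SndMTI, then restores the cached values after a delay.
; ChangeOpacity only forwards to the parent, leaving SndMTI untouched.
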(event EventBeginPlay
  (bind _snd_mti (Variables|Default|GetSnd_MTI))
  (|CallParentFunction)
  (Utilities|IsValid _snd_mti
    (:Is%20Valid
      (bind _returnvalue (Rendering|Material|GetVectorParameterValue _snd_mti "EmissiveColor" :!class /Script/Engine.MaterialInstanceDynamic))
      (Variables|Default|SetSnd_Init_Color _returnvalue)
      (bind _returnvalue_2 (Rendering|Material|GetScalarParameterValue _snd_mti "EmissiveMutiplier" :!class /Script/Engine.MaterialInstanceDynamic))
      (Variables|Default|SetSnd_Init_Multiplier _returnvalue_2))))

(event EventChangeOpacity
  (params (StartAlpha :type Float%20%28single-precision%29) (EndAlpha :type Float%20%28single-precision%29))
  (|CallParentFunction StartAlpha EndAlpha))

(event EventDamageFlash
  (bind _snd_mti (Variables|Default|GetSnd_MTI))
  (bind _snd_mti_2 (Variables|Default|GetSnd_MTI))
  (|CallParentFunction)
  (Rendering|Material|SetVectorParameterValue _snd_mti "EmissiveColor" (Variables|Default|GetFlash%20Color) :!class /Script/Engine.MaterialInstanceDynamic)
  (Rendering|Material|SetScalarParameterValue _snd_mti "EmissiveMutiplier" (Variables|Default|GetFlash%20Intensity) :!class /Script/Engine.MaterialInstanceDynamic)
  (Utilities|FlowControl|Delay (Variables|Default|GetFlash%20Duration))
  (Rendering|Material|SetVectorParameterValue _snd_mti_2 "EmissiveColor" (Variables|Default|GetSnd_Init_Color) :!class /Script/Engine.MaterialInstanceDynamic)
  (Rendering|Material|SetScalarParameterValue _snd_mti_2 "EmissiveMutiplier" (Variables|Default|GetSnd_Init_Multiplier) :!class /Script/Engine.MaterialInstanceDynamic)
  (Utilities|FlowControl|Delay (Variables|Default|GetFlash%20Duration)))

(fn ConstructionScript
  (|CallParentFunction))