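; Sword weapon Blueprint for the Fighter boss monster that provides a timed emissive damage flash.
; BeginPlay caches the initial emissive color and multiplier from the material instance FstMTI, if it is valid.
; DamageFlash overrides both parameters with the flash color and intensity, waits for the flash duration, then restores the cached values.
; This graph neither creates FstMTI nor calls DamageFlash itself.
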(event EventBeginPlay
  (bind _fst_mti (Variables|Default|GetFst_MTI))
  (Utilities|IsValid _fst_mti
    (:Is%20Valid
      (bind _returnvalue (Rendering|Material|GetVectorParameterValue _fst_mti "EmissiveColor" :!class /Script/Engine.MaterialInstanceDynamic))
      (Variables|Default|SetFst_Init_Color _returnvalue)
      (bind _returnvalue_2 (Rendering|Material|GetScalarParameterValue _fst_mti "EmissiveMutiplier" :!class /Script/Engine.MaterialInstanceDynamic))
      (Variables|Default|SetFst_Init_Multiplier _returnvalue_2))))

(event EventDamageFlash
  (bind _fst_mti (Variables|Default|GetFst_MTI))
  (bind _fst_mti_2 (Variables|Default|GetFst_MTI))
  (Rendering|Material|SetVectorParameterValue _fst_mti_2 "EmissiveColor" (Variables|Default|GetFlash%20Color) :!class /Script/Engine.MaterialInstanceDynamic)
  (Rendering|Material|SetScalarParameterValue _fst_mti_2 "EmissiveMutiplier" (Variables|Default|GetFlash%20Intensity) :!class /Script/Engine.MaterialInstanceDynamic)
  (Utilities|FlowControl|Delay (Variables|Default|GetFlash%20Duration))
  (Rendering|Material|SetVectorParameterValue _fst_mti "EmissiveColor" (Variables|Default|GetFst_Init_Color) :!class /Script/Engine.MaterialInstanceDynamic)
  (Rendering|Material|SetScalarParameterValue _fst_mti "EmissiveMutiplier" (Variables|Default|GetFst_Init_Multiplier) :!class /Script/Engine.MaterialInstanceDynamic))

(fn ConstructionScript)