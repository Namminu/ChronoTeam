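; BP_Lightning is a lightning strike actor from the Fighter boss weapons that plays a thunder sound when it spawns.
; Its CalculateLightningAttack event waits briefly, plays the attack sound, then runs a stationary sphere trace for Pawns at the root scene's relative location.
; A hit component tagged PLAYER results in damage to its actor.
; Nothing in this graph calls the attack event.
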(event EventCalculateLightningAttack
  (bind _rootscene (Variables|Default|GetRootScene))
  (bind _relativelocation (Variables|/Script/Engine.SceneComponent|GetRelativeLocation _rootscene))
  (Utilities|FlowControl|Delay 0.55)
  (Audio|PlaySoundatLocation "/Game/Minwoo_develop/MonsterSound/Fighter/Fighter_TrdGimic_ThunderAttackSound_Cue.Fighter_TrdGimic_ThunderAttackSound_Cue" (Transformation|GetActorLocation) "0, 0, 0" 1.0 1.0 0.0 0 0 0 0)
  (bind _outhit (Collision|SphereTraceForObjects _relativelocation _relativelocation 1e+02 (Utilities|Array|MakeArray "ObjectTypeQuery3") false 0 "None"))
  (if true
    (if (Components|ComponentHasTag (.HitComponent (Collision|BreakHitResult _outhit)) "PLAYER")
      (Game|Damage|ApplyDamage (.HitActor (Collision|BreakHitResult _outhit)) 1.0 0 0 "/Script/Engine.DamageType"))))

(event EventBeginPlay
  (Audio|PlaySoundatLocation "/Game/Minwoo_develop/MonsterSound/Fighter/Fighter_TrdGimic_ThunderSound_Cue.Fighter_TrdGimic_ThunderSound_Cue" (Transformation|GetActorLocation) "0, 0, 0" 1.0 1.0 0.0 0 0 0 0))

(fn ConstructionScript)