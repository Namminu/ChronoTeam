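; BP_SndTornado is a tornado hazard actor for the Fighter boss that damages the player and starts dormant with tick disabled.
; SetTornadoAttack sets the Niagara effect, enables tick, plays spawn and sustain sounds, then destroys the actor after five seconds.
; While active, each tick sphere-traces for pawns at the root's relative location and damages a hit component tagged PLAYER every frame, with no cooldown.
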(event EventBeginPlay
  (Actor|Tick|SetActorTickEnabled false))

(event EventTick
  (params (DeltaSeconds :type Float%20%28single-precision%29))
  (bind _rootscene (Variables|Default|GetRootScene))
  (bind _relativelocation (Variables|/Script/Engine.SceneComponent|GetRelativeLocation _rootscene))
  (bind (_outhit _returnvalue) (Collision|SphereTraceForObjects _relativelocation _relativelocation 2.2e+02 (Utilities|Array|MakeArray "ObjectTypeQuery3") false 0 "None"))
  (if _returnvalue
    (if (Components|ComponentHasTag (.HitComponent (Collision|BreakHitResult _outhit)) "PLAYER")
      (Game|Damage|ApplyDamage (.HitActor (Collision|BreakHitResult _outhit)) 2.0 0 0 "/Script/Engine.DamageType"))))

(event EventSetTornadoAttack
  (bind _returnvalue (Transformation|GetActorLocation))
  (Class|NiagaraComponent|SetAsset (Variables|Default|GetTornadoEffect) "/Game/All_Asset/sA_DarkKnight_Set/Fx/NS_Aoe_1.NS_Aoe_1" true)
  (Actor|Tick|SetActorTickEnabled true)
  (Audio|PlaySoundatLocation "/Game/Minwoo_develop/MonsterSound/Fighter/Fighter_AddSound/Fighter_SndGImic_TornadoBorn_Sound_Cue.Fighter_SndGImic_TornadoBorn_Sound_Cue" _returnvalue "0, 0, 0" 1.0 1.0 0.0 0 0 0 0)
  (Audio|PlaySoundatLocation "/Game/Minwoo_develop/MonsterSound/Fighter/Fighter_AddSound/Fighter_SndGimic_TornadoKeep_Sound_Cue.Fighter_SndGimic_TornadoKeep_Sound_Cue" _returnvalue "0, 0, 0" 1.0 1.0 0.0 0 0 0 0)
  (Utilities|FlowControl|Delay 5.0)
  (Actor|DestroyActor))

(fn ConstructionScript)