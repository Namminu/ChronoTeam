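; BP_FstArrow is a Fighter boss weapon actor that deals delayed area damage to the player unless a marble blocks it.
; On BeginPlay it binds Sphere overlap, where contact with a MARBLE-tagged component sets IsOverlapped and disables the sphere's collision.
; After a short delay, it either hides its Niagara effect if blocked, or sphere-traces for a Pawn at the root's location and damages a PLAYER-tagged hit.
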(event Custom|Check%20Sphere%20Overlap%20to%20Marble
  (params (OverlappedComponent :type Primitive%20Component%20Object%20Reference) (OtherActor :type Actor%20Object%20Reference) (OtherComp :type Primitive%20Component%20Object%20Reference) (OtherBodyIndex :type Integer) (bFromSweep :type Boolean) (SweepResult :type Hit%20Result%20Structure%20%28by%20ref%29))
  (if (Components|ComponentHasTag OtherComp "MARBLE")
    (Variables|Default|SetIsOverlapped true)
    (Collision|SetCollisionEnabled (Variables|Default|GetSphere) "NoCollision")))

(event EventBeginPlay
  (bind _defaultsceneroot (Variables|Default|GetDefaultSceneRoot))
  (bind _relativelocation (Variables|/Script/Engine.SceneComponent|GetRelativeLocation _defaultsceneroot))
  (Collision|BindEventtoOnComponentBeginOverlap (Variables|Default|GetSphere) (delegate Custom|Check%20Sphere%20Overlap%20to%20Marble))
  (Utilities|FlowControl|Delay 1.3)
  (if (Variables|Default|GetIsOverlapped)
    (Development|SetHiddeninGame (Variables|Default|GetNiagara) true false)
    (else
      (bind (_outhit _returnvalue) (Collision|SphereTraceForObjects _relativelocation _relativelocation 8e+01 (Utilities|Array|MakeArray "ObjectTypeQuery3") false 0 "None"))
      (if _returnvalue
        (if (Components|ComponentHasTag (.HitComponent (Collision|BreakHitResult _outhit)) "PLAYER")
          (Game|Damage|ApplyDamage (.HitActor (Collision|BreakHitResult _outhit)) 1.0 0 0 "/Script/Engine.DamageType"))))))

(event EventDestroyed
  (Development|PrintString "Hello"))

(fn ConstructionScript)