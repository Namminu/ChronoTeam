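; Clock pin weapon actor for the Chrono boss that turns toward the player, then launches at their position.
; LaunchPin snapshots the player's location and timeline-lerps the pin there with a lowered Z.
; On arrival it sphere-traces to damage a PLAYER-tagged component, spawns a Niagara effect and enables collision.
; After a delay, BacktoBossSocket fades the dynamic material's opacity and destroys the actor rather than moving it back.
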(event EventBacktoBossSocket
  (Class|ChronoWeaponClockPin|ChangeOpacity))

(event EventBeginPlay
  (bind _pinmesh (Variables|Default|GetPinMesh))
  (Collision|SetCollisionEnabled (Variables|Default|GetPinMesh) "NoCollision")
  (Utilities|IsValid _pinmesh
    (:Is%20Valid
      (bind _returnvalue (Rendering|Material|CreateDynamicMaterialInstance _pinmesh 0 0 "None" :!class /Script/Engine.PrimitiveComponent))
      (Variables|Default|SetMeshMTI _returnvalue)
      (Utilities|FlowControl|Delay 0.3)
      (bind _새_트랙_0 (Timeline|Look%20Player PlayFromStart)
        (:Update
          (Transformation|SetActorRotation (Math|Rotator|Lerp(Rotator) (Transformation|GetActorRotation) (Math|Rotator|FindLookatRotation (Transformation|GetActorLocation) (Transformation|GetActorLocation (Game|GetPlayerCharacter 0))) _새_트랙_0 true)))))))

(event EventChangeOpacity
  (bind _새_트랙_0 (Timeline|Change%20Opacity%20Line PlayFromStart)
    (:Update
      (Rendering|Material|SetScalarParameterValue (Variables|Default|GetMeshMTI) "Opacity" (Math|Float|Lerp 1.0 0.0 _새_트랙_0) :!class /Script/Engine.MaterialInstanceDynamic))
    (:Finished
      (Actor|DestroyActor))))

(event EventCalculateHitRange
  (bind _implusepoint (Variables|Default|GetImplusePoint))
  (bind _returnvalue (Transformation|GetWorldLocation _implusepoint))
  ;[1 1 1] Calculate Hit Range For Player And Apply Damage
  (bind (_outhit _returnvalue_2) (Collision|SphereTraceForObjects _returnvalue _returnvalue 1.5e+02 (Utilities|Array|MakeArray "ObjectTypeQuery3") false 0 "ForDuration"))
  (if _returnvalue_2
    (if (Components|ComponentHasTag (.HitComponent (Collision|BreakHitResult _outhit)) "PLAYER")
      (Game|Damage|ApplyDamage (.HitActor (Collision|BreakHitResult _outhit)) 1.0 0 0 "/Script/Engine.DamageType"))))

(event EventLaunchPin
  (Variables|Default|SetInit%20Player%20Location (Transformation|GetActorLocation (Game|GetPlayerCharacter 0)))
  (bind _새_트랙_0 (Timeline|Temp%20Launch PlayFromStart)
    (:Update
      (Transformation|SetActorLocation (Math|Vector|MakeVector (.x (Math|Vector|Lerp(Vector) (Transformation|GetActorLocation) (Variables|Default|GetInit%20Player%20Location) _새_트랙_0)) (.y (Math|Vector|Lerp(Vector) (Transformation|GetActorLocation) (Variables|Default|GetInit%20Player%20Location) _새_트랙_0)) (- (.z (Variables|Default|GetInit%20Player%20Location)) (Variables|Default|GetZ_DownDegree))) false false))
    (:Finished
      (Class|ChronoWeaponClockPin|CalculateHitRange)
      (AddComponent|AddNiagaraComponent true (Math|Transform|MakeTransform (Transformation|GetWorldLocation (Variables|Default|GetEffect%20Point)) "0, 0, 0" "1.000000,1.000000,1.000000"))
      (Collision|SetCollisionEnabled (Variables|Default|GetPinMesh) "QueryAndPhysics")
      (Utilities|FlowControl|Delay 3.0)
      (Class|ChronoWeaponClockPin|BacktoBossSocket))))

(fn ConstructionScript)