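; Meteor actor for the Chrono boss's skill that plays a falling sound, then after a short delay damages the player at its location.
; The hit plays an impact sound and runs a single sphere trace for Pawns, with debug drawing on, damaging only a component tagged PLAYER.
; It finds Chrono in the level and binds to its die and in-sequence events to destroy itself, unbinding when destroyed.
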(event Custom|Calculate%20Meteor%20Hit%20Damage
  (bind _returnvalue (Transformation|GetActorLocation))
  (Audio|PlaySoundatLocation "/Game/Minwoo_develop/MonsterSound/Chrono/Skill/Chrono_Skill_MeteorHitSound_Cue.Chrono_Skill_MeteorHitSound_Cue" _returnvalue "0, 0, 0" 1.0 1.0 0.0 0 0 0 0)
  (bind (_outhit _returnvalue_2) (Collision|SphereTraceForObjects _returnvalue _returnvalue 4.5e+02 (Utilities|Array|MakeArray "ObjectTypeQuery3") false 0 "ForDuration"))
  (if _returnvalue_2
    (if (Components|ComponentHasTag (.HitComponent (Collision|BreakHitResult _outhit)) "PLAYER")
      (Game|Damage|ApplyDamage (.HitActor (Collision|BreakHitResult _outhit)) 1.0 0 0 "/Script/Engine.DamageType"))))

(event Custom|BeginInSequence
  (Actor|DestroyActor))

(event EventBeginPlay
  (CallFunction|CasttoChrono)
  (Audio|PlaySoundatLocation "/Game/Minwoo_develop/MonsterSound/Chrono/Skill/Chrono_Skill_MeteorFallingSound_Cue.Chrono_Skill_MeteorFallingSound_Cue" (Transformation|GetActorLocation) "0, 0, 0" 1.0 1.0 0.0 0 0 0 0)
  (Utilities|FlowControl|Delay 1.2)
  (CallFunction|CalculateMeteorHitDamage))

(event EventDestroyed
  (bind _chrono (Variables|Default|GetChrono))
  (EventDispatchers|UnbindEventfromOnChronoDie _chrono (delegate Custom|BeginInSequence))
  (EventDispatchers|UnbindEventfromOnChronoinSequence _chrono (delegate Custom|BeginInSequence)))

(fn ConstructionScript)

(fn CasttoChrono
  (bind _outactors (Actor|GetAllActorsOfClass "/Game/Minwoo_develop/AI_Develop/BP_Monster/MonsterClass/Boss_Monster/Chrono/CHRONO.CHRONO_C"))
  (for _array_element _outactors
    _)
  (bind _output_get (Variables|Default|SetChrono _array_element))
  (EventDispatchers|BindEventtoOnChronoinSequence _output_get (EventDispatchers|CreateEvent :!event Custom|BeginInSequence))
  (EventDispatchers|BindEventtoOnChronoDie _output_get (EventDispatchers|CreateEvent :!event Custom|BeginInSequence)))