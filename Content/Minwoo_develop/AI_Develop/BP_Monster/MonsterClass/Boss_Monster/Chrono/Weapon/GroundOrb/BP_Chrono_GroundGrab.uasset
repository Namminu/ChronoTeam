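; Ground grab hazard for the Chrono boss that drags the player to its center.
; When a PLAYER-tagged actor enters the Box, a one-second timer starts toward the grab event, and leaving the Box clears it.
; The grab plays a timeline that lerps the cached player's current location toward this actor's X and Y without sweep, keeping the player's own height.
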(event Custom|Get%20Player%20Grab
  (bind _returnvalue (Transformation|GetActorLocation))
  (bind _bp_player (Variables|Default|GetBP_Player))
  (bind _새_트랙_0 (Timeline|Set%20Player%20Location%20To%20Effect PlayFromStart)
    (:Update
      (Transformation|SetActorLocation _bp_player (Math|Vector|Lerp(Vector) (Transformation|GetActorLocation _bp_player) (Math|Vector|MakeVector (.x _returnvalue) (.y _returnvalue) (.z (Transformation|GetActorLocation (Variables|Default|GetBP_Player)))) _새_트랙_0) false false))))

(event Custom|Begin%20Overlap%20To%20Collision
  (params (OverlappedComponent :type Primitive%20Component%20Object%20Reference) (OtherActor :type Actor%20Object%20Reference) (OtherComp :type Primitive%20Component%20Object%20Reference) (OtherBodyIndex :type Integer) (bFromSweep :type Boolean) (SweepResult :type Hit%20Result%20Structure%20%28by%20ref%29))
  (if (Actor|ActorHasTag OtherActor "PLAYER")
    (bind _returnvalue (Utilities|Time|SetTimerbyFunctionName 0 "Get Player Grab" 1.0))))

(event Custom|EndOverlap%20To%20Collision
  (params (OverlappedComponent :type Primitive%20Component%20Object%20Reference) (OtherActor :type Actor%20Object%20Reference) (OtherComp :type Primitive%20Component%20Object%20Reference) (OtherBodyIndex :type Integer))
  (if (Actor|ActorHasTag OtherActor "PLAYER")
    (Utilities|Time|ClearandInvalidateTimerbyHandle (stale Custom|Begin%20Overlap%20To%20Collision _returnvalue))))

(event EventBeginPlay
  (bind _box (Variables|Default|GetBox))
  (bind _asbp_third_person_character (Utilities|Casting|CastToBP_ThirdPersonCharacter (Game|GetPlayerCharacter 0)))
  (Variables|Default|SetBP_Player _asbp_third_person_character)
  (Collision|BindEventtoOnComponentBeginOverlap _box (delegate Custom|Begin%20Overlap%20To%20Collision))
  (Collision|BindEventtoOnComponentEndOverlap _box (delegate Custom|EndOverlap%20To%20Collision)))

(fn ConstructionScript)