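; Clock pin projectile weapon of the Chrono boss that aims at the player, launches and deals damage on impact.
; A timeline turns it toward the player's location captured at the start, then sets the projectile component's speed.
; On hit it attaches to non-player surfaces and sphere-traces for pawns to spawn Niagara and damage the player.
; After a delay it zeroes speed, detaches and calls BackToBossSocket, which is empty here.
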(event EventBacktoBossSocket)

(event EventRotatetoPlayer
  ;[1 1 1] Rotate To Player Func
  (Variables|Default|SetInit%20Player%20Location (Transformation|GetActorLocation (Game|GetPlayerCharacter 0)))
  (bind _새_트랙_0 (Timeline|Look%20Player PlayFromStart)
    (:Update
      (Transformation|SetActorRotation (Math|Rotator|Lerp(Rotator) (Transformation|GetActorRotation) (Math|Rotator|FindLookatRotation (Transformation|GetActorLocation) (Variables|Default|GetInit%20Player%20Location)) _새_트랙_0 true)))
    (:Finished
      (Class|ChronoWeaponClockPin|LaunchPin (Variables|Default|GetLaunchSpeed)))))

(event EventCalculateHitRange
  (bind _implusepoint (Variables|Default|GetImplusePoint))
  (bind _returnvalue (Transformation|GetWorldLocation _implusepoint))
  ;[1 1 1] Calculate Hit Range For Player And Apply Damage
  (bind (_outhit _returnvalue_2) (Collision|SphereTraceForObjects _returnvalue _returnvalue 1.5e+02 (Utilities|Array|MakeArray "ObjectTypeQuery3") false 0 "ForDuration"))
  (if _returnvalue_2
    (AddComponent|AddNiagaraComponent true (Math|Transform|MakeTransform (.ImpactPoint (Collision|BreakHitResult _outhit)) (Math|Conversions|RotationFromXVector (.ImpactNormal (Collision|BreakHitResult _outhit))) "5.000000,5.000000,1.000000"))
    (if (Components|ComponentHasTag (.HitComponent (Collision|BreakHitResult _outhit)) "PLAYER")
      (Game|Damage|ApplyDamage (.HitActor (Collision|BreakHitResult _outhit)) 1.0 0 0 "/Script/Engine.DamageType"))))

(event Collision|EventHit
  (params (MyComp :type Primitive%20Component%20Object%20Reference) (Other :type Actor%20Object%20Reference) (OtherComp :type Primitive%20Component%20Object%20Reference) (bSelfMoved :type Boolean) (HitLocation :type Vector :default "0, 0, 0") (HitNormal :type Vector :default "0, 0, 0") (NormalImpulse :type Vector :default "0, 0, 0") (Hit :type Hit%20Result%20Structure%20%28by%20ref%29))
  (bind _projectilecomponent (Variables|Default|GetProjectileComponent))
  ;[1 1 1] Hit Event
  (if (Actor|ActorHasTag Other "PLAYER")
    _
    (else
      (Transformation|AttachComponentToComponent OtherComp "None" "KeepWorld" "KeepWorld" "KeepWorld" true)))
  (Class|ChronoWeaponClockPin|CalculateHitRange)
  (Utilities|FlowControl|Delay (Variables|Default|GetAttach%20Delay))
  (bind _output_get (Variables|/Script/Engine.ProjectileMovementComponent|SetInitialSpeed _projectilecomponent 0.0))
  (Variables|/Script/Engine.ProjectileMovementComponent|SetMaxSpeed _projectilecomponent _output_get)
  (Transformation|DetachFromActor "KeepWorld" "KeepWorld" "KeepWorld")
  (Class|ChronoWeaponClockPin|BacktoBossSocket))

(event EventLaunchPin
  (params (Speed :type Float%20%28single-precision%29))
  (bind _projectilecomponent (Variables|Default|GetProjectileComponent))
  (bind _output_get (Variables|/Script/Engine.ProjectileMovementComponent|SetInitialSpeed _projectilecomponent Speed))
  (Variables|/Script/Engine.ProjectileMovementComponent|SetMaxSpeed _projectilecomponent (+ _output_get 1e+02)))

(fn ConstructionScript)