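; BP_TestRock is a short-lived rock weapon, filed under the Golem boss, that damages the player on overlap.
; On BeginPlay it spawns a BP_Circle decal marker and attaches it to its Box, using the mesh's negated world height as relative Z to drop the marker to world zero.
; The rock destroys itself after a short delay.
; A DoOnce limits damage to one hit on an actor tagged PLAYER.
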(event EventBeginPlay
  (Utilities|FlowControl|Sequence
    (:then_0
      (bind _returnvalue (Game|SpawnActorfromClass "/Game/Minwoo_develop/AI_Develop/BP_Monster/MonsterClass/Boss_Monster/Golem/Material/BP_Circle.BP_Circle_C" (Math|Transform|MakeTransform (Math|Vector|MakeVector 0.0 0.0 (* (.z (Transformation|GetWorldLocation (Variables|Default|GetStaticMesh))) -1.0)) "0, 0, 0" "1.000000,1.000000,1.000000") "Undefined" "MultiplyWithRoot" 0 0))
      (bind _output_get (Variables|Default|SetDecal%20MT _returnvalue))
      (Transformation|AttachComponentToComponent _output_get (Variables|Default|GetBox) "None" "KeepRelative" "KeepRelative" "KeepWorld" true))
    (:then_1
      (Utilities|FlowControl|Delay 2.5)
      (Actor|DestroyActor))))

(event Collision|EventActorBeginOverlap
  (params (OtherActor :type Actor%20Object%20Reference))
  (if (Actor|ActorHasTag OtherActor "PLAYER")
    (Utilities|FlowControl|DoOnce false
      (:Completed
        (Game|Damage|ApplyDamage OtherActor 1.0 0 0)))))

(fn ConstructionScript)