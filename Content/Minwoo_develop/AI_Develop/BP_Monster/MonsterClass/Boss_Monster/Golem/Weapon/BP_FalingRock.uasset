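; BP_FalingRock is a falling-rock hazard among the Golem boss's weapons that damages the player on overlap.
; On BeginPlay it spawns a BP_Circle marker at the static mesh's X and Y position, then destroys itself after a short delay.
; The first overlap with an actor tagged PLAYER applies damage through a DoOnce and destroys the marker.
; The timed self-destruction does not explicitly remove the marker.
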(event EventBeginPlay
  (bind _staticmesh (Variables|Default|GetStaticMesh))
  (bind _returnvalue (Transformation|GetWorldLocation _staticmesh))
  (Utilities|FlowControl|Sequence
    (:then_0
      (bind _returnvalue_2 (Game|SpawnActorfromClass "/Game/Minwoo_develop/AI_Develop/BP_Monster/MonsterClass/Boss_Monster/Golem/Material/BP_Circle.BP_Circle_C" (Math|Transform|MakeTransform (Math|Vector|MakeVector (.x _returnvalue) (.y _returnvalue) 0.0) "0, 0, 0" "1.000000,1.000000,1.000000") "Undefined" "MultiplyWithRoot" 0 0))
      (Variables|Default|SetDecal%20MT _returnvalue_2))
    (:then_1
      (Utilities|FlowControl|Delay 2.5)
      (Actor|DestroyActor))))

(event Collision|EventActorBeginOverlap
  (params (OtherActor :type Actor%20Object%20Reference))
  (if (Actor|ActorHasTag OtherActor "PLAYER")
    (Utilities|FlowControl|DoOnce false
      (:Completed
        (Game|Damage|ApplyDamage OtherActor 1.0 0 0)
        (bind _decal_mt (Variables|Default|GetDecal%20MT)
          (:then
            (Actor|DestroyActor _decal_mt))
          (:else))))))

(fn ConstructionScript)