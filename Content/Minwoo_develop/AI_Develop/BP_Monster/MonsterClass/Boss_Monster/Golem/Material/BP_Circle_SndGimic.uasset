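; Circular danger-range indicator for a Golem boss gimmick, shown as an outline and a filling area.
; BeginPlay creates dynamic material instances for Circum and Area, using the Circum1Area0 parameter to switch one shared look between ring and fill.
; SetDanagerRangeEffect takes an EffectTime and, after a brief delay, runs a timeline that drives the area's AreaValue.
; The actor destroys itself shortly after the timeline finishes.
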(event Custom|Set%20Danager%20Range%20Effect
  (params (Effect%20Time :type Float%20%28double-precision%29))
  (Utilities|FlowControl|Delay 0.1)
  (bind _areavaluealpha (Timeline|타임라인 PlayFromStart)
    (:Update
      (Rendering|Material|SetScalarParameterValue (Variables|Default|GetArea%20Ref) "AreaValue" _areavaluealpha :!class /Script/Engine.MaterialInstanceDynamic))
    (:Finished
      (Utilities|FlowControl|Delay 0.1)
      (Actor|DestroyActor))))

(event EventBeginPlay
  (Utilities|FlowControl|Sequence
    (:then_0
      (bind _returnvalue (Rendering|Material|CreateDynamicMaterialInstance (Variables|Default|GetCircum) :!class /Script/Engine.DecalComponent))
      (bind _output_get (Variables|Default|SetCircumRef _returnvalue))
      (Rendering|Material|SetScalarParameterValue _output_get "Circum1Area0" 1.0 :!class /Script/Engine.MaterialInstanceDynamic))
    (:then_1
      (bind _returnvalue_2 (Rendering|Material|CreateDynamicMaterialInstance (Variables|Default|GetArea) :!class /Script/Engine.DecalComponent))
      (bind _output_get_2 (Variables|Default|SetArea%20Ref _returnvalue_2))
      (Rendering|Material|SetScalarParameterValue _output_get_2 "Circum1Area0" 0.0 :!class /Script/Engine.MaterialInstanceDynamic))))

(fn ConstructionScript)