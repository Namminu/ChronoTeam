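; Monster sword weapon Blueprint that drives the weapon's material for damage flashes and opacity fades.
; BeginPlay and SetFlashMTI create a dynamic material instance on the weapon or static mesh and cache its initial emissive color and multiplier.
; DamageFlash applies a flash color and intensity, then restores the cached values after a delay.
; ChangeOpacity compares start and end alpha to play a Disappear or Appear timeline that lerps Opacity.
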(event EventSetFlashMTI
  (bind _returnvalue (Actor|GetComponentbyClass "/Script/Engine.StaticMeshComponent"))
  (Utilities|IsValid (Variables|DAMAGEFLASH|GetFlash%20MTI)
    (:Is%20Valid
      (bind _returnvalue_2 (Rendering|Material|CreateDynamicMaterialInstance (Variables|Default|GetWeapon) 0 0 "None" :!class /Script/Engine.PrimitiveComponent))
      (Variables|DAMAGEFLASH|SetFlash%20MTI _returnvalue_2))
    (:Is%20Not%20Valid
      (Utilities|IsValid _returnvalue
        (:Is%20Valid
          (bind _returnvalue_3 (Rendering|Material|CreateDynamicMaterialInstance _returnvalue 0 0 "None" :!class /Script/Engine.PrimitiveComponent))
          (Variables|DAMAGEFLASH|SetFlash%20MTI _returnvalue_3)))))
  (bind _returnvalue_4 (Rendering|Material|GetVectorParameterValue (Variables|DAMAGEFLASH|GetFlash%20MTI) "EmissiveColor" :!class /Script/Engine.MaterialInstanceDynamic))
  (Variables|Default|SetInit%20Emissive%20Color _returnvalue_4)
  (bind _returnvalue_5 (Rendering|Material|GetScalarParameterValue (Variables|DAMAGEFLASH|GetFlash%20MTI) "EmissiveMutiplier" :!class /Script/Engine.MaterialInstanceDynamic))
  (Variables|Default|SetInit%20Emissive%20Mutiplier _returnvalue_5))

(event EventChangeOpacity
  (params (StartAlpha :type Float%20%28single-precision%29) (EndAlpha :type Float%20%28single-precision%29))
  ;[1 1 1] Change Opacity
  (if (> StartAlpha EndAlpha)
    ;;[1 1 1] IF (Opacity : Disappear)
    (bind _새_트랙_0 (Timeline|Disappear Play)
      (:Update
        (Rendering|Material|SetScalarParameterValue (Variables|DAMAGEFLASH|GetFlash%20MTI) "Opacity" (Math|Float|Lerp StartAlpha EndAlpha _새_트랙_0) :!class /Script/Engine.MaterialInstanceDynamic)))
    (else
      ;;[1 1 1] IF (Opacity : Appear)
      (bind _새_트랙_0_2 (Timeline|Appear Play)
        (:Update
          (Rendering|Material|SetScalarParameterValue (Variables|DAMAGEFLASH|GetFlash%20MTI) "Opacity" (Math|Float|Lerp StartAlpha EndAlpha _새_트랙_0_2) :!class /Script/Engine.MaterialInstanceDynamic))))))

(event EventDamageFlash
  (bind _flash_mti (Variables|DAMAGEFLASH|GetFlash%20MTI))
  (bind _flash_mti_2 (Variables|DAMAGEFLASH|GetFlash%20MTI))
  ;[1 1 1] Damage Flash
  (Rendering|Material|SetVectorParameterValue _flash_mti_2 "EmissiveColor" (Variables|DAMAGEFLASH|GetFlash%20Color) :!class /Script/Engine.MaterialInstanceDynamic)
  (Rendering|Material|SetScalarParameterValue _flash_mti_2 "EmissiveMutiplier" (Variables|DAMAGEFLASH|GetFlash%20Intensity) :!class /Script/Engine.MaterialInstanceDynamic)
  (Utilities|FlowControl|Delay (Variables|DAMAGEFLASH|GetFlash%20Duration))
  (Rendering|Material|SetVectorParameterValue _flash_mti "EmissiveColor" (Variables|Default|GetInit%20Emissive%20Color) :!class /Script/Engine.MaterialInstanceDynamic)
  (Rendering|Material|SetScalarParameterValue _flash_mti "EmissiveMutiplier" (Variables|Default|GetInit%20Emissive%20Mutiplier) :!class /Script/Engine.MaterialInstanceDynamic)
  (Utilities|FlowControl|Delay (Variables|DAMAGEFLASH|GetFlash%20Duration)))

(event EventBeginPlay
  (bind _returnvalue (Actor|GetComponentbyClass "/Script/Engine.StaticMeshComponent"))
  (Utilities|IsValid (Variables|DAMAGEFLASH|GetFlash%20MTI)
    (:Is%20Valid
      (bind _returnvalue_2 (Rendering|Material|CreateDynamicMaterialInstance (Variables|Default|GetWeapon) 0 0 "None" :!class /Script/Engine.PrimitiveComponent))
      (Variables|DAMAGEFLASH|SetFlash%20MTI _returnvalue_2))
    (:Is%20Not%20Valid
      (Utilities|IsValid _returnvalue
        (:Is%20Valid
          (bind _returnvalue_3 (Rendering|Material|CreateDynamicMaterialInstance _returnvalue 0 0 "None" :!class /Script/Engine.PrimitiveComponent))
          (Variables|DAMAGEFLASH|SetFlash%20MTI _returnvalue_3)))))
  (bind _returnvalue_4 (Rendering|Material|GetVectorParameterValue (Variables|DAMAGEFLASH|GetFlash%20MTI) "EmissiveColor" :!class /Script/Engine.MaterialInstanceDynamic))
  (Variables|Default|SetInit%20Emissive%20Color _returnvalue_4)
  (bind _returnvalue_5 (Rendering|Material|GetScalarParameterValue (Variables|DAMAGEFLASH|GetFlash%20MTI) "EmissiveMutiplier" :!class /Script/Engine.MaterialInstanceDynamic))
  (Variables|Default|SetInit%20Emissive%20Mutiplier _returnvalue_5))

(fn ConstructionScript)