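; Magician monster big attack actor that rings the player with five swords and closes them inward.
; On BeginPlay it activates five sword effect and hitbox pairs at staggered delays, then detaches from the player.
; A timeline then lerps each hitbox's relative XY toward the capsule, keeping its height.
; The timeline update also fires the hit effect and starts a one-second delay before the actor destroys itself.
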(event EventAttackFinally
  (bind _capsule (Variables|Default|GetCapsule))
  (bind _relativelocation (Variables|/Script/Engine.SceneComponent|GetRelativeLocation _capsule))
  (bind _새_트랙_2 (Timeline|타임라인 Play)
    (:Update
      (for _array_element (Variables|Default|GetHitBoxes)
        (Transformation|SetRelativeLocationAndRotation _array_element (Math|Vector|MakeVector (.x (Math|Vector|Lerp(Vector) (Math|Vector|MakeVector (.x (Variables|/Script/Engine.SceneComponent|GetRelativeLocation _array_element)) (.y (Variables|/Script/Engine.SceneComponent|GetRelativeLocation _array_element)) 0.0) (Math|Vector|MakeVector (.x _relativelocation) (.y _relativelocation) 0.0) _새_트랙_2)) (.y (Math|Vector|Lerp(Vector) (Math|Vector|MakeVector (.x (Variables|/Script/Engine.SceneComponent|GetRelativeLocation _array_element)) (.y (Variables|/Script/Engine.SceneComponent|GetRelativeLocation _array_element)) 0.0) (Math|Vector|MakeVector (.x _relativelocation) (.y _relativelocation) 0.0) _새_트랙_2)) (.z (Variables|/Script/Engine.SceneComponent|GetRelativeLocation _array_element))) (Variables|/Script/Engine.SceneComponent|GetRelativeRotation _array_element) false false))
      (Components|Activation|Activate (Variables|Default|GetHitEffect) false)
      (Utilities|FlowControl|Delay 1.0)
      (Actor|DestroyActor))))

(event EventBeginPlay
  (bind _sworddelay (Variables|Default|GetswordDelay))
  (Utilities|FlowControl|Delay _sworddelay)
  (Class|MagicianBigAttack|ActivateEffect (Variables|Default|GetSwordHitBox4) (Variables|Default|GetSwordEffect4))
  (Utilities|FlowControl|Delay _sworddelay)
  (Class|MagicianBigAttack|ActivateEffect (Variables|Default|GetSwordHitBox1) (Variables|Default|GetSwordEffect1))
  (Utilities|FlowControl|Delay _sworddelay)
  (Class|MagicianBigAttack|ActivateEffect (Variables|Default|GetSwordHitBox3) (Variables|Default|GetSwordEffect3))
  (Utilities|FlowControl|Delay _sworddelay)
  (Class|MagicianBigAttack|ActivateEffect (Variables|Default|GetSwordHitBox2) (Variables|Default|GetSwordEffect2))
  (Utilities|FlowControl|Delay _sworddelay)
  (Class|MagicianBigAttack|ActivateEffect (Variables|Default|GetSwordHitBox) (Variables|Default|GetSwordEffect))
  (Utilities|FlowControl|Delay 0.5)
  (Class|MagicianBigAttack|DetachfromPlayer)
  (Utilities|FlowControl|Delay 0.5)
  (CallFunction|AttackFinally))

(fn ConstructionScript)