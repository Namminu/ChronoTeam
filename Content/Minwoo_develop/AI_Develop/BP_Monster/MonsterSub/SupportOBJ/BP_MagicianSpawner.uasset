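; BP_MagicianSpawner is a child monster spawner that spawns magicians one at a time with a Niagara effect.
; SpawnMonster activates the effect, runs the parent spawn after a delay, binds the monster's death event, then animates effect scale by timeline before deactivating.
; Each death triggers a delayed respawn until SpawnCount is reached, then removes the spawner from ConnectDoor's array.
; InitFunc resets effect scale and initializes SpawnedMonster, destroying it four seconds later.
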(event Custom|Magician%20Die%20Event
  (if (== (Variables|Default|GetCurrentSpawn) (Variables|Default|GetSpawnCount))
    (EventDispatchers|UnbindEventfromMonsterDie (Variables|Default|GetSpawnedMonster) (EventDispatchers|CreateEvent :!event Custom|Magician%20Die%20Event))
    (Utilities|Array|RemoveItem (Variables|/Script/TeamChrono.NotifierDoor|GetSpawnerArray (Variables|Default|GetConnectDoor)) self)
    (else
      (Utilities|FlowControl|Delay 2.0)
      (Class|MonsterSpawner|SpawnMonster))))

(event EventBeginPlay
  (Components|Activation|Deactivate (Variables|Default|GetNiagara)))

(event EventInitFunc
  (bind _spawnedmonster (Variables|Default|GetSpawnedMonster))
  (|CallParentFunction)
  (Niagara|SetNiagaraVariable(Float) (Variables|Default|GetNiagara) "AllSizeScale" 2.5)
  (Class|BaseMonster|InitFunc _spawnedmonster)
  (Utilities|FlowControl|Delay 4.0)
  (Class|BaseMonster|MonDestroy _spawnedmonster))

(event EventTempSpawnerInitFunc)

(event EventSpawnMonster
  (bind _niagara (Variables|Default|GetNiagara))
  (Utilities|FlowControl|Sequence
    (:then_0
      (Components|Activation|Activate (Variables|Default|GetNiagara) true))
    (:then_1
      (Utilities|FlowControl|Delay 1.2)
      (|CallParentFunction)
      (EventDispatchers|BindEventtoMonsterDie (Variables|Default|GetSpawnedMonster) (EventDispatchers|CreateEvent :!event Custom|Magician%20Die%20Event)))
    (:then_2
      (Utilities|FlowControl|Delay 3.0)
      (bind _새_트랙_0 (Timeline|타임라인 Play)
        (:Update
          (Niagara|SetNiagaraVariable(Float) _niagara "AllSizeScale" _새_트랙_0))
        (:Finished
          (Components|Activation|Deactivate _niagara))))))

(fn ConstructionScript)