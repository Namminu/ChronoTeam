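; Monster spawner child Blueprint that spawns monsters one after another and keeps a connected door's tracking arrays updated.
; It extends parent spawn logic by binding to the monster's death, respawning after a short delay until the spawn count is reached, then removing itself from the door's spawner array.
; Separate events add or remove the monster in the door's array.
; InitFunc initializes the monster, then destroys and deregisters it after a delay.
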(event Custom|Monster%20Die%20So%20Spawn%20Next%20Monster
  (if (== (Variables|Default|GetCurrentSpawn) (Variables|Default|GetSpawnCount))
    (EventDispatchers|UnbindEventfromMonsterDie (Variables|Default|GetSpawnedMonster) (EventDispatchers|CreateEvent :!event Custom|Monster%20Die%20So%20Spawn%20Next%20Monster))
    (Utilities|Array|RemoveItem (Variables|/Script/TeamChrono.NotifierDoor|GetSpawnerArray (Variables|Default|GetConnectDoor)) self)
    (else
      (Utilities|FlowControl|Delay 1.0)
      (Class|MonsterSpawner|SpawnMonster))))

(event EventSpawnMonster
  (|CallParentFunction)
  (EventDispatchers|BindEventtoMonsterDie (Variables|Default|GetSpawnedMonster) (delegate Custom|Monster%20Die%20So%20Spawn%20Next%20Monster)))

(event EventAddMonster
  (Utilities|Array|Add (Variables|/Script/TeamChrono.NotifierDoor|GetMonsterArray (Variables|Default|GetConnectDoor)) (Variables|Default|GetSpawnedMonster)))

(event EventInitFunc
  (bind _spawnedmonster (Variables|Default|GetSpawnedMonster))
  (|CallParentFunction)
  (Class|BaseMonster|InitFunc _spawnedmonster)
  (Utilities|FlowControl|Delay 4.0)
  (Class|BaseMonster|MonDestroy _spawnedmonster)
  (Class|MonsterSpawner|RemoveMonster))

(event EventRemoveMonster
  (Utilities|Array|RemoveItem (Variables|/Script/TeamChrono.NotifierDoor|GetMonsterArray (Variables|Default|GetConnectDoor)) (Variables|Default|GetSpawnedMonster)))

(fn ConstructionScript)