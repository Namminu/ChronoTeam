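; BP_DamageFlash is a component-style Blueprint meant to flash its owner's skeletal mesh when it takes damage, but it is currently inactive.
; BeginPlay and the DamageFlash event are empty, with all logic left in disconnected nodes.
; The unwired setup binds to OnTakeAnyDamage, creates a dynamic material for slot 0 and caches its emissive color and multiplier.
; The unwired flash overrides both parameters, then restores them after a delay.
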(event Custom|DamageFlash
  (params (DamagedActor :type Actor%20Object%20Reference) (Damage :type Float%20%28single-precision%29) (DamageType :type Damage%20Type%20Object%20Reference) (InstigatedBy :type Controller%20Object%20Reference) (DamageCauser :type Actor%20Object%20Reference)))

(event EventBeginPlay)