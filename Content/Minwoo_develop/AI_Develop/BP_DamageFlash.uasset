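; Actor component that briefly flashes its owner's skeletal mesh whenever the owner takes damage.
; On BeginPlay it binds to the owner's any-damage event, creates a dynamic instance of the mesh's first material and caches the initial emissive color and multiplier.
; Each hit applies the flash color and intensity to those parameters, then restores the cached values after a delay.
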(event Custom|DamageFlash
  (params (DamagedActor :type Actor%20Object%20Reference) (Damage :type Float%20%28single-precision%29) (DamageType :type Damage%20Type%20Object%20Reference) (InstigatedBy :type Controller%20Object%20Reference) (DamageCauser :type Actor%20Object%20Reference))
  (bind _flash_mti (Variables|Initialization|GetFlash%20MTI))
  (bind _flash_mti_2 (Variables|Initialization|GetFlash%20MTI))
  (Rendering|Material|SetVectorParameterValue _flash_mti_2 "EmissiveColor" (Variables|FlashSetting|GetFlash%20Color) :!class /Script/Engine.MaterialInstanceDynamic)
  (Rendering|Material|SetScalarParameterValue _flash_mti_2 "EmissiveMutiplier" (Variables|FlashSetting|GetFlash%20Intensity) :!class /Script/Engine.MaterialInstanceDynamic)
  (Utilities|FlowControl|Delay (Variables|FlashSetting|GetFlash%20Duration))
  (Rendering|Material|SetVectorParameterValue _flash_mti "EmissiveColor" (Variables|Initialization|GetInit%20Emissive%20Color) :!class /Script/Engine.MaterialInstanceDynamic)
  (Rendering|Material|SetScalarParameterValue _flash_mti "EmissiveMutiplier" (Variables|Initialization|GetInit%20Emissive%20Mutiplier) :!class /Script/Engine.MaterialInstanceDynamic))

(event EventBeginPlay
  (bind _returnvalue (Components|GetOwner))
  (Variables|Initialization|SetOwner _returnvalue)
  (EventDispatchers|BindEventtoOnTakeAnyDamage _returnvalue (EventDispatchers|CreateEvent :!event Custom|DamageFlash))
  (Utilities|IsValid (Actor|GetComponentbyClass (Variables|Initialization|GetOwner) "/Script/Engine.SkeletalMeshComponent")
    (:Is%20Valid
      (bind _returnvalue_2 (Rendering|Material|CreateDynamicMaterialInstance (Actor|GetComponentbyClass (Variables|Initialization|GetOwner) "/Script/Engine.SkeletalMeshComponent") 0 0 "None" :!class /Script/Engine.PrimitiveComponent))
      (Variables|Initialization|SetFlash%20MTI _returnvalue_2)
      (bind _returnvalue_3 (Rendering|Material|GetVectorParameterValue (Variables|Initialization|GetFlash%20MTI) "EmissiveColor" :!class /Script/Engine.MaterialInstanceDynamic))
      (Variables|Initialization|SetInit%20Emissive%20Color _returnvalue_3)
      (bind _returnvalue_4 (Rendering|Material|GetScalarParameterValue (Variables|Initialization|GetFlash%20MTI) "EmissiveMutiplier" :!class /Script/Engine.MaterialInstanceDynamic))
      (Variables|Initialization|SetInit%20Emissive%20Mutiplier _returnvalue_4))))