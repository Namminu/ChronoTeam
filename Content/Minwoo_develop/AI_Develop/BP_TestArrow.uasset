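; BP_TestArrow is a test arrow actor with unfinished logic for destroying itself after travelling a set distance.
; BeginPlay records the start location, and Tick is empty.
; A disconnected chain, which never runs, prints the world X displacement from that start and destroys the actor once it exceeds TargetPosition.
; The Blueprint graphs contain no movement logic.
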(event EventBeginPlay
  (Variables|Default|SetStartPosition (Transformation|GetActorLocation)))

(event EventTick
  (params (DeltaSeconds :type Float%20%28single-precision%29)))

(fn ConstructionScript)