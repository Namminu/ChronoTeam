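; BP_SetFireOnStove is a trigger that lights fires on two stoves when the player character enters its box.
; BeginPlay caches the player's BP_ThirdPersonCharacter, and the Box overlap event responds only to that actor.
; Each overlap attaches a dungeon fire emitter at both stove fire locations and raises their point lights to a bright intensity.
; Nothing guards against repeat triggering, so re-entering the box spawns additional emitters.
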(event OnComponentBeginOverlap(Box)
  (params (OverlappedComponent :type Primitive%20Component%20Object%20Reference) (OtherActor :type Actor%20Object%20Reference) (OtherComp :type Primitive%20Component%20Object%20Reference) (OtherBodyIndex :type Integer) (bFromSweep :type Boolean) (SweepResult :type Hit%20Result%20Structure%20%28by%20ref%29))
  (if (== OtherActor (Variables|Default|GetBP_Player))
    (Utilities|FlowControl|Sequence
      (:then_0
        (Effects|SpawnEmitterAttached "/Game/All_Asset/Fantastic_Dungeon_Pack/effects/PS_FX_fire_dungeon_01.PS_FX_fire_dungeon_01" (Variables|Default|GetStove2FireLocation) "None")
        (Rendering|Components|Light|SetIntensity (Variables|Default|GetPointLight) 31852.0))
      (:then_1
        (Effects|SpawnEmitterAttached "/Game/All_Asset/Fantastic_Dungeon_Pack/effects/PS_FX_fire_dungeon_01.PS_FX_fire_dungeon_01" (Variables|Default|GetStove1FireLocation) "None")
        (Rendering|Components|Light|SetIntensity (Variables|Default|GetPointLight1) 31852.0)))))

(event EventBeginPlay
  (bind _asbp_third_person_character (Utilities|Casting|CastToBP_ThirdPersonCharacter (Game|GetPlayerCharacter 0)))
  (Variables|Default|SetBP_Player _asbp_third_person_character))

(fn ConstructionScript)