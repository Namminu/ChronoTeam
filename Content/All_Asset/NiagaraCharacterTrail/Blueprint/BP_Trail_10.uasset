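; BP_Trail_10 drives a material-based motion trail effect on a character's skeletal mesh.
; Call_Trail_10 replaces the first material slot with a dynamic instance of MI_Male_Body_9 and starts a looping, roughly per-frame timer.
; Each tick feeds the reversed capsule forward vector into Direction and scales Intensity with movement speed, so the effect points behind the character and strengthens as it moves faster.
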(event Custom|Call_Trail_10
  ;[0 0.4494 1] Apply the effect to the get skeletal mesh
  (Utilities|Time|SetTimerbyEvent (delegate Custom|Timer) 0.016 true)
  (bind _returnvalue (Rendering|Material|CreateDynamicMaterialInstance (Variables|/Script/Engine.Character|GetMesh (Variables|Default|GetCharacter)) 0 "/Game/All_Asset/NiagaraCharacterTrail/DemoRoom/SkeletalMeshExample/Character/Materials/MI_Male_Body_9.MI_Male_Body_9" "None" :!class /Script/Engine.PrimitiveComponent))
  (Variables|Default|SetDMI _returnvalue))

(event Custom|Timer
  (bind _dmi (Variables|Default|GetDMI))
  (bind _character (Variables|Default|GetCharacter))
  ;[0 0.4494 1] Apply the effect to the get skeletal mesh
  (Rendering|Material|SetVectorParameterValue _dmi "Direction" (Math|Conversions|ToLinearColor(Vector) (* (Math|Vector|GetForwardVector (Variables|/Script/Engine.Character|GetCapsuleComponent _character)) -1.0)) :!class /Script/Engine.MaterialInstanceDynamic)
  (Rendering|Material|SetScalarParameterValue _dmi "Intensity" (Math|Float|Lerp 0.0 1e+03 (/ (Math|Vector|VectorLength (Transformation|GetVelocity _character)) 1.5e+03)) :!class /Script/Engine.MaterialInstanceDynamic))

(event EventBeginPlay
  ;[0 0.4494 1] Apply the effect to the get skeletal mesh
)