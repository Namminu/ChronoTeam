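; BP_Trail_1 is a short-lived afterimage actor that leaves a shadow snapshot of a character's pose as a trail effect.
; When Call_Trail_1 runs, its PoseableMesh copies the Character's skeletal mesh and current pose, with M_Shadow on the first two material slots.
; It randomizes the material's Random parameter, then a timeline animates Alpha and destroys the actor on finish.
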(event Custom|Call_Trail_1
  (bind _character (Variables|Default|GetCharacter))
  (bind _poseablemesh (Variables|Default|GetPoseableMesh))
  (bind _poseablemesh_2 (Variables|Default|GetPoseableMesh))
  (bind _mesh (Variables|/Script/Engine.Character|GetMesh _character))
  ;[0 0.5467 1] Apply the effect to the get skeletal mesh
  (Components|SkinnedMesh|SetSkinnedAssetandUpdate _poseablemesh_2 (Variables|/Script/Engine.SkinnedMeshComponent|GetSkeletalMesh _mesh) true)
  (Rendering|Material|SetMaterial _poseablemesh_2 0 "/Game/All_Asset/NiagaraCharacterTrail/Materials/M_Shadow.M_Shadow")
  (Rendering|Material|SetMaterial _poseablemesh_2 1 "/Game/All_Asset/NiagaraCharacterTrail/Materials/M_Shadow.M_Shadow")
  (Rendering|Material|SetScalarParameterValueonMaterials _poseablemesh "Random" (Math|Random|RandomFloat))
  (Class|PoseableMeshComponent|CopyPosefromSkeletalComponent _poseablemesh _mesh)
  (bind _newtrack_0 (Timeline|Timeline_0 PlayFromStart)
    (:Update
      (Rendering|Material|SetScalarParameterValueonMaterials (Variables|Default|GetPoseableMesh) "Alpha" _newtrack_0))
    (:Finished
      (Actor|DestroyActor))))

(fn ConstructionScript)