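; Demo character that showcases one of ten trail effects, chosen by its Style value at BeginPlay.
; Style 1 uses a looping timer to repeatedly spawn a BP_Trail_1 actor at the mesh transform and hand it the character.
; The other styles initialize their matching BPTrail object with the character and call its trail function.
; For demonstration, chained AIMoveTo calls walk the character back and forth between TargetA and TargetB.
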(event Custom|Trail_1
  ;[0 0.1626 1] If you want to apply this effect to your custom characters, you can Migrate the BP_Trail (in the blueprint folder) to your project, and then copy this node into your character blueprint
  (bind _returnvalue (Game|SpawnActorfromClass "/Game/All_Asset/NiagaraCharacterTrail/Blueprint/BP_Trail_1.BP_Trail_1_C" (Transformation|GetWorldTransform (Variables|Character|GetMesh)) "Undefined" "OverrideRootScale" 0 0))
  (Variables|/Game/All_Asset/NiagaraCharacterTrail/Blueprint/BP_Trail_1.BP_Trail_1_C|SetCharacter _returnvalue self)
  (Default|CallTrail1 _returnvalue))

(event Custom|Move
  (bind _self self)
  (bind _returnvalue (AI|GetAIController _self))
  ;[1 0 0.4186] For demonstration
  (AI|AIMoveTo _returnvalue (Transformation|GetWorldLocation (Variables|/Script/Engine.Actor|GetRootComponent (Variables|Default|GetTarget_A))) 0 -1.0 "Default" "Default" true true :!label _label
    (:OnMoveFinished
      (AI|AIMoveTo _returnvalue (Transformation|GetWorldLocation (Variables|/Script/Engine.Actor|GetRootComponent (Variables|Default|GetTarget_B))) 0 -1.0 "Default" "Default" true true
        (:OnMoveFinished
          (goto _label))))))

(event EventBeginPlay
  (bind _bp_trail_2 (Variables|Default|GetBP_Trail_2))
  (bind _bp_trail_3 (Variables|Default|GetBP_Trail_3))
  (bind _bp_trail_8 (Variables|Default|GetBP_Trail_8))
  (bind _bp_trail_9 (Variables|Default|GetBP_Trail_9))
  (bind _bp_trail_4 (Variables|Default|GetBP_Trail_4))
  (bind _bp_trail_7 (Variables|Default|GetBP_Trail_7))
  (bind _bp_trail_5 (Variables|Default|GetBP_Trail_5))
  (bind _bp_trail_6 (Variables|Default|GetBP_Trail_6))
  (bind _bp_trail_10 (Variables|Default|GetBP_Trail_10))
  (switch int (Variables|Default|GetStyle)
    (:1
      ;[0 0.1626 1] If you want to apply this effect to your custom characters, you can Migrate the BP_Trail (in the blueprint folder) to your project, and then copy this node into your character blueprint
      (Utilities|Time|SetTimerbyEvent (delegate Custom|Trail_1) 0.15 true)
      (CallFunction|Move))
    (:2
      ;[0 0.3128 1] Style 2
      (Default|Initialize _bp_trail_2 self)
      (Default|CallTrail2 _bp_trail_2)
      (CallFunction|Move))
    (:3
      ;[0 0.4337 1] Style3
      (Default|Initialize _bp_trail_3 self)
      (Default|CallTrail3 _bp_trail_3)
      (CallFunction|Move))
    (:4
      ;[0 0.4337 1] Style4
      (Default|Initialize _bp_trail_4 self)
      (Default|CallTrail4 _bp_trail_4)
      (CallFunction|Move))
    (:5
      ;[0 0.4337 1] Style5
      (Default|Initialize _bp_trail_5 self)
      (Default|CallTrail5 _bp_trail_5)
      (CallFunction|Move))
    (:6
      ;[0 0.4337 1] Style6
      (Default|Initialize _bp_trail_6 self)
      (Default|CallTrail6 _bp_trail_6)
      (CallFunction|Move))
    (:7
      ;[0 0.4337 1] Style7
      (Default|Initialize _bp_trail_7 self)
      (Default|CallTrail7 _bp_trail_7)
      (CallFunction|Move))
    (:8
      ;[0 0.4337 1] Style8
      (Default|Initialize _bp_trail_8 self)
      (Default|CallTrail8 _bp_trail_8)
      (CallFunction|Move))
    (:9
      ;[0 0.4337 1] Style9
      (Default|Initialize _bp_trail_9 self)
      (Default|CallTrail9 _bp_trail_9)
      (CallFunction|Move))
    (:10
      ;[0 0.4337 1] Style10
      (Default|Initialize _bp_trail_10 self)
      (Default|CallTrail10 _bp_trail_10)
      (CallFunction|Move))))

(fn ConstructionScript)