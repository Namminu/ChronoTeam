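; BP_Trail_4 applies a Niagara trail effect to a character's skeletal mesh.
; Call_Trail_4 spawns P_Trail_2 attached to the mesh, then after a brief delay binds that mesh to the system's skeletal mesh user variable.
; A non-looping timer then triggers Tick, which feeds the character's movement speed into the effect's "V" float parameter.
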(event Custom|Call_Trail_4
  (bind _character (Variables|Default|GetCharacter))
  (bind _mesh (Variables|/Script/Engine.Character|GetMesh _character))
  ;[0 0.03735 1] Apply the effect to the get skeletal mesh
  (bind _returnvalue (Niagara|SpawnSystemAttached "/Game/All_Asset/NiagaraCharacterTrail/Niagara/P_Trail_2.P_Trail_2" _mesh "None" "0, 0, 0" "0, 0, 0" "KeepRelativeOffset" false))
  (Utilities|FlowControl|Delay 0.02)
  (Class|NiagaraFunctionLibrary|OverrideSystemUserVariableSkeletalMeshComponent _returnvalue "Skeletal Mesh" _mesh)
  (Utilities|Time|SetTimerbyEvent (delegate Custom|Tick) 0.1))

(event Custom|Tick
  ;[0 0.03735 1] Apply the effect to the get skeletal mesh
  (Niagara|SetNiagaraVariable(Float) (stale Custom|Call_Trail_4 _returnvalue) "V" (Math|Vector|VectorLength (Variables|/Script/Engine.MovementComponent|GetVelocity (Variables|/Script/Engine.Character|GetCharacterMovement (Variables|Default|GetCharacter))))))