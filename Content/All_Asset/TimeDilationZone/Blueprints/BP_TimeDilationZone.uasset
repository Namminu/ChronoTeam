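; Time dilation zone built from instanced mesh volumes that changes time for overlapping actors, per actor or globally.
; Begin overlaps pass tag/class filters; ActivationType sets whether crossings start, end or toggle the effect.
; Per-actor mode fades CustomTimeDilation on Tick through in/out timer maps.
; Transitions fire particles, sounds and BPI_TimeDilation messages to actor and controllers; SaveChanges stores instance transforms in a GUID-named SaveGame.
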(event OnComponentBeginOverlap(InstancedStaticMesh)
  (params (OverlappedComponent :type Primitive%20Component%20Object%20Reference) (OtherActor :type Actor%20Object%20Reference) (OtherComp :type Primitive%20Component%20Object%20Reference) (OtherBodyIndex :type Integer) (bFromSweep :type Boolean) (SweepResult :type Hit%20Result%20Structure%20%28by%20ref%29))
  (bind _passedfilter_ (CallFunction|CheckTagorClass OtherActor))
  (if _passedfilter_
    (switch Utilities|FlowControl|Switch|SwitchonActivationType_Enum (Variables|TimeZone|GetActivationType)
      (:NewEnumerator0
        (CallFunction|StartOverlapEvent OtherActor))
      (:NewEnumerator1
        (if (Utilities|Map|Contains (Variables|Base|GetActorInArray) OtherActor)
          (CallFunction|EndOverlapEvent OtherActor)
          (else
            (CallFunction|StartOverlapEvent OtherActor)))))))

(event OnComponentEndOverlap(InstancedStaticMesh)
  (params (OverlappedComponent :type Primitive%20Component%20Object%20Reference) (OtherActor :type Actor%20Object%20Reference) (OtherComp :type Primitive%20Component%20Object%20Reference) (OtherBodyIndex :type Integer))
  (switch Utilities|FlowControl|Switch|SwitchonActivationType_Enum (Variables|TimeZone|GetActivationType)
    (:NewEnumerator0
      (CallFunction|EndOverlapEvent OtherActor))
    (:NewEnumerator2
      (if (Utilities|Map|Contains (Variables|Base|GetActorInArray) OtherActor)
        (CallFunction|EndOverlapEvent OtherActor)
        (else
          (CallFunction|StartOverlapEvent OtherActor))))))

(event EventTick
  (params (DeltaSeconds :type Float%20%28single-precision%29))
  (Variables|Base|SetDeltaSeconds DeltaSeconds)
  (CallFunction|FadeinTickEvaluation)
  (CallFunction|FadeOutTickEvaluation))

(fn ConstructionScript
  (Components|StaticMesh|SetStaticMesh (Variables|Default|GetInstancedStaticMesh) (Variables|TimeZone|GetShapeMesh))
  (Components|InstancedStaticMesh|AddInstances (Variables|Default|GetInstancedStaticMesh) (Variables|TimeZone|GetInstances) false false))

(fn SaveChanges
  (bind _instancedstaticmesh (Variables|Default|GetInstancedStaticMesh))
  (bind _returnvalue (SaveGame|DoesSaveGameExist (TimeZone|SlotName)))
  (if _returnvalue
    (bind _returnvalue_2 (SaveGame|LoadGamefromSlot (TimeZone|SlotName)))
    (Variables|Base|SetTDZoneDataSave_Ref (.AsTDZone%20Data%20Save%20Game (Utilities|Casting|CastToTDZoneData_SaveGame _returnvalue_2)))
    (else
      (bind _returnvalue_3 (SaveGame|CreateSaveGameObject "/Game/All_Asset/TimeDilationZone/Data/TDZoneData_SaveGame.TDZoneData_SaveGame_C"))
      (Variables|Base|SetTDZoneDataSave_Ref _returnvalue_3)))
  (if (== (Components|InstancedStaticMesh|GetInstanceCount (Variables|Default|GetInstancedStaticMesh)) (Utilities|Array|Length (Variables|TimeZone|GetInstances)))
    (for _index (range 0 (- (Components|InstancedStaticMesh|GetInstanceCount _instancedstaticmesh) 1))
      (Utilities|Array|SetArrayElem (Variables|/Game/All_Asset/TimeDilationZone/Data/TDZoneData_SaveGame.TDZoneData_SaveGame_C|GetInstances (Variables|Base|GetTDZoneDataSave_Ref)) _index (.OutInstanceTransform (Components|InstancedStaticMesh|GetInstanceTransform _instancedstaticmesh _index false)) true))
    (else
      (Variables|/Game/All_Asset/TimeDilationZone/Data/TDZoneData_SaveGame.TDZoneData_SaveGame_C|SetInstances (Variables|Base|GetTDZoneDataSave_Ref) (Variables|TimeZone|GetInstances))
      (SaveGame|SaveGametoSlot (Variables|Base|GetTDZoneDataSave_Ref) (TimeZone|SlotName))))
  (SaveGame|SaveGametoSlot (Variables|Base|GetTDZoneDataSave_Ref) (TimeZone|SlotName))
  (CallFunction|LoadSaveGameInstances))

(fn EndOverlapEvent
  (params (ActorRef :type Actor%20Object%20Reference))
  (if (Variables|TimeZone|Time|GetTimeDilationPerActor?)
    (CallFunction|ActorintoActorOutArrayTransfer ActorRef)
    (else
      (Utilities|Time|SetGlobalTimeDilation (Variables|TimeZone|Time|GetTimeDilationOut))))
  (CallFunction|EndOverlapTrigger ActorRef))

(fn StartOverlapEvent
  (params (ActorRef :type Actor%20Object%20Reference))
  (bind _customtimedilation (Variables|/Script/Engine.Actor|GetCustomTimeDilation ActorRef))
  (if (Variables|TimeZone|Time|GetTimeDilationPerActor?)
    (Utilities|Map|Add (Variables|Base|GetActorInArray) ActorRef (Math|Float|MapRangeUnclamped _customtimedilation _customtimedilation (Variables|TimeZone|Time|GetTimeDilationIn) (Variables|TimeZone|Time|GetTimeDilationFadeIn) 0.0))
    (else
      (Utilities|Time|SetGlobalTimeDilation (Variables|TimeZone|Time|GetTimeDilationIn))))
  (CallFunction|StartOverlapTrigger ActorRef))

(fn FadeinTickEvaluation
  (bind _actorinarray (Variables|Base|GetActorInArray))
  (bind _keys (Utilities|Map|Keys _actorinarray))
  (bind _values (Utilities|Map|Values _actorinarray))
  (for (_array_element _array_index) _keys
    (if (not (== (Utilities|Array|Get(acopy) _values _array_index) 0.0))
      (Utilities|Map|Add (Variables|Base|GetActorInArray) _array_element (select (Math|Float|NearlyEqual(Float) (- (Utilities|Array|Get(acopy) _values _array_index) (Variables|Base|GetDeltaSeconds)) 0.0 0.02) (Math|Float|MakeLiteralFloat 0.0) (- (Utilities|Array|Get(acopy) _values _array_index) (Variables|Base|GetDeltaSeconds))))
      (Variables|/Script/Engine.Actor|SetCustomTimeDilation _array_element (Math|Float|MapRangeClamped (select (Math|Float|NearlyEqual(Float) (- (Utilities|Array|Get(acopy) _values _array_index) (Variables|Base|GetDeltaSeconds)) 0.0 0.02) (Math|Float|MakeLiteralFloat 0.0) (- (Utilities|Array|Get(acopy) _values _array_index) (Variables|Base|GetDeltaSeconds))) 0.0 (Variables|TimeZone|Time|GetTimeDilationFadeIn) (Variables|TimeZone|Time|GetTimeDilationIn) (Variables|/Script/Engine.Actor|GetCustomTimeDilation _array_element))))))

(fn FadeOutTickEvaluation
  (bind _actoroutarray (Variables|Base|GetActorOutArray))
  (bind _keys (Utilities|Map|Keys _actoroutarray))
  (bind _values (Utilities|Map|Values _actoroutarray))
  (for (_array_element _array_index) _keys
    (if (== (Utilities|Array|Get(acopy) _values _array_index) 0.0)
      (Utilities|Map|Remove (Variables|Base|GetActorOutArray) _array_element)
      (else
        (Utilities|Map|Add (Variables|Base|GetActorOutArray) _array_element (select (Math|Float|NearlyEqual(Float) (- (Utilities|Array|Get(acopy) _values _array_index) (Variables|Base|GetDeltaSeconds)) 0.0 0.01) (Math|Float|MakeLiteralFloat 0.0) (- (Utilities|Array|Get(acopy) _values _array_index) (Variables|Base|GetDeltaSeconds))))
        (Variables|/Script/Engine.Actor|SetCustomTimeDilation _array_element (Math|Float|MapRangeClamped (select (Math|Float|NearlyEqual(Float) (- (Utilities|Array|Get(acopy) _values _array_index) (Variables|Base|GetDeltaSeconds)) 0.0 0.01) (Math|Float|MakeLiteralFloat 0.0) (- (Utilities|Array|Get(acopy) _values _array_index) (Variables|Base|GetDeltaSeconds))) 0.0 (Variables|TimeZone|Time|GetTimeDilationFadeOut) (Variables|TimeZone|Time|GetTimeDilationOut) (Variables|/Script/Engine.Actor|GetCustomTimeDilation _array_element)))))))

(fn ActorintoActorOutArrayTransfer
  (params (ActorRef :type Actor%20Object%20Reference))
  (if (Utilities|Map|Contains (Variables|Base|GetActorInArray) ActorRef)
    (Utilities|Map|Add (Variables|Base|GetActorOutArray) ActorRef (Math|Float|MapRangeClamped (.Value (Utilities|Map|Find (Variables|Base|GetActorInArray) ActorRef)) 0.0 (Variables|TimeZone|Time|GetTimeDilationFadeIn) (Variables|TimeZone|Time|GetTimeDilationFadeOut) 0.0))
    (Utilities|Map|Remove (Variables|Base|GetActorInArray) ActorRef)))

(fn StartOverlapTrigger
  (params (ActorRef :type Actor%20Object%20Reference))
  (bind _returnvalue (Game|GetPlayerController 0))
  (bind _soundin (Variables|TimeZone|Sound|GetSoundIn))
  (bind _returnvalue_2 (AI|GetAIController ActorRef))
  (bind _returnvalue_3 (Transformation|GetActorLocation ActorRef))
  (Utilities|FlowControl|Sequence
    (:then_0
      (Utilities|IsValid (Variables|TimeZone|Particles|GetParticleIn)
        (:Is%20Valid
          (if (Variables|TimeZone|Particles|GetDestroyOnExit?)
            (bind _returnvalue_4 (Niagara|SpawnSystemAttached (Variables|TimeZone|Particles|GetParticleIn) (Variables|/Script/Engine.Actor|GetRootComponent ActorRef) "None" _returnvalue_3 "0, 0, 0" "SnapToTargetIncludingScale" false))
            (Variables|Default|SetParticleIn_Ref _returnvalue_4)
            (Transformation|SetWorldLocation _returnvalue_4 _returnvalue_3 false false)
            (else
              (Niagara|SpawnSystematLocation (Variables|TimeZone|Particles|GetParticleIn) (Transformation|GetActorLocation ActorRef) "0, 0, 0" "1.000000,1.000000,1.000000" true true "None" false))))))
    (:then_1
      (Utilities|IsValid _soundin
        (:Is%20Valid
          (Audio|PlaySoundatLocation _soundin (Transformation|GetActorLocation ActorRef) "0, 0, 0" 1.0 1.0 0.0 0 0 0 0))))
    (:then_2
      (if (Utilities|DoesObjectImplementInterface _returnvalue "/Game/All_Asset/TimeDilationZone/Blueprints/BPI_TimeDilation.BPI_TimeDilation_C")
        (Class|BPITimeDilation|StartTimeDilation(Message) _returnvalue self (Variables|TimeZone|Time|GetTimeDilationIn) (Variables|TimeZone|Time|GetTimeDilationOut))))
    (:then_3
      (if (Utilities|DoesObjectImplementInterface ActorRef "/Game/All_Asset/TimeDilationZone/Blueprints/BPI_TimeDilation.BPI_TimeDilation_C")
        (Class|BPITimeDilation|StartTimeDilation(Message) ActorRef self (Variables|TimeZone|Time|GetTimeDilationIn) (Variables|TimeZone|Time|GetTimeDilationOut))))
    (:then_4
      (if (Utilities|DoesObjectImplementInterface _returnvalue_2 "/Game/All_Asset/TimeDilationZone/Blueprints/BPI_TimeDilation.BPI_TimeDilation_C")
        (Class|BPITimeDilation|StartTimeDilation(Message) _returnvalue_2 self (Variables|TimeZone|Time|GetTimeDilationIn) (Variables|TimeZone|Time|GetTimeDilationOut))))))

(fn EndOverlapTrigger
  (params (ActorRef :type Actor%20Object%20Reference))
  (bind _returnvalue (Game|GetPlayerController 0))
  (bind _soundout (Variables|TimeZone|Sound|GetSoundOut))
  (bind _particlein_ref (Variables|Default|GetParticleIn_Ref))
  (bind _returnvalue_2 (AI|GetAIController ActorRef))
  (bind _returnvalue_3 (Transformation|GetActorLocation ActorRef))
  (Utilities|FlowControl|Sequence
    (:then_0
      (Utilities|IsValid (Variables|TimeZone|Particles|GetParticleOut)
        (:Is%20Valid
          (Niagara|SpawnSystematLocation (Variables|TimeZone|Particles|GetParticleOut) _returnvalue_3 "0, 0, 0" "1.000000,1.000000,1.000000" true true "None" false))))
    (:then_1
      (Utilities|IsValid _soundout
        (:Is%20Valid
          (Audio|PlaySoundatLocation _soundout _returnvalue_3 "0, 0, 0" 1.0 1.0 0.0 0 0 0 0))))
    (:then_2
      (if (Utilities|DoesObjectImplementInterface _returnvalue "/Game/All_Asset/TimeDilationZone/Blueprints/BPI_TimeDilation.BPI_TimeDilation_C")
        (Class|BPITimeDilation|EndTimeDilation(Message) _returnvalue self (Variables|TimeZone|Time|GetTimeDilationIn) (Variables|TimeZone|Time|GetTimeDilationOut))))
    (:then_3
      (if (Utilities|DoesObjectImplementInterface ActorRef "/Game/All_Asset/TimeDilationZone/Blueprints/BPI_TimeDilation.BPI_TimeDilation_C")
        (Class|BPITimeDilation|EndTimeDilation(Message) ActorRef self (Variables|TimeZone|Time|GetTimeDilationIn) (Variables|TimeZone|Time|GetTimeDilationOut))))
    (:then_4
      (if (Utilities|DoesObjectImplementInterface _returnvalue_2 "/Game/All_Asset/TimeDilationZone/Blueprints/BPI_TimeDilation.BPI_TimeDilation_C")
        (Class|BPITimeDilation|EndTimeDilation(Message) _returnvalue_2 self (Variables|TimeZone|Time|GetTimeDilationIn) (Variables|TimeZone|Time|GetTimeDilationOut))))
    (:then_5
      (if (Variables|TimeZone|Particles|GetDestroyOnExit?)
        (Utilities|IsValid _particlein_ref
          (:Is%20Valid
            (Components|DestroyComponent _particlein_ref)))))))

(fn SlotName
  (return (Utilities|String|Append "TDZoneData" (Guid|ToString(Guid) (Variables|Default|GetActorGuid)))))

(fn LoadSaveGameInstances
  (bind _returnvalue (SaveGame|LoadGamefromSlot (TimeZone|SlotName)))
  (bind _astdzone_data_save_game (Utilities|Casting|CastToTDZoneData_SaveGame _returnvalue))
  (Variables|Base|SetTDZoneDataSave_Ref _astdzone_data_save_game)
  (Variables|TimeZone|SetInstances (Variables|/Game/All_Asset/TimeDilationZone/Data/TDZoneData_SaveGame.TDZoneData_SaveGame_C|GetInstances (Variables|Base|GetTDZoneDataSave_Ref))))

(fn CheckTagorClass
  (params (ActorRef :type Actor%20Object%20Reference))
  (if (and (== (Utilities|Array|Length (Variables|TimeZone|Filters|GetTagFilters)) 0) (== (Utilities|Array|Length (Variables|TimeZone|Filters|GetClassFilters)) 0))
    (return true)
    (else
      (for _array_element (Variables|TimeZone|Filters|GetTagFilters)
        (if (Utilities|Array|ContainsItem (Variables|/Script/Engine.Actor|GetTags ActorRef) _array_element)
          (return true)))
      (for _array_element_2 (Variables|TimeZone|Filters|GetClassFilters)
        (if (== _array_element_2 (Utilities|GetClass ActorRef))
          (return true)))
      (return false))))