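; Shield hit-effect controller that displays one impact on a copy of the shield's static mesh.
; OnImpact copies the passed mesh, creates a dynamic instance of the hit material and applies it to slot 0.
; Two timelines share one update that feeds the material its Phase, Opacity and HitPosition, the latter being the mesh's world location plus the impact offset.
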(event EventOnImpact
  (params (Location :type Vector :default "0, 0, 0") (Mesh :type Static%20Mesh%20Component%20Object%20Reference) (HitMaterial :type Material%20Interface%20Object%20Reference))
  (Utilities|IsValid Mesh
    (:Is%20Valid
      (Components|StaticMesh|SetStaticMesh (Variables|/Script/Engine.StaticMeshComponent|GetStaticMesh Mesh))
      (bind _returnvalue (Rendering|Material|CreateDynamicMaterialInstance 0 HitMaterial "None" :!class /Script/Engine.PrimitiveComponent))
      (bind _output_get (Variables|Default|SetDynamicMaterial _returnvalue))
      (for _index (range 0 0)
        (Rendering|Material|SetMaterial _index _output_get)
        (Rendering|Material|SetMaterial (Variables|Default|GetStaticMesh) _index _output_get))
      (Utilities|FlowControl|Sequence
        (:then_0
          (bind _time (Timeline|Timeline PlayFromStart)
            (:Update
              _)))
        (:then_1
          (bind _newtrack_0 (Timeline|ShieldOpacity Play)
            (:Update
              _))))
      (Rendering|Material|SetVectorParameterValue (Variables|Default|GetDynamicMaterial) "HitPosition" (Math|Conversions|ToLinearColor(Vector) (+ (Transformation|GetWorldLocation Mesh) Location)) :!class /Script/Engine.MaterialInstanceDynamic)
      (Rendering|Material|SetScalarParameterValue (Variables|Default|GetDynamicMaterial) "Phase" _time :!class /Script/Engine.MaterialInstanceDynamic)
      (Rendering|Material|SetScalarParameterValue (Variables|Default|GetDynamicMaterial) "Opacity" _newtrack_0 :!class /Script/Engine.MaterialInstanceDynamic))))

(fn ConstructionScript)