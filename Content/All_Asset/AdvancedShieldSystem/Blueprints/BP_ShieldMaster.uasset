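; Master shield actor: a configurable sphere that animates in on BeginPlay with a decal fade and Niagara ground and orb effects set up in construction.
; Hits spawn rate-limited child impact actors, passing hit offset, sphere and material.
; Overlaps drive post-process through a curve timeline and MPC_ShieldsPP, weighted by whether the player is inside.
; Optional Time Dilation mode slows overlapping actors tagged "SlowMo" until they exit.
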(event OnComponentBeginOverlap(Sphere)
  (params (OverlappedComponent :type Primitive%20Component%20Object%20Reference) (OtherActor :type Actor%20Object%20Reference) (OtherComp :type Primitive%20Component%20Object%20Reference) (OtherBodyIndex :type Integer) (bFromSweep :type Boolean) (SweepResult :type Hit%20Result%20Structure%20%28by%20ref%29))
  (bind _postprocess (Variables|Default|GetPostProcess))
  ;[0 0 0] OverlapEvent
  (Utilities|FlowControl|Sequence
    (:then_0
      ;[0 0 0] EnterPP
      (Variables|/Script/Engine.PostProcessComponent|SetSettings _postprocess (Variables|PostProcess|GetPP_Settings))
      (Components|Timeline|SetPlayRate (Variables|Default|GetPPTimeline) (Variables|PostProcess|GetPostProcessSpeed))
      (bind _newtrack_0 (Timeline|PPTimeline PlayFromStart)
        (:Update
          (Rendering|Material|SetScalarParameterValue "/Game/All_Asset/AdvancedShieldSystem/Materials/CollectionParmeters/MPC_ShieldsPP.MPC_ShieldsPP" "Intensity" (Math|Curves|GetFloatValue (Variables|PostProcess|GetPostProcessCurve) _newtrack_0) :!class /Script/Engine.KismetMaterialLibrary)
          (Rendering|Material|SetVectorParameterValue "/Game/All_Asset/AdvancedShieldSystem/Materials/CollectionParmeters/MPC_ShieldsPP.MPC_ShieldsPP" "Color" (Math|Conversions|ToLinearColor(Color) (Variables|PostProcess|GetPP_Color)) :!class /Script/Engine.KismetMaterialLibrary)
          (Variables|/Script/Engine.PostProcessComponent|SetBlendWeight _postprocess (select (Collision|IsOverlappingActor (Variables|Default|GetSphere) (Game|Player|GetPlayerPawn 0) :!class /Script/Engine.PrimitiveComponent) 1.0 0.0)))))
    (:then_1
      ;[0 0 0] SlowMotion / Needs Actor Tag "SlowMo"
      (if (Variables|Default|GetIsSlowMo?)
        (if (Actor|ActorHasTag OtherActor "SlowMo")
          (Variables|/Script/Engine.Actor|SetCustomTimeDilation OtherActor (Variables|Base|GetTimeDilation)))))))

(event OnComponentEndOverlap(Sphere)
  (params (OverlappedComponent :type Primitive%20Component%20Object%20Reference) (OtherActor :type Actor%20Object%20Reference) (OtherComp :type Primitive%20Component%20Object%20Reference) (OtherBodyIndex :type Integer))
  ;[0 0 0] OverlapEvent
  (Utilities|FlowControl|Sequence
    (:then_0
      ;[0 0 0] EnterPP
      (Components|Timeline|SetPlayRate (Variables|Default|GetPPTimeline) (Variables|PostProcess|GetPostProcessSpeed))
      (bind _newtrack_0 (Timeline|PPTimeline PlayFromStart)
        (:Update
          (Rendering|Material|SetScalarParameterValue "/Game/All_Asset/AdvancedShieldSystem/Materials/CollectionParmeters/MPC_ShieldsPP.MPC_ShieldsPP" "Intensity" (Math|Curves|GetFloatValue (Variables|PostProcess|GetPostProcessCurve) _newtrack_0) :!class /Script/Engine.KismetMaterialLibrary)
          (Rendering|Material|SetVectorParameterValue "/Game/All_Asset/AdvancedShieldSystem/Materials/CollectionParmeters/MPC_ShieldsPP.MPC_ShieldsPP" "Color" (Math|Conversions|ToLinearColor(Color) (Variables|PostProcess|GetPP_Color)) :!class /Script/Engine.KismetMaterialLibrary)
          (Variables|/Script/Engine.PostProcessComponent|SetBlendWeight (Variables|Default|GetPostProcess) (select (Collision|IsOverlappingActor (Variables|Default|GetSphere) (Game|Player|GetPlayerPawn 0) :!class /Script/Engine.PrimitiveComponent) 1.0 0.0)))))
    (:then_1
      ;[0 0 0] SlowMotion / Needs Actor Tag "SlowMo"
      (Variables|/Script/Engine.Actor|SetCustomTimeDilation OtherActor 1.0))
    (:then_2)))

(event OnComponentHit(Sphere)
  (params (HitComponent :type Primitive%20Component%20Object%20Reference) (OtherActor :type Actor%20Object%20Reference) (OtherComp :type Primitive%20Component%20Object%20Reference) (NormalImpulse :type Vector :default "0, 0, 0") (Hit :type Hit%20Result%20Structure%20%28by%20ref%29))
  (bind _sphere (Variables|Default|GetSphere))
  ;[0 0 0] Hit
  (if (not (Variables|Hit|GetSpawnDelayActive))
    (Variables|Hit|SetSpawnDelayActive true)
    (bind _returnvalue (AddComponent|AddChildActorComponent false (Math|Transform|MakeTransform (Variables|Hit|GetLocationOffset) "0, 0, 0" (* "1.000000,1.000000,1.000000" (Variables|Base|GetShieldSize)))))
    (Class|BPHitInterface|OnImpact(Message) (Variables|/Script/Engine.ChildActorComponent|GetChildActor _returnvalue) (- (.location Hit) (Transformation|GetWorldLocation _sphere)) _sphere (Variables|Base|GetHit%20Material))
    (Utilities|FlowControl|Delay (Variables|Hit|GetSpawnedActorReduction))
    (Variables|Hit|SetSpawnDelayActive false)))

(event EventActorOnInputTouchLeave
  (params (FingerIndex :type ETouchIndex%20Enum :default "Touch1")))

(event EventBeginPlay
  ;[0 0 0] DealFade
  (Rendering|Components|Decal|SetFadeIn (Variables|Default|GetDecal) (Variables|Decal|GetDecalFadeDelay) (Variables|Decal|GetDecalFadeDuration))
  (Components|Timeline|SetPlayRate (Variables|Default|GetCirveTick) (Variables|Base|GetAppearSpeed))
  (bind _newtrack_0 (Timeline|CirveTick Play)
    (:Update
      (Rendering|Material|SetScalarParameterValue (Variables|Default|GetInstanceMaterial) "Appear" (Math|Curves|GetFloatValue (Variables|Base|GetAppearCurve) _newtrack_0) :!class /Script/Engine.MaterialInstanceDynamic))))

(fn ConstructionScript
  (bind _sphere (Variables|Default|GetSphere))
  (bind _groundvfx (Variables|Default|GetGroundVFX))
  (bind _orbvfx (Variables|Default|GetOrbVFX))
  (Utilities|FlowControl|Sequence
    (:then_0
      (Rendering|Material|SetMaterial _sphere 0 (Variables|Base|GetShieldMaterial))
      (Transformation|SetWorldScale3D _sphere (Math|Conversions|ToVector(Float) (Variables|Base|GetShieldSize)))
      (bind _returnvalue (Rendering|Material|CreateDynamicMaterialInstance _sphere 0 0 "None" :!class /Script/Engine.PrimitiveComponent))
      (Variables|Default|SetInstanceMaterial _returnvalue))
    (:then_1
      (Rendering|Components|Decal|SetDecalMaterial (Variables|Default|GetDecal) (Variables|Decal|GetDecalMaterial)))
    (:then_2
      (switch Utilities|FlowControl|Switch|SwitchonEnum_ShieldFunction (Variables|Base|GetFunctionality)
        (:NewEnumerator2
          (Variables|Default|SetIsSlowMo? false))
        (:NewEnumerator0
          (Variables|Default|SetIsSlowMo? true))))
    (:then_3
      ;[0 0 0 1 20] GroundVFX
      (Effects|Components|ParticleSystem|SetColorParameter _groundvfx "User.Color" (Variables|GroundVFX|GetGroundVFXColor))
      (Class|NiagaraComponent|SetAsset _groundvfx (Variables|GroundVFX|GetGroundEffect) true))
    (:then_4
      (Effects|Components|ParticleSystem|SetColorParameter _orbvfx "User.Color01" (Variables|Orb|GetOrbColor_01))
      (Effects|Components|ParticleSystem|SetColorParameter _orbvfx "User.Color02" (Variables|Orb|GetOrbColor_02))
      (Class|NiagaraComponent|SetAsset _orbvfx (Variables|Orb|GetOrbParticle) true))))