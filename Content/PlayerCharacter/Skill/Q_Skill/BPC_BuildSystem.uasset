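; Player component for the Q skill, which places up to three shield zones at the mouse cursor.
; Q enters slow-motion build mode with a cursor-following preview; attack spawns the zone and plays a montage.
; A looping timer applies stamina changes while zones exist; empty stamina outside build mode destroys them all.
; Pressing Q at the limit also clears zones, as does right-click during build mode, which cancels the preview too.
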(event Custom|Preview%20Loop
  (bind _returnvalue (Game|GetPlayerController 0))
  (bind _hitresult (Game|Player|GetHitResultUnderCursorbyChannel _returnvalue "TraceTypeQuery1" true))
  (if (.bblockinghit _hitresult)
    (Utilities|FlowControl|Sequence
      (:then_0
        (Utilities|FlowControl|DoOnce false
          (:Completed
            (bind _returnvalue_2 (Game|SpawnActorfromClass "/Game/PlayerCharacter/Skill/Q_Skill/BP_QSkillBuild.BP_QSkillBuild_C" (Variables|Default|GetBuild%20Preview%20Transform) "AlwaysSpawn" "MultiplyWithRoot" 0 0))
            (bind _output_get (Variables|Default|SetBuild%20BP _returnvalue_2))
            (Transformation|SetWorldScale3D (Variables|/Script/Engine.Actor|GetRootComponent _output_get) (Math|Conversions|ToVector(Float) (Variables|/Game/ThirdPerson/Blueprints/BP_ThirdPersonCharacter.BP_ThirdPersonCharacter_C|GetShieldSize (Variables|Default|GetPlayer%20BP))))
            (Collision|SetCollisionEnabled (Variables|/Game/PlayerCharacter/Skill/Q_Skill/BP_QSkillBuild.BP_QSkillBuild_C|GetSphere _output_get) "NoCollision"))))
      (:then_1
        (bind _build_bp (Variables|Default|GetBuild%20BP)
          (:then
            (bind _output_get_2 (Variables|Default|SetBuild%20Preview%20Transform (Math|Transform|MakeTransform (.location _hitresult) "0, 0, 0" (Transformation|GetWorldScale (Variables|/Script/Engine.Actor|GetRootComponent (Variables|Default|GetBuild%20BP))))))
            (Transformation|SetWorldTransform (Variables|/Script/Engine.Actor|GetRootComponent _build_bp) _output_get_2 false false))
          (:else))))))

(event Custom|Reset%20Build%20Mode
  (Utilities|FlowControl|DoOnce false) ; enters at Reset
)

(event Custom|Stop%20Build%20Mode
  ;[1 1 1] Q스킬 스킬 범위 삭제
  (Variables|/Script/TeamChrono.TeamChronoCharacter|SetIsQSkillBuilding (Variables|Default|GetPlayer%20BP) (stale Input|EnhancedActionEvents|EnhancedInputActionIA_QSkill _output_get_3))
  (CallFunction|ResetBuildMode))

(event Custom|QskillingEnd
  ;[1 1 1] Q스킬 공간 삭제
  (if (Variables|Default|GetIsQskillDoing)
    (for _array_element (Variables|Default|GetQSkill%20BP)
      (Actor|DestroyActor _array_element))
    (Variables|Default|SetIsQskillDoing false)
    (Utilities|Time|ClearandInvalidateTimerbyHandle (Variables|Default|GetQskillingTimer))
    (Utilities|Array|Clear (Variables|Default|GetQSkill%20BP))
    (Default|QSkillEnd (Variables|/Game/ThirdPerson/Blueprints/BP_ThirdPersonCharacter.BP_ThirdPersonCharacter_C|GetWB%20QSkill%20Count%20UI (Variables|Default|GetPlayer%20BP)))))

(event Input|EnhancedActionEvents|EnhancedInputActionIA_QSkill
  (params (ActionValue :type Boolean) (ElapsedSeconds :type Float%20%28double-precision%29) (TriggeredSeconds :type Float%20%28double-precision%29) (InputAction :type Input%20Action%20Object%20Reference :default "/Game/ThirdPerson/Input/Actions/IA_QSkill.IA_QSkill"))
  (bind _player_bp (Variables|Default|GetPlayer%20BP))
  (bind _player_bp_2 (Variables|Default|GetPlayer%20BP))
  (bind _player_bp_3 (Variables|Default|GetPlayer%20BP))
  (:Started
    (if (and (not (Variables|/Script/TeamChrono.TeamChronoCharacter|GetIsClimbing (Variables|Default|GetPlayer%20BP))) (not (Variables|Default|GetIsMontaging)))
      (if (>= (Utilities|Array|Length (Variables|Default|GetQSkill%20BP)) 3)
        ;[1 1 1] Q스킬 공간 삭제
        (if (Variables|Default|GetIsQskillDoing)
          (for _array_element (Variables|Default|GetQSkill%20BP)
            (Actor|DestroyActor _array_element))
          (Variables|Default|SetIsQskillDoing false)
          (Utilities|Time|ClearandInvalidateTimerbyHandle (Variables|Default|GetQskillingTimer))
          (Utilities|Array|Clear (Variables|Default|GetQSkill%20BP))
          (Default|QSkillEnd (Variables|/Game/ThirdPerson/Blueprints/BP_ThirdPersonCharacter.BP_ThirdPersonCharacter_C|GetWB%20QSkill%20Count%20UI (Variables|Default|GetPlayer%20BP))))
        (elif (not (Variables|Default|GetinBuildMode))
          (if (> (Variables|/Script/TeamChrono.TeamChronoCharacter|GetpcStamina _player_bp) (Variables|/Script/TeamChrono.TeamChronoCharacter|GetQSkillStamina _player_bp))
            ;[1 1 1] Q스킬 스킬 범위 생성
            (if (not (Variables|/Script/TeamChrono.TeamChronoCharacter|Getm_bIsDodging (Variables|Default|GetPlayer%20BP)))
              (bind _output_get (Variables|Default|SetinBuildMode true))
              (bind _output_get_2 (Variables|/Script/TeamChrono.TeamChronoCharacter|SetIsQSkillBuilding _player_bp_2 _output_get))
              (Default|BlendScreen _player_bp_2 _output_get_2)
              (Class|TeamChronoCharacter|StaminaVariation _player_bp_2 (Variables|/Script/TeamChrono.TeamChronoCharacter|GetQSkillStamina _player_bp_2))
              (Class|TeamChronoCharacter|IsNotLongAttacking _player_bp_2)
              (Utilities|Time|SetGlobalTimeDilation 0.2)))
          (else
            ;[1 1 1] Q스킬 스킬 범위 삭제
            (bind _build_bp (Variables|Default|GetBuild%20BP)
              (:then
                (Actor|DestroyActor _build_bp)
                (Utilities|Time|SetGlobalTimeDilation 1.0)
                (Default|BlendScreen _player_bp_3 false)
                (Class|TeamChronoCharacter|StaminaVariation _player_bp_3 (* (Variables|/Script/TeamChrono.TeamChronoCharacter|GetQSkillEndStamina _player_bp_3) -1.0))
                (bind _output_get_3 (Variables|Default|SetinBuildMode false))
                (Variables|/Script/TeamChrono.TeamChronoCharacter|SetIsQSkillBuilding (Variables|Default|GetPlayer%20BP) _output_get_3)
                (CallFunction|ResetBuildMode))
              (:else))))))))

(event Input|EnhancedActionEvents|EnhancedInputActionIA_Attack
  (params (ActionValue :type Boolean) (ElapsedSeconds :type Float%20%28double-precision%29) (TriggeredSeconds :type Float%20%28double-precision%29) (InputAction :type Input%20Action%20Object%20Reference :default "/Game/ThirdPerson/Input/Actions/IA_Attack.IA_Attack"))
  (bind _returnvalue (Game|GetPlayerController 0))
  (bind _player_bp (Variables|Default|GetPlayer%20BP))
  (bind _qskill_bp (Variables|Default|GetQSkill%20BP))
  (bind _player_bp_2 (Variables|Default|GetPlayer%20BP))
  (bind _returnvalue_2 (Transformation|GetActorLocation _player_bp))
  (bind _hitresult (Game|Player|GetHitResultUnderCursorbyChannel _returnvalue "TraceTypeQuery1" true))
  (bind _location (Collision|BreakHitResult _hitresult))
  (bind _returnvalue_3 (Math|Rotator|FindLookatRotation _returnvalue_2 _location))
  (:Started
    ;[1 1 1] 공간 생성
    (if (Variables|Default|GetinBuildMode)
      (bind _returnvalue_4 (Game|SpawnActorfromClass "/Game/PlayerCharacter/Skill/Q_Skill/BP_ShieldMaster_QSkill.BP_ShieldMaster_QSkill_C" (Variables|Default|GetBuild%20Preview%20Transform) "AlwaysSpawn" "MultiplyWithRoot" 0 0))
      (bind _returnvalue_5 (Utilities|Array|Add _qskill_bp _returnvalue_4))
      (Utilities|Time|SetGlobalTimeDilation 1.0)
      (Default|SizeChange (Utilities|Array|Get(acopy) _qskill_bp _returnvalue_5) (Variables|/Game/ThirdPerson/Blueprints/BP_ThirdPersonCharacter.BP_ThirdPersonCharacter_C|GetShieldSize (Variables|Default|GetPlayer%20BP)))
      (Variables|Default|SetIsQskillDoing true)
      (Class|TeamChronoCharacter|IsNotDodging (Variables|Default|GetPlayer%20BP))
      (bind _returnvalue_6 (Utilities|Time|SetTimerbyFunctionName 0 "QSkilling" 0.05 true))
      (Variables|Default|SetQskillingTimer _returnvalue_6)
      (Default|BlendScreen (Variables|Default|GetPlayer%20BP) false)
      (Variables|Default|SetinBuildMode false)
      (bind _build_bp (Variables|Default|GetBuild%20BP)
        (:then
          (Actor|DestroyActor _build_bp)
          (Transformation|SetActorRotation _player_bp (Math|Rotator|MakeRotator 0.0 0.0 (.yaw _returnvalue_3)))
          (Variables|Default|SetIsMontaging true)
          (Animation|Montage|PlayMontage (Variables|/Script/Engine.Character|GetMesh _player_bp_2) "/Game/PlayerCharacter/Animation/Montage/AM_Qskill_retarget.AM_Qskill_retarget" 2.0
            (:then
              (Default|QSkillCounting (Variables|/Game/ThirdPerson/Blueprints/BP_ThirdPersonCharacter.BP_ThirdPersonCharacter_C|GetWB%20QSkill%20Count%20UI (Variables|Default|GetPlayer%20BP)) (Utilities|Array|Length (Variables|Default|GetQSkill%20BP))))
            (:OnBlendOut
              (Variables|/Script/TeamChrono.TeamChronoCharacter|SetDodgeRotation _player_bp_2 (Math|Rotator|MakeRotator 0.0 0.0 (.yaw _returnvalue_3)))
              (CallFunction|StopBuildMode)
              (Variables|Default|SetIsMontaging false))))
        (:else)))))

(event Input|EnhancedActionEvents|EnhancedInputActionIA_RightClick
  (params (ActionValue :type Boolean) (ElapsedSeconds :type Float%20%28double-precision%29) (TriggeredSeconds :type Float%20%28double-precision%29) (InputAction :type Input%20Action%20Object%20Reference :default "/Game/ThirdPerson/Input/Actions/IA_RightClick.IA_RightClick"))
  (bind _player_bp (Variables|Default|GetPlayer%20BP))
  (:Started
    (if (Variables|Default|GetinBuildMode)
      (CallFunction|QskillingEnd)
      (Variables|Default|SetQskillDelete true)
      ;[1 1 1] Q스킬 스킬 범위 삭제
      (bind _build_bp (Variables|Default|GetBuild%20BP)
        (:then
          (Actor|DestroyActor _build_bp)
          (Utilities|Time|SetGlobalTimeDilation 1.0)
          (Default|BlendScreen _player_bp false)
          (Class|TeamChronoCharacter|StaminaVariation _player_bp (* (Variables|/Script/TeamChrono.TeamChronoCharacter|GetQSkillEndStamina _player_bp) -1.0))
          (bind _output_get (Variables|Default|SetinBuildMode false))
          (Variables|/Script/TeamChrono.TeamChronoCharacter|SetIsQSkillBuilding (Variables|Default|GetPlayer%20BP) _output_get)
          (CallFunction|ResetBuildMode))
        (:else))))
  (:Completed
    (Variables|Default|SetQskillDelete false)))

(event EventBeginPlay
  (bind _asbp_third_person_character (Utilities|Casting|CastToBP_ThirdPersonCharacter (Components|GetOwner)))
  (Variables|Default|SetPlayer%20BP _asbp_third_person_character))

(event EventTick
  (params (DeltaSeconds :type Float%20%28single-precision%29))
  ;[1 1 1] Q스킬 눌렀을때 마우스 위치 확인
  (if (Variables|Default|GetinBuildMode)
    (CallFunction|PreviewLoop)
    (else
      ;[1 1 1] 마나가 없으면 공간 삭제
      (if (<= (Variables|/Script/TeamChrono.TeamChronoCharacter|GetpcStamina (Variables|Default|GetPlayer%20BP)) 0.0)
        (Utilities|Time|ClearandInvalidateTimerbyHandle (Variables|Default|GetQskillingTimer))
        (CallFunction|QskillingEnd)))))

(fn QSkilling
  (bind _player_bp (Variables|Default|GetPlayer%20BP)
    (:then
      (Class|TeamChronoCharacter|StaminaVariation _player_bp (* (Variables|/Script/TeamChrono.TeamChronoCharacter|GetQSkillingStamina _player_bp) 0.05)))
    (:else)))