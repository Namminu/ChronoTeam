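; Player scan component that fades a post-process scan effect in and out through StartScan and EndScan.
; A state machine advances normalized time on Tick and feeds time, fade flags and player location to the MC_GhisScanEffect parameter collection.
; A lazily spawned BP_Scan_Actor hosts the dynamic post-process material, with blend weight shaped by an optional curve and optional destruction on fade-out.
; Tick also prints time and state for debugging.
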(event EventBeginPlay
  (bind _asbp_third_person_character (Utilities|Casting|CastToBP_ThirdPersonCharacter (Game|GetPlayerCharacter 0))
    (:then
      (Variables|세팅|Actor|SetBP%20Third%20Person%20Character _asbp_third_person_character)
      (Scan|State|UpdateScanState "NewEnumerator3" true)
      (Rendering|Material|SetScalarParameterValue "/Game/PlayerCharacter/Tab_Skill/MC_GhisScanEffect.MC_GhisScanEffect" "GridCellSize" (Variables|Default|GetGridCellSize) :!class /Script/Engine.KismetMaterialLibrary)
      (Rendering|Material|SetScalarParameterValue "/Game/PlayerCharacter/Tab_Skill/MC_GhisScanEffect.MC_GhisScanEffect" "Range" (Variables|Default|GetRange) :!class /Script/Engine.KismetMaterialLibrary))
    (:CastFailed
      (Scan|State|UpdateScanState "NewEnumerator4" true))))

(event EventTick
  (params (DeltaSeconds :type Float%20%28single-precision%29))
  (Scan|UpdateScanTime DeltaSeconds)
  (Development|PrintString (Utilities|String|ToString(Float) (Variables|Scan|GetScanNormalizedTime)) true false "(R=0.000000,G=0.660000,B=1.000000,A=1.000000)" 0.0)
  (Development|PrintString (Utilities|String|EnumtoString (Variables|Scan|stata|GetState)) true false "(R=0.000000,G=0.660000,B=1.000000,A=1.000000)" 0.0)
  (switch Utilities|FlowControl|Switch|SwitchonEBP_Scan_State (Scan|State|GetScanState)
    (:NewEnumerator0
      (Scan|Actor|UpdateScanPPBlendWeght :!label _label))
    (:NewEnumerator1
      _)
    (:NewEnumerator2
      (goto _label))
    (:NewEnumerator3
      _))
  (bind _bp_third_person_character (Variables|세팅|Actor|GetBP%20Third%20Person%20Character)
    (:then
      (Rendering|Material|SetVectorParameterValue "/Game/PlayerCharacter/Tab_Skill/MC_GhisScanEffect.MC_GhisScanEffect" "Location" (Math|Conversions|ToLinearColor(Vector) (Transformation|GetActorLocation _bp_third_person_character)) :!class /Script/Engine.KismetMaterialLibrary))
    (:else)))

(fn GetScanState
  (return (Variables|Scan|stata|GetState)))

(fn UpdateScanState
  (params (State :type EBP_Scan_State%20Enum :default "NewEnumerator0") (Force :type Boolean))
  (if (or (Utilities|Enum|NotEqual(Enum) State (Variables|Scan|stata|GetState)) Force)
    (Utilities|FlowControl|Sequence
      (:then_0
        (switch Utilities|FlowControl|Switch|SwitchonEBP_Scan_State (Variables|Scan|stata|GetState) ; exit current state
          (:NewEnumerator1
            (Rendering|Material|SetScalarParameterValue "/Game/PlayerCharacter/Tab_Skill/MC_GhisScanEffect.MC_GhisScanEffect" "bFadedIn" 0.0 :!class /Script/Engine.KismetMaterialLibrary))
          (:NewEnumerator3
            (Rendering|Material|SetScalarParameterValue "/Game/PlayerCharacter/Tab_Skill/MC_GhisScanEffect.MC_GhisScanEffect" "bFadeOut" 0.0 :!class /Script/Engine.KismetMaterialLibrary)
            (Components|Tick|SetComponentTickEnabled true))))
      (:then_1
        (bind _output_get (Variables|Scan|stata|SetState State))
        (switch Utilities|FlowControl|Switch|SwitchonEBP_Scan_State _output_get ; enter new state
          (:NewEnumerator1
            (Rendering|Material|SetScalarParameterValue "/Game/PlayerCharacter/Tab_Skill/MC_GhisScanEffect.MC_GhisScanEffect" "bFadedIn" 1.0 :!class /Script/Engine.KismetMaterialLibrary)
            (Scan|Actor|UpdateScanPPBlendWeght))
          (:NewEnumerator3
            (Rendering|Material|SetScalarParameterValue "/Game/PlayerCharacter/Tab_Skill/MC_GhisScanEffect.MC_GhisScanEffect" "bFadeOut" 1.0 :!class /Script/Engine.KismetMaterialLibrary)
            (Scan|Actor|UpdateScanPPBlendWeght)
            (Components|Tick|SetComponentTickEnabled true :!label _label)
            (Scan|Actor|DestroyPPActor))
          (:NewEnumerator4
            (goto _label))))
      (:then_2
        (return true)))
    (else
      (return false))))

(fn StartScan
  (switch Utilities|FlowControl|Switch|SwitchonEBP_Scan_State (Scan|State|GetScanState)
    (:NewEnumerator0
      _)
    (:NewEnumerator1
      _)
    (:NewEnumerator2
      (bind _updated (Scan|State|UpdateScanState "NewEnumerator0" false :!label _label))
      (return _updated))
    (:NewEnumerator3
      (goto _label))
    (:NewEnumerator4
      _))
  (return false))

(fn EndScan
  (switch Utilities|FlowControl|Switch|SwitchonEBP_Scan_State (Scan|State|GetScanState)
    (:NewEnumerator0
      _)
    (:NewEnumerator1
      _)
    (:NewEnumerator2
      (return false))
    (:NewEnumerator3
      (return false))
    (:NewEnumerator4
      (return false)))
  (bind _updated (Scan|State|UpdateScanState "NewEnumerator2" false))
  (return _updated))

(fn UpdateScanTime
  (params (DeltaTime :type Float%20%28double-precision%29))
  (Utilities|FlowControl|Sequence
    (:then_0
      (switch Utilities|FlowControl|Switch|SwitchonEBP_Scan_State (Scan|State|GetScanState)
        (:NewEnumerator0
          (bind _output_get (Variables|Scan|SetScanNormalizedTime (+ (Variables|Scan|GetScanNormalizedTime) (* DeltaTime (Variables|세팅|Speed|GetFadeInSpeed)))))
          (if (>= _output_get 1.0)
            (Variables|Scan|SetScanNormalizedTime 1.0)
            (Scan|State|UpdateScanState "NewEnumerator1" false)))
        (:NewEnumerator2
          (bind _output_get_2 (Variables|Scan|SetScanNormalizedTime (- (Variables|Scan|GetScanNormalizedTime) (* DeltaTime (Variables|세팅|Speed|GetFadeOutSpeed)))))
          (if (<= _output_get_2 0.0)
            (Variables|Scan|SetScanNormalizedTime 0.0)
            (Scan|State|UpdateScanState "NewEnumerator3" false)))
        (:NewEnumerator4
          (return false)))
      (Rendering|Material|SetScalarParameterValue "/Game/PlayerCharacter/Tab_Skill/MC_GhisScanEffect.MC_GhisScanEffect" "NormalizedTime" (Variables|Scan|GetScanNormalizedTime) :!class /Script/Engine.KismetMaterialLibrary))
    (:then_1
      (return true))))

(fn UpdateScanPPBlendWeght
  (bind _scannormalizedtime (Variables|Scan|GetScanNormalizedTime))
  (bind _ppblendcrv (Variables|세팅|Material|GetPPBlendCrv)
    (:then
      (LocalVariables|SetThis%20Time (Math|Curves|GetFloatValue _ppblendcrv _scannormalizedtime)))
    (:else
      (LocalVariables|SetThis%20Time _scannormalizedtime)))
  (bind _scanactor (Scan|Actor|GetScanPPActor))
  (Utilities|IsValid _scanactor
    (:Is%20Valid
      (Utilities|IsValid (Variables|/Game/PlayerCharacter/Tab_Skill/BP_Scan_Actor.BP_Scan_Actor_C|GetPostProcess _scanactor)
        (:Is%20Valid
          (Variables|/Script/Engine.PostProcessComponent|SetBlendWeight (Variables|/Game/PlayerCharacter/Tab_Skill/BP_Scan_Actor.BP_Scan_Actor_C|GetPostProcess _scanactor) (LocalVariables|GetThis%20Time)))))))

(fn DestroyPPActor
  (if (and (Utilities|IsValid (Variables|Scan|Actor|GetScan%20Actor)) (Variables|세팅|Actor|GetDestroy%20Actor))
    (Actor|DestroyActor (Variables|Scan|Actor|GetScan%20Actor))
    (Variables|Scan|Actor|SetScan%20Actor 0)))

(fn GetScanPPActor
  (bind _bp_third_person_character (Variables|세팅|Actor|GetBP%20Third%20Person%20Character))
  (bind _returnvalue (Transformation|GetActorLocation _bp_third_person_character))
  (bind _scan_actor (Variables|Scan|Actor|GetScan%20Actor)
    (:then
      (return _scan_actor))
    (:else
      (bind _returnvalue_2 (Game|SpawnActorfromClass "/Game/PlayerCharacter/Tab_Skill/BP_Scan_Actor.BP_Scan_Actor_C" (Math|Transform|MakeTransform (Math|Vector|MakeVector (+ (Variables|/Game/ThirdPerson/Blueprints/BP_ThirdPersonCharacter.BP_ThirdPersonCharacter_C|GetTeleportDistance _bp_third_person_character) (.x _returnvalue)) (.y _returnvalue) (.z _returnvalue))) "Undefined" "MultiplyWithRoot" 0 0))
      (Variables|Scan|Actor|SetScan%20Actor _returnvalue_2)
      (Utilities|FlowControl|Sequence
        (:then_0
          (Utilities|IsValid (Variables|Scan|Material|GetPPMID)
            (:Is%20Valid
              _)
            (:Is%20Not%20Valid
              (bind _ppmaterial (Variables|세팅|Material|GetPPMaterial)
                (:then
                  (bind _returnvalue_3 (Rendering|Material|CreateDynamicMaterialInstance _ppmaterial "None" "None" :!class /Script/Engine.KismetMaterialLibrary))
                  (Variables|Scan|Material|SetPPMID _returnvalue_3))
                (:else))))
          (Utilities|IsValid (Variables|/Game/PlayerCharacter/Tab_Skill/BP_Scan_Actor.BP_Scan_Actor_C|GetPostProcess (Variables|Scan|Actor|GetScan%20Actor))
            (:Is%20Valid
              (Utilities|Struct|SetmembersinPostProcessSettings (Variables|/Script/Engine.PostProcessComponent|GetSettings (Variables|/Game/PlayerCharacter/Tab_Skill/BP_Scan_Actor.BP_Scan_Actor_C|GetPostProcess (Variables|Scan|Actor|GetScan%20Actor))) (Utilities|Struct|MakeWeightedBlendables (Utilities|Array|MakeArray (Utilities|Struct|MakeWeightedBlendable 1.0 (Variables|Scan|Material|GetPPMID))))))))
        (:then_1
          (return _scan_actor))))))