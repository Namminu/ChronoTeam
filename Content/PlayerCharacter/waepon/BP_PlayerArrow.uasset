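; Player arrow projectile that damages monsters and switches and can ignite into a fire arrow.
; Overlapping a FIRE-tagged actor replaces it with BP_PlayerFireArrow at its transform after a brief delay.
; On hit it plays a sound, attaches to the struck component, applies tag-filtered damage and passes the hit location to GOLEM monsters.
; It then adds a Niagara component, disables collision, stops moving and destroys itself after a few seconds.
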(event OnComponentBeginOverlap(Box)
  (params (OverlappedComponent :type Primitive%20Component%20Object%20Reference) (OtherActor :type Actor%20Object%20Reference) (OtherComp :type Primitive%20Component%20Object%20Reference) (OtherBodyIndex :type Integer) (bFromSweep :type Boolean) (SweepResult :type Hit%20Result%20Structure%20%28by%20ref%29))
  (if (Actor|ActorHasTag OtherActor "FIRE")
    (Utilities|FlowControl|Delay 0.1)
    (Game|SpawnActorfromClass "/Game/PlayerCharacter/waepon/BP_PlayerFireArrow.BP_PlayerFireArrow_C" (Transformation|GetActorTransform self) "Undefined" "MultiplyWithRoot" 0 0)
    (Actor|DestroyActor)))

(event OnComponentHit(Box)
  (params (HitComponent :type Primitive%20Component%20Object%20Reference) (OtherActor :type Actor%20Object%20Reference) (OtherComp :type Primitive%20Component%20Object%20Reference) (NormalImpulse :type Vector :default "0, 0, 0") (Hit :type Hit%20Result%20Structure%20%28by%20ref%29))
  (bind _returnvalue (Components|ComponentHasTag OtherComp "MONSTER"))
  (Audio|PlaySoundatLocation "/Game/PlayerCharacter/PlayerSound/Weapon/Player_Arrow_HitSound_Cue.Player_Arrow_HitSound_Cue" (Transformation|GetActorLocation) "0, 0, 0" 1.0 1.0 0.0 0 0 0 0)
  (Transformation|AttachComponentToComponent OtherComp "None" "KeepWorld" "KeepWorld" "KeepWorld" true)
  (if _returnvalue
    (bind _asgolem (Utilities|Casting|CastToGOLEM OtherActor)
      (:then
        (Class|BossGolem|SetHittedLocation _asgolem (.Location (Collision|BreakHitResult Hit))))
      (:CastFailed
        _)))
  (if (or _returnvalue (Actor|ActorHasTag OtherActor "SWITCH"))
    (Game|Damage|ApplyDamage OtherActor 1e+01 0 0)
    (Development|SetHiddeninGame (Variables|컴포넌트|GetNiagara) true false))
  (AddComponent|AddNiagaraComponent true (Transformation|GetActorTransform self))
  (Collision|SetCollisionEnabled (Variables|컴포넌트|GetBox) "NoCollision")
  (Variables|/Script/Engine.MovementComponent|SetVelocity (Variables|컴포넌트|GetProjectileMovement) "0, 0, 0")
  (Utilities|FlowControl|Delay 3.0)
  (Actor|DestroyActor))

(event EventBeginPlay
  (Audio|PlaySoundatLocation "/Game/PlayerCharacter/PlayerSound/Weapon/Player_ArrowSound_Cue.Player_ArrowSound_Cue" (Transformation|GetActorLocation) "0, 0, 0" 1.0 1.0 0.0 0 0 0 0))

(fn ConstructionScript)