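; BP_PlayerBomb is a player bomb actor that damages whatever its mesh hits and bursts into a BP_Firebomb.
; On component hit, a MONSTER tag check routes to a GOLEM cast that records the hit location; a failed cast halts the chain.
; Successful casts and untagged hits both apply fixed damage, spawn BP_Firebomb slightly above the mesh, then destroy the bomb.
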(event OnComponentHit(StaticMesh)
  (params (HitComponent :type Primitive%20Component%20Object%20Reference) (OtherActor :type Actor%20Object%20Reference) (OtherComp :type Primitive%20Component%20Object%20Reference) (NormalImpulse :type Vector :default "0, 0, 0") (Hit :type Hit%20Result%20Structure%20%28by%20ref%29))
  (bind _staticmesh (Variables|Default|GetStaticMesh))
  (bind _returnvalue (Transformation|GetWorldTransform _staticmesh))
  (if (Components|ComponentHasTag OtherComp "MONSTER")
    (bind _asgolem (Utilities|Casting|CastToGOLEM OtherActor))
    (Class|BossGolem|SetHittedLocation _asgolem (.Location (Collision|BreakHitResult Hit))))
  (Game|Damage|ApplyDamage OtherActor 1e+01 0 0)
  (Game|SpawnActorfromClass "/Game/PlayerCharacter/waepon/BP_Firebomb.BP_Firebomb_C" (Math|Transform|MakeTransform (Math|Vector|MakeVector (.x (.location _returnvalue)) (.y (.location _returnvalue)) (+ (.z (.location _returnvalue)) 1e+01)) "0, 0, 0" "1.000000,1.000000,1.000000") "Undefined" "MultiplyWithRoot" 0 0)
  (Actor|DestroyActor))

(event EventBeginPlay)

(event Collision|EventActorBeginOverlap
  (params (OtherActor :type Actor%20Object%20Reference)))

(event EventTick
  (params (DeltaSeconds :type Float%20%28single-precision%29)))

(fn ConstructionScript)