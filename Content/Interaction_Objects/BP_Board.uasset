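; BP_Board is a readable board that supplies an "[F] 읽기" (Read) prompt and shows its text on screen.
; Interactive toggles a WB_Script widget, created anew on each opening and filled with MainText, with IsScript tracking the open state.
; The widget also closes when an overlap with the Sphere ends or the game pauses.
; Tick is enabled on opening to watch for pause and disabled on closing.
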(event OnComponentEndOverlap(Sphere)
  (params (OverlappedComponent :type Primitive%20Component%20Object%20Reference) (OtherActor :type Actor%20Object%20Reference) (OtherComp :type Primitive%20Component%20Object%20Reference) (OtherBodyIndex :type Integer))
  (if (Variables|Default|GetIsScript)
    (Widget|RemovefromParent (Variables|Default|GetWB%20Script))
    (Variables|Default|SetIsScript false)
    (Actor|Tick|SetActorTickEnabled false)))

(event EventBeginPlay)

(event Collision|EventActorBeginOverlap
  (params (OtherActor :type Actor%20Object%20Reference)))

(event EventTick
  (params (DeltaSeconds :type Float%20%28single-precision%29))
  (if (Game|IsGamePaused)
    (if (Variables|Default|GetIsScript)
      (Widget|RemovefromParent (Variables|Default|GetWB%20Script))
      (Variables|Default|SetIsScript false)
      (Actor|Tick|SetActorTickEnabled false))))

(event EventInteractive
  (if (not (Variables|Default|GetIsScript))
    (Variables|Default|SetIsScript true)
    (bind _returnvalue (UserInterface|CreateWidget "/Game/UI/WB_Script.WB_Script_C"))
    (bind _output_get (Variables|Default|SetWB%20Script _returnvalue))
    (Default|MainText _output_get (Variables|Default|GetMainText))
    (UserInterface|Viewport|AddtoViewport _output_get 0)
    (Actor|Tick|SetActorTickEnabled true)
    (elif (Variables|Default|GetIsScript)
      (Widget|RemovefromParent (Variables|Default|GetWB%20Script))
      (Variables|Default|SetIsScript false)
      (Actor|Tick|SetActorTickEnabled false))))

(fn ConstructionScript)

(fn WidgetText
  (return "[F] 읽기"))