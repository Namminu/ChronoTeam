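; Interactable checkpoint Blueprint, prompted with "[F] 저장하기" (save), that sets the player's spawn transform and restores HP to max.
; Interacting broadcasts the player's spawn-change dispatcher, so each point compares transforms and only the active one shows its helix.
; The active point spins two meshes through a Timeline that replays itself until another point takes over.
; Sphere overlap flags whether this point is already active, blocking repeat interaction.
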(event OnComponentBeginOverlap(Sphere)
  (params (OverlappedComponent :type Primitive%20Component%20Object%20Reference) (OtherActor :type Actor%20Object%20Reference) (OtherComp :type Primitive%20Component%20Object%20Reference) (OtherBodyIndex :type Integer) (bFromSweep :type Boolean) (SweepResult :type Hit%20Result%20Structure%20%28by%20ref%29))
  (if (== (Variables|/Game/ThirdPerson/Blueprints/BP_ThirdPersonCharacter.BP_ThirdPersonCharacter_C|GetPlayerSpawnTransfrom (Variables|Default|GetBP%20Player)) (Transformation|GetWorldTransform (Variables|Default|GetSpawnTransfrom)))
    (Variables|Default|SetIs%20Operationing true)
    (else
      (Variables|Default|SetIs%20Operationing false))))

(event Custom|IsSpawnChange
  (if (== (Variables|/Game/ThirdPerson/Blueprints/BP_ThirdPersonCharacter.BP_ThirdPersonCharacter_C|GetPlayerSpawnTransfrom (Variables|Default|GetBP%20Player)) (Transformation|GetWorldTransform (Variables|Default|GetSpawnTransfrom)))
    (Development|SetHiddeninGame (Variables|Default|GetNE_Helix1) false false)
    (Variables|Default|SetIsPoint true)
    (bind _새_트랙_0 (Timeline|타임라인 PlayFromStart)
      (:Update
        (Transformation|SetWorldRotation (Variables|Default|GetRe_HP_Object) (Math|Rotator|Lerp(Rotator) "0, 0, 0" "360.000000,0.000000,0.000000" _새_트랙_0) false false)
        (Transformation|SetWorldRotation (Variables|Default|GetRe_HP_Object001) (Math|Rotator|Lerp(Rotator) "0, 0, 0" "0.000000,0.000000,360.000000" _새_트랙_0) false false))
      (:Finished
        (if (Variables|Default|GetIsPoint)
          (Timeline|타임라인 PlayFromStart))))
    (else
      (Development|SetHiddeninGame (Variables|Default|GetNE_Helix1) true false)
      (Variables|Default|SetIsPoint false))))

(event EventBeginPlay
  (|CallParentFunction)
  (Development|SetHiddeninGame (Variables|Default|GetNE_Helix1) true false)
  (EventDispatchers|BindEventtoIsSpawnPointChange (Variables|Default|GetBP%20Player) (delegate Custom|IsSpawnChange)))

(event EventInteractive
  (bind _bp_player (Variables|Default|GetBP%20Player))
  (if (not (Variables|Default|GetIs%20Operationing))
    (Variables|/Game/ThirdPerson/Blueprints/BP_ThirdPersonCharacter.BP_ThirdPersonCharacter_C|SetPlayerSpawnTransfrom (Variables|Default|GetBP%20Player) (Transformation|GetWorldTransform (Variables|Default|GetSpawnTransfrom)))
    (Development|SetHiddeninGame (Variables|Default|GetWidget) true false)
    (Default|ESkillHPFix _bp_player (Variables|/Script/TeamChrono.TeamChronoCharacter|GetP_MaxHP _bp_player))
    (Default|CallIsSpawnPointChange (Variables|Default|GetBP%20Player))))

(fn ConstructionScript)

(fn WidgetText
  (return (Utilities|Text|ToText(String) (Utilities|String|Append "[F] " "저장하기"))))