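; HP recovery pickup, a "Crystal of Life" (생명의 수정) that the player uses through an [F] interaction prompt.
; A looping Timeline spins the mesh in yaw from BeginPlay.
; On first interaction it calls the player's PlusHPRecovery, hides mesh, widget and magic-circle effect, adds a Niagara effect above the mesh, then destroys itself after a short delay.
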(event EventBeginPlay
  (|CallParentFunction)
  (bind _새_트랙_0 (Timeline|타임라인_0 Play)
    (:Update
      (Transformation|SetWorldRotation (Variables|Default|GetStaticMesh) (Math|Rotator|MakeRotator 0.0 1.8e+02 (Math|Float|Lerp 0.0 3.6e+02 _새_트랙_0)) false false))
    (:Finished
      (if true
        (Timeline|타임라인_0 PlayFromStart)))))

(event EventInteractive
  (bind _staticmesh (Variables|Default|GetStaticMesh))
  (bind _returnvalue (Transformation|GetWorldLocation _staticmesh))
  (if (not (Variables|Default|GetIs%20Operationing))
    (Variables|Default|SetIs%20Operationing true)
    (Default|PlusHPRecovery (Variables|Default|GetBP%20Player))
    (Development|SetHiddeninGame (Variables|Default|GetWidget) true false)
    (Development|SetHiddeninGame (Variables|Default|GetStaticMesh) true false)
    (Development|SetHiddeninGame (Variables|Default|GetNS_MagicCircle_UpHpEffect) true false)
    (AddComponent|AddNiagaraComponent true (Math|Transform|MakeTransform (Math|Vector|MakeVector (.x _returnvalue) (.y _returnvalue) (+ (.z _returnvalue) 35.0)) "0, 0, 0" "1.000000,1.000000,1.000000"))
    (Utilities|FlowControl|Delay 2.0)
    (Actor|DestroyActor)))

(fn ConstructionScript
  (|CallParentFunction))

(fn WidgetText
  (return (Utilities|Text|ToText(String) (Utilities|String|Append "[F] " "생명의 수정"))))