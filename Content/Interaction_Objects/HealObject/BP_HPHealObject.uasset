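; Interactable healing object that restores the player's HP by adding their max HP, usable only when HP is not full.
; Interacting hides the "[F] 회복하기" (Heal) prompt, attaches a heal Niagara actor to the player, spawns an impact actor and brightens the mesh's glow material.
; A timeline raises the object, then reverses to lower it, with flags blocking reuse until it lands and the prompt returns for an in-range player.
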(event EventBeginPlay
  (bind _skeletalmesh (Variables|Default|GetSkeletalMesh))
  (|CallParentFunction)
  (Variables|Default|SetStartLocation (Transformation|GetActorLocation))
  (bind _returnvalue (Rendering|Material|CreateDynamicMaterialInstance _skeletalmesh 0 (Rendering|Material|GetMaterial _skeletalmesh 0) "None" :!class /Script/Engine.PrimitiveComponent))
  (Variables|Default|SetGlow%20MT _returnvalue))

(event EventInteractive
  (bind _startlocation (Variables|Default|GetStartLocation))
  (bind _startlocation_2 (Variables|Default|GetStartLocation))
  (if (not (Variables|Default|GetIs%20Operationing))
    (bind _bp_player (Variables|Default|GetBP%20Player)
      (:then
        (if (!= (Variables|/Script/TeamChrono.TeamChronoCharacter|GetP_MaxHP _bp_player) (Variables|/Script/TeamChrono.TeamChronoCharacter|GetP_CurrentHP _bp_player))
          (Variables|Default|SetIs%20Operationing true)
          (Default|PlusHP _bp_player (Variables|/Script/TeamChrono.TeamChronoCharacter|GetP_MaxHP _bp_player))
          (Development|SetHiddeninGame (Variables|Default|GetWidget) true false)
          (bind _returnvalue (Game|SpawnActorfromClass "/Game/Interaction_Objects/HealObject/BP_HealNiagara.BP_HealNiagara_C" (Math|Transform|MakeTransform "0, 0, 0" "0, 0, 0" "1.000000,1.000000,1.000000") "Undefined" "MultiplyWithRoot" 0 0))
          (Transformation|AttachActorToActor _returnvalue (Variables|Default|GetBP%20Player) "None" "KeepRelative" "KeepRelative" "KeepRelative" true)
          (bind _returnvalue_2 (Game|SpawnActorfromClass "/Game/Interaction_Objects/HealObject/BP_HPObjectImpact.BP_HPObjectImpact_C" (Math|Transform|MakeTransform (Math|Vector|MakeVector (.x _startlocation) (.y _startlocation) (+ (.z _startlocation) 0.1)) "0, 0, 0" "1.000000,1.000000,1.000000") "Undefined" "MultiplyWithRoot" 0 0))
          (Rendering|Material|SetScalarParameterValue (Variables|Default|GetGlow%20MT) "Glow Instense" 2e+01 :!class /Script/Engine.MaterialInstanceDynamic)
          (bind _새_트랙_0 (Timeline|타임라인 PlayFromStart)
            (:Update
              (Transformation|SetActorLocation (Math|Vector|MakeVector (.x _startlocation_2) (.y _startlocation_2) (+ (.z _startlocation_2) (Math|Float|Lerp 0.0 5e+01 _새_트랙_0))) false false))
            (:Finished
              (if (not (Variables|Default|GetisSky))
                (Variables|Default|SetisSky true)
                (Utilities|FlowControl|Sequence
                  (:then_0
                    (Utilities|FlowControl|Delay 1.9)
                    (Rendering|Material|SetScalarParameterValue (Variables|Default|GetGlow%20MT) "Glow Instense" 1.0 :!class /Script/Engine.MaterialInstanceDynamic))
                  (:then_1
                    (Timeline|타임라인 ReverseFromEnd)))
                (else
                  (Variables|Default|SetisSky false)
                  (Variables|Default|SetIs%20Operationing false)
                  (Actor|DestroyActor _returnvalue_2)
                  (if (Variables|/Game/ThirdPerson/Blueprints/BP_ThirdPersonCharacter.BP_ThirdPersonCharacter_C|GetInteractionRanging (Variables|Default|GetBP%20Player))
                    (Development|SetHiddeninGame (Variables|Default|GetWidget) false false))))))))
      (:else))))

(fn ConstructionScript)

(fn WidgetText
  (return (Utilities|Text|ToText(String) (Utilities|String|Append "[F] " "회복하기"))))