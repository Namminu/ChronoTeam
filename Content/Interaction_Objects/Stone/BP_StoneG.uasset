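; BP_StoneG is an interactable stone pickup that bobs between two points and shows an "[F] 획득하기" (acquire) prompt.
; A timeline lerps Main between Start and End, ping-ponging via the IsFly flag.
; On first interaction it flags BPPlayer, hides its visuals and adds a Niagara effect.
; After a short delay it records StoneG in GI_TeamChrono and destroys itself.
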(event EventBeginPlay
  (|CallParentFunction)
  (bind _새_트랙_0 (Timeline|타임라인 Play)
    (:Update
      (Transformation|SetWorldLocation (Variables|Default|Getmain) (Math|Vector|Lerp(Vector) (Transformation|GetWorldLocation (Variables|Default|GetStart)) (Transformation|GetWorldLocation (Variables|Default|GetEnd)) _새_트랙_0) false false))
    (:Finished
      (if (not (Variables|Default|GetIsFly))
        (Variables|Default|SetIsFly true)
        (Timeline|타임라인 ReverseFromEnd)
        (else
          (Variables|Default|SetIsFly false)
          (Timeline|타임라인 PlayFromStart))))))

(event EventInteractive
  (bind _staticmesh (Variables|Default|GetStaticMesh))
  (bind _returnvalue (Transformation|GetWorldLocation _staticmesh))
  (if (not (Variables|Default|GetIs%20Operationing))
    (Variables|Default|SetIs%20Operationing true)
    (Variables|/Game/ThirdPerson/Blueprints/BP_ThirdPersonCharacter.BP_ThirdPersonCharacter_C|SetIsStoneG (Variables|Default|GetBP%20Player) true)
    (Development|SetHiddeninGame (Variables|Default|GetWidget) true false)
    (Development|SetHiddeninGame (Variables|Default|GetStaticMesh) true false)
    (Development|SetHiddeninGame (Variables|Default|GetNS_MagicCircle_UpHpEffect) true false)
    (AddComponent|AddNiagaraComponent true (Math|Transform|MakeTransform (Math|Vector|MakeVector (.x _returnvalue) (.y _returnvalue) (+ (.z _returnvalue) 35.0)) "0, 0, 0" "1.000000,1.000000,1.000000"))
    (Utilities|FlowControl|Delay 2.0)
    (bind _asgi_team_chrono (Utilities|Casting|CastToGI_TeamChrono (Game|GetGameInstance)))
    (Variables|/Game/zGameInstance_TeamChrono/GI_TeamChrono.GI_TeamChrono_C|SetStoneG _asgi_team_chrono true)
    (Actor|DestroyActor)))

(fn ConstructionScript
  (|CallParentFunction))

(fn WidgetText
  (return (Utilities|Text|ToText(String) (Utilities|String|Append "[F] " "획득하기"))))