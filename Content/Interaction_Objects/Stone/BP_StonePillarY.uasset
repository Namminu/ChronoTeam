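; BP_StonePillarY is an interactable stone pillar that accepts the Y stone when the player's IsStoneY flag is set.
; Capsule overlap shows or hides a prompt widget and binds or unbinds Interactive on the player's OnInteraction event.
; Interactive runs once while IsOperationing is unset, playing a casting emitter and delayed Niagara effect before revealing StoneY and calling Operation.
; The prompt text from WidgetText is still a placeholder string.
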(event OnComponentBeginOverlap(Capsule)
  (params (OverlappedComponent :type Primitive%20Component%20Object%20Reference) (OtherActor :type Actor%20Object%20Reference) (OtherComp :type Primitive%20Component%20Object%20Reference) (OtherBodyIndex :type Integer) (bFromSweep :type Boolean) (SweepResult :type Hit%20Result%20Structure%20%28by%20ref%29))
  (bind _bp_player (Variables|Default|GetBP%20Player)
    (:then
      (if (== _bp_player OtherActor)
        (Variables|/Game/ThirdPerson/Blueprints/BP_ThirdPersonCharacter.BP_ThirdPersonCharacter_C|SetInteractionRanging _bp_player true)
        (EventDispatchers|BindEventtoOnInteraction (Variables|Default|GetBP%20Player) (delegate Custom|Interactive))
        (if (not (Variables|Default|GetIs%20Operationing))
          (Development|SetHiddeninGame (Variables|Default|GetWidget) false false))))
    (:else)))

(event OnComponentEndOverlap(Capsule)
  (params (OverlappedComponent :type Primitive%20Component%20Object%20Reference) (OtherActor :type Actor%20Object%20Reference) (OtherComp :type Primitive%20Component%20Object%20Reference) (OtherBodyIndex :type Integer))
  (bind _bp_player (Variables|Default|GetBP%20Player)
    (:then
      (if (== _bp_player OtherActor)
        (Variables|/Game/ThirdPerson/Blueprints/BP_ThirdPersonCharacter.BP_ThirdPersonCharacter_C|SetInteractionRanging _bp_player false)
        (EventDispatchers|UnbindallEventsfromOnInteraction (Variables|Default|GetBP%20Player))
        (Development|SetHiddeninGame (Variables|Default|GetWidget) true false)))
    (:else)))

(event Custom|Interactive
  (if (Variables|/Game/ThirdPerson/Blueprints/BP_ThirdPersonCharacter.BP_ThirdPersonCharacter_C|GetIsStoneY (Variables|Default|GetBP%20Player))
    (if (not (Variables|Default|GetIs%20Operationing))
      (Variables|Default|SetIs%20Operationing true)
      (Effects|SpawnEmitteratLocation "/Game/MagicBeams/Particles/P_Casting_08.P_Casting_08" (Transformation|GetWorldLocation (Variables|Default|GetStone_Y)) "0, 0, 0" "3.000000,3.000000,3.000000")
      (Development|SetHiddeninGame (Variables|Default|GetWidget) true false)
      (Utilities|FlowControl|Delay 1.6)
      (AddComponent|AddNiagaraComponent true (Math|Transform|MakeTransform (Transformation|GetWorldLocation (Variables|Default|GetStone_Y)) "0, 0, 0" "3.000000,3.000000,3.000000"))
      (Utilities|FlowControl|Delay 0.1)
      (Development|SetHiddeninGame (Variables|Default|GetStone_Y) false false)
      (CallFunction|Operation))))

(event EventBeginPlay
  (|CallParentFunction)
  (bind _asbp_third_person_character (Utilities|Casting|CastToBP_ThirdPersonCharacter (Game|GetPlayerCharacter 0)))
  (Variables|Default|SetBP%20Player _asbp_third_person_character)
  (bind _aswb_interaction (Utilities|Casting|CastToWB_Interaction (UserInterface|GetUserWidgetObject (Variables|Default|GetWidget))))
  (bind _output_get (Variables|Default|SetWB%20Interaction _aswb_interaction))
  (bind _newparam (CallFunction|WidgetText))
  (Default|InteractionText _output_get _newparam))

(event Collision|EventActorBeginOverlap
  (params (OtherActor :type Actor%20Object%20Reference))
  (|CallParentFunction OtherActor) ; 지금 이 노드는 비활성 상태입니다. \n핀을 끌어서 다른 노드를 연결하면 활성화됩니다.
)

(event EventTick
  (params (DeltaSeconds :type Float%20%28single-precision%29))
  (|CallParentFunction DeltaSeconds) ; 지금 이 노드는 비활성 상태입니다. \n핀을 끌어서 다른 노드를 연결하면 활성화됩니다.
)

(fn ConstructionScript
  (|CallParentFunction))

(fn WidgetText
  (return "111111111"))