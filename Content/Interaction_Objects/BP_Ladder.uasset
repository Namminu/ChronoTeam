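; Climbable ladder actor that can optionally start hidden as the reward of a multi-switch puzzle.
; The construction script stacks section meshes by rung count and fits the climb and top trigger boxes to the height.
; In puzzle mode it tallies switches, updates fire indicators, completes a spawned stand-in ladder, then polls on Tick to reveal itself.
; Overlaps bind the third-person character's interaction to toggle climbing, show ladder UI and trigger the top climb.
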(event OnComponentBeginOverlap(PlayerClimbCheck)
  (params (OverlappedComponent :type Primitive%20Component%20Object%20Reference) (OtherActor :type Actor%20Object%20Reference) (OtherComp :type Primitive%20Component%20Object%20Reference) (OtherBodyIndex :type Integer) (bFromSweep :type Boolean) (SweepResult :type Hit%20Result%20Structure%20%28by%20ref%29))
  (bind _asbp_third_person_character (Utilities|Casting|CastToBP_ThirdPersonCharacter OtherActor))
  (Variables|/Game/ThirdPerson/Blueprints/BP_ThirdPersonCharacter.BP_ThirdPersonCharacter_C|SetInteractionRanging _asbp_third_person_character true)
  (EventDispatchers|BindEventtoOnInteraction _asbp_third_person_character (delegate Custom|Interactive))
  (Default|LadderUI _asbp_third_person_character true))

(event OnComponentEndOverlap(PlayerClimbCheck)
  (params (OverlappedComponent :type Primitive%20Component%20Object%20Reference) (OtherActor :type Actor%20Object%20Reference) (OtherComp :type Primitive%20Component%20Object%20Reference) (OtherBodyIndex :type Integer))
  (bind _asbp_third_person_character (Utilities|Casting|CastToBP_ThirdPersonCharacter OtherActor))
  (Variables|/Game/ThirdPerson/Blueprints/BP_ThirdPersonCharacter.BP_ThirdPersonCharacter_C|SetInteractionRanging _asbp_third_person_character false)
  (Default|ToggleClimbing _asbp_third_person_character false self)
  (EventDispatchers|UnbindallEventsfromOnInteraction _asbp_third_person_character)
  (Default|LadderUI _asbp_third_person_character false))

(event OnComponentBeginOverlap(TopBox)
  (params (OverlappedComponent :type Primitive%20Component%20Object%20Reference) (OtherActor :type Actor%20Object%20Reference) (OtherComp :type Primitive%20Component%20Object%20Reference) (OtherBodyIndex :type Integer) (bFromSweep :type Boolean) (SweepResult :type Hit%20Result%20Structure%20%28by%20ref%29))
  (bind _asbp_third_person_character (Utilities|Casting|CastToBP_ThirdPersonCharacter OtherActor))
  (if (Variables|/Script/TeamChrono.TeamChronoCharacter|GetIsClimbing _asbp_third_person_character)
    (Default|ClimbingTop _asbp_third_person_character)))

(event Custom|Interactive
  (if (Variables|/Script/TeamChrono.TeamChronoCharacter|GetIsClimbing (stale OnComponentBeginOverlap(PlayerClimbCheck) _asbp_third_person_character))
    (Default|ToggleClimbing (stale OnComponentBeginOverlap(PlayerClimbCheck) _asbp_third_person_character) false self)
    (Default|LadderUI (stale OnComponentBeginOverlap(PlayerClimbCheck) _asbp_third_person_character) true)
    (else
      (Default|ToggleClimbing (stale OnComponentBeginOverlap(PlayerClimbCheck) _asbp_third_person_character) true self)
      (Default|LadderUI (stale OnComponentBeginOverlap(PlayerClimbCheck) _asbp_third_person_character) false))))

(event Custom|MakingLadder
  (Default|GimicComplete (Variables|Default|GetBP_Look))
  (Actor|Tick|SetActorTickEnabled true))

(event Custom|IsBeginSwitch
  (params (IsGimic :type Boolean))
  (if IsGimic
    (Math|Integer|IncrementInt (Variables|Default|GetSwitchOperationNum)
      (:%20%20
        _))
    (else
      (Math|Integer|DecrementInt (Variables|Default|GetSwitchOperationNum)
        (:%20%20
          _))))
  (CallFunction|IsGimicSuccess)
  (for (_array_element _array_index) (Variables|Default|GetBP_ClearFire)
    (Default|FIreonOff _array_element (> (Variables|Default|GetSwitchOperationNum) _array_index))))

(event EventBeginPlay
  (if (Variables|Default|GetIsGimicBool)
    (for _array_element (Variables|Default|GetBP_Switches)
      (EventDispatchers|BindEventtoBeginSwitch _array_element (delegate Custom|IsBeginSwitch)))
    (bind _returnvalue (Game|SpawnActorfromClass "/Game/Interaction_Objects/BP_GimicLookLadder.BP_GimicLookLadder_C" (Transformation|GetWorldTransform (Variables|Default|GetLookSpawn)) "Undefined" "MultiplyWithRoot" 0 0))
    (bind _output_get (Variables|Default|SetBP_Look _returnvalue))
    (Variables|/Game/Interaction_Objects/BP_GimicLookLadder.BP_GimicLookLadder_C|SetNumberOfRungs _output_get (Variables|Default|GetNumberOfRungs))
    (Rendering|SetActorHiddenInGame true)
    (Collision|SetCollisionEnabled (Variables|Default|GetPlayerClimbCheck) "NoCollision")))

(event EventTick
  (params (DeltaSeconds :type Float%20%28single-precision%29))
  (if (Variables|/Game/Interaction_Objects/BP_GimicLookLadder.BP_GimicLookLadder_C|GetIsComplete (Variables|Default|GetBP_Look))
    (Rendering|SetActorHiddenInGame false)
    (Actor|DestroyActor (Variables|Default|GetBP_Look))
    (Collision|SetCollisionEnabled (Variables|Default|GetPlayerClimbCheck) "QueryOnly")
    (Actor|Tick|SetActorTickEnabled false)))

(fn ConstructionScript
  (bind _playercimbcheckboxsize_xy (Variables|Default|GetPlayerCimbCheckBoxSize_XY))
  (Utilities|FlowControl|Sequence
    (:then_0
      (Variables|Default|SetLadderSectionMeshHeight (* (.z (.boxextent (StaticMesh|GetBounds (Variables|Default|GetLadderSectionMesh)))) 2.0)))
    (:then_1
      (for _index (range 0 (- (Variables|Default|GetNumberOfRungs) 1))
        (bind _returnvalue (AddComponent|AddStaticMeshComponent false (Math|Transform|MakeTransform (Math|Vector|MakeVector 0.0 0.0 (* _index (Variables|Default|GetLadderSectionMeshHeight))) "0, 0, 0" "1.000000,1.000000,1.000000")))
        (Components|StaticMesh|SetStaticMesh _returnvalue (Variables|Default|GetLadderSectionMesh))))
    (:then_2
      (Components|Box|SetBoxExtent (Variables|Default|GetPlayerClimbCheck) (Math|Vector|MakeVector _playercimbcheckboxsize_xy _playercimbcheckboxsize_xy (/ (* (Variables|Default|GetNumberOfRungs) (Variables|Default|GetLadderSectionMeshHeight)) 2)) true)
      (Transformation|SetRelativeLocation (Variables|Default|GetPlayerClimbCheck) (Math|Vector|MakeVector 0.0 (Variables|Default|GetNew%20Location%20Y) (+ (/ (* (Variables|Default|GetNumberOfRungs) (Variables|Default|GetLadderSectionMeshHeight)) 2) (.z (.min (StaticMesh|GetBoundingBox (Variables|Default|GetLadderSectionMesh)))))) false false)
      (Transformation|SetRelativeLocation (Variables|Default|GetTopBox) (Math|Vector|MakeVector 0.0 (Variables|Default|GetNew%20Location%20Y) (+ (* (Variables|Default|GetNumberOfRungs) (Variables|Default|GetLadderSectionMeshHeight)) (.z (.min (StaticMesh|GetBoundingBox (Variables|Default|GetLadderSectionMesh)))) 1.3e+02)) false false)
      (Transformation|SetRelativeLocation (Variables|Default|GetArrow) (Math|Vector|MakeVector 0.0 (Math|Float|SelectFloat 4e+01 -4e+01 (>= (Variables|Default|GetNew%20Location%20Y) 0.0)) 8e+01) false false)
      (Transformation|SetRelativeLocation (Variables|Default|GetLookSpawn) (Math|Vector|MakeVector 0.0 0.0 (* (Variables|Default|GetLadderSectionMeshHeight) (- (Variables|Default|GetNumberOfRungs) 1))) false false))))

(fn IsGimicSuccess
  (if (== (Utilities|Array|Length (Variables|Default|GetBP_Switches)) (Variables|Default|GetSwitchOperationNum))
    (for _array_element (Variables|Default|GetBP_Switches)
      (Variables|/Game/Puzzle/BP_BaseSwitch.BP_BaseSwitch_C|SetMultipleGimicSuccess _array_element true)
      (Default|Operation _array_element))
    (CallFunction|MakingLadder)))