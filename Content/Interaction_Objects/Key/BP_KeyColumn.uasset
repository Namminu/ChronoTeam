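; BP_KeyColumn is a switch-triggered column that opens its jail object and produces a key.
; BeginPlay caches the jail mesh's start location and an end point directly below it.
; SwitchInteraction chains two timeline lerps, first lowering the jail, then moving MoveStaticMesh between the Start and End components.
; When both finish, it hides the placeholder Key component and spawns a BP_Key actor at its location and rotation.
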(event EventBeginPlay
  (|CallParentFunction)
  (Variables|Default|SetJailStartLocation (Transformation|GetWorldLocation (Variables|Default|GetJail_Object005)))
  (Variables|Default|SetJailEndLocation (- (Transformation|GetWorldLocation (Variables|Default|GetJail_Object005)) "0.000000,0.000000,190.000000")))

(event Collision|EventActorBeginOverlap
  (params (OtherActor :type Actor%20Object%20Reference)))

(event EventTick
  (params (DeltaSeconds :type Float%20%28single-precision%29)))

(event EventSwitchInteraction
  (bind _key (Variables|Default|GetKey))
  (bind _returnvalue (Transformation|GetWorldTransform _key))
  (bind _새_트랙_0 (Timeline|타임라인_1 Play)
    (:Update
      (Transformation|SetWorldLocation (Variables|Default|GetJail_Object005) (Math|Vector|Lerp(Vector) (Variables|Default|GetJailStartLocation) (Variables|Default|GetJailEndLocation) _새_트랙_0) false false))
    (:Finished
      (bind _새_트랙_0_2 (Timeline|타임라인_0 Play)
        (:Update
          (Transformation|SetWorldLocation (Variables|Default|GetMove_StaticMesh) (Math|Vector|Lerp(Vector) (Transformation|GetWorldLocation (Variables|Default|GetStart)) (Transformation|GetWorldLocation (Variables|Default|GetEnd)) _새_트랙_0_2) false false))
        (:Finished
          (Development|SetHiddeninGame (Variables|Default|GetKey) true false)
          (Game|SpawnActorfromClass "/Game/Interaction_Objects/Key/BP_Key.BP_Key_C" (Math|Transform|MakeTransform (.location _returnvalue) (.rotation _returnvalue) "1.000000,1.000000,1.000000") "Undefined" "MultiplyWithRoot" 0 0))))))

(fn ConstructionScript
  (|CallParentFunction))