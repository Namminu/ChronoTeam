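; BP_keyDoor is an interactable key lock that animates a key being inserted and turned when Interactive fires.
; Chained timelines move the Key from KeyStart to KeyEnd, then lerp its rotation between them, with short delays.
; It then adds a Niagara component and hides the key and KeyBox.
; The door-slide timeline and setting of the IsOperationing guard are disconnected, and WidgetText returns placeholder-like "1111".
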(event EventBeginPlay
  (|CallParentFunction))

(event Collision|EventActorBeginOverlap
  (params (OtherActor :type Actor%20Object%20Reference)))

(event EventTick
  (params (DeltaSeconds :type Float%20%28single-precision%29)))

(event EventInteractive
  (bind _key_start (Variables|Default|GetKey_Start))
  (bind _returnvalue (Transformation|GetWorldTransform _key_start))
  (if (not (Variables|Default|GetIs%20Operationing))
    (Transformation|SetWorldLocationAndRotation (Variables|Default|GetKey) (.location _returnvalue) (.rotation _returnvalue) false false)
    (Development|SetHiddeninGame (Variables|Default|GetKey) false false)
    (Development|SetHiddeninGame (Variables|Default|GetWidget) true false)
    (Utilities|FlowControl|Delay 0.2)
    (bind _새_트랙_0 (Timeline|타임라인_0 PlayFromStart)
      (:Update
        (Transformation|SetWorldLocation (Variables|Default|GetKey) (Math|Vector|Lerp(Vector) (Transformation|GetWorldLocation (Variables|Default|GetKey_Start)) (Transformation|GetWorldLocation (Variables|Default|GetKey_End)) _새_트랙_0) false false))
      (:Finished
        (Utilities|FlowControl|Delay 0.2)
        (bind _새_트랙_0_2 (Timeline|타임라인_1 PlayFromStart)
          (:Update
            (Transformation|SetWorldRotation (Variables|Default|GetKey) (Math|Rotator|Lerp(Rotator) (Transformation|GetWorldRotation (Variables|Default|GetKey_Start)) (Transformation|GetWorldRotation (Variables|Default|GetKey_End)) _새_트랙_0_2 true) false false))
          (:Finished
            (Utilities|FlowControl|Delay 0.2)
            (AddComponent|AddNiagaraComponent true (Math|Transform|MakeTransform (Transformation|GetWorldLocation (Variables|Default|GetKey)) "0, 0, 0" "10.000000,10.000000,10.000000"))
            (Development|SetHiddeninGame (Variables|Default|GetKey) true false)
            (Development|SetHiddeninGame (Variables|Default|GetKey_Box) true false)))))))

(fn ConstructionScript)

(fn WidgetText
  (return "1111"))