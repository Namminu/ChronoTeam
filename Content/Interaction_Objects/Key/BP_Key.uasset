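; Collectible key actor that spins in place and shows an [F] acquire prompt until the player interacts with it.
; Interacting hides the prompt and lifts the key while it spins progressively faster, by restarting one timeline from later offsets with rescaled alpha, then handing off to a looping timeline.
; When the rise ends, it adds a key to the player, hides the mesh, spawns a Niagara effect and destroys itself after a delay.
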(event EventBeginPlay
  (|CallParentFunction)
  (Variables|Default|SetStartYaw (.yaw (Transformation|GetActorRotation)))
  (bind _새_트랙_0 (Timeline|타임라인 Play)
    (:Update
      (if (not (Variables|Default|GetIs%20Operationing))
        (Transformation|SetWorldRotation (Variables|Default|GetKey) (Math|Rotator|MakeRotator 0.0 0.0 (+ (Variables|Default|GetStartYaw) (Math|Float|Lerp 0.0 3.6e+02 _새_트랙_0))) false false)
        (else
          (Timeline|타임라인 Stop))))
    (:Finished
      (if (not (Variables|Default|GetIs%20Operationing))
        (Timeline|타임라인 PlayFromStart)))))

(event EventInteractive
  (if (not (Variables|Default|GetIs%20Operationing))
    (Variables|Default|SetIs%20Operationing true)
    (Development|SetHiddeninGame (Variables|Default|GetWidget) true false)
    (Variables|Default|SetStartYaw (.yaw (Transformation|GetWorldRotation (Variables|Default|GetKey))))
    (Variables|Default|SetKeyLocation (Transformation|GetWorldLocation (Variables|Default|GetKey)))
    (Utilities|FlowControl|Sequence
      (:then_0
        (bind _새_트랙_0 (Timeline|타임라인_0 Play)
          (:Update
            (Transformation|SetWorldLocation (Variables|Default|GetKey) (Math|Vector|MakeVector (.x (Variables|Default|GetKeyLocation)) (.y (Variables|Default|GetKeyLocation)) (+ (.z (Variables|Default|GetKeyLocation)) (Math|Float|Lerp 0.0 2e+02 _새_트랙_0))) false false))
          (:Finished
            (Default|PlusKey (Variables|Default|GetBP%20Player))
            (Development|SetHiddeninGame (Variables|Default|GetKey) true false)
            (AddComponent|AddNiagaraComponent true (Math|Transform|MakeTransform (Transformation|GetWorldLocation (Variables|Default|GetKey)) "0, 0, 0" "3.000000,3.000000,3.000000"))
            (Utilities|FlowControl|Delay 2.0)
            (Actor|DestroyActor))))
      (:then_1
        (Utilities|FlowControl|Sequence :!label _label
          (:then_0
            (bind _새_트랙_0_2 (Timeline|타임라인_1 SetNewTime)
              (:Update
                (Transformation|SetWorldRotation (Variables|Default|GetKey) (Math|Rotator|MakeRotator 0.0 0.0 (+ (Variables|Default|GetStartYaw) (Math|Float|Lerp 0.0 3.6e+02 (/ (- _새_트랙_0_2 (- 1.0 (Variables|Default|GetKeyTurnTime))) (Variables|Default|GetKeyTurnTime))))) false false))
              (:Finished
                (if (>= (Variables|Default|GetKeyTurnTime) 0.4)
                  (Variables|Default|SetKeyTurnTime (- (Variables|Default|GetKeyTurnTime) 0.2))
                  (goto _label)
                  (else
                    (bind _새_트랙_0_3 (Timeline|타임라인_2 Play)
                      (:Update
                        (Transformation|SetWorldRotation (Variables|Default|GetKey) (Math|Rotator|MakeRotator 0.0 0.0 (+ (Variables|Default|GetStartYaw) (Math|Float|Lerp 0.0 3.6e+02 _새_트랙_0_3))) false false))
                      (:Finished
                        (if true
                          (Timeline|타임라인_2 PlayFromStart)))))))))
          (:then_1
            (Timeline|타임라인_1 Play)))))))

(fn ConstructionScript
  (|CallParentFunction))

(fn WidgetText
  (return (Utilities|Text|ToText(String) (Utilities|String|Append "[F] " "획득하기"))))