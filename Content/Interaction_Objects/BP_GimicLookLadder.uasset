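; BP_GimicLookLadder is a gimmick ladder that visually extends downward when GimicComplete fires.
; The event re-calls itself after a short Delay, each pass adding a collision-free mesh section at a fixed spacing below the last and playing the Ladder_down sound.
; Once NumberOfRungs is reached it sets IsComplete.
; The construction script only measures section height, as its rung-building loop is disconnected and the measurement goes unused at runtime.
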(event Custom|GimicComplete
  (if (> (Variables|Default|GetNumberOfRungs) (Variables|Default|GetMakingLookLadder))
    (bind _returnvalue (AddComponent|AddStaticMeshComponent false (Math|Transform|MakeTransform (Math|Vector|MakeVector 0.0 0.0 (* (* (Variables|Default|GetMakingLookLadder) 48) -1.0)) "0, 0, 0" "1.000000,1.000000,1.000000")))
    (Collision|SetCollisionEnabled _returnvalue "NoCollision")
    (Audio|PlaySoundatLocation "/Game/Sound/Plus_Sound/ladder_down.ladder_down" (Transformation|GetActorLocation) "0, 0, 0" 1.0 1.0 0.0 0 0 0 0)
    (Utilities|FlowControl|Delay 0.1)
    (Math|Integer|IncrementInt (Variables|Default|GetMakingLookLadder)
      (:%20%20
        (CallFunction|GimicComplete)))
    (else
      (Variables|Default|SetIsComplete true))))

(event EventBeginPlay)

(event EventTick
  (params (DeltaSeconds :type Float%20%28single-precision%29)))

(fn ConstructionScript
  (Utilities|FlowControl|Sequence
    (:then_0
      (Variables|Default|SetLadderSectionMeshHeight (* (.z (.boxextent (StaticMesh|GetBounds (Variables|Default|GetLadderSectionMesh)))) 2.0)))))