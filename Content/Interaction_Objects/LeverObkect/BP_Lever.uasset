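; BP_Lever is an interactable lever that toggles linked BP_Door actors, with an optional timed return.
; Interacting hides the prompt, plays a sound, switches the doors and rotates the handle between Start and End transforms via timeline.
; Unless NoTime is set, a second timeline starts offset so the return lasts ReturnTime, then re-enables interaction.
; Tick, enabled during operation, copies CustomTimeDilation changes to the doors.
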(event EventBeginPlay
  (|CallParentFunction)
  (for _array_element (Variables|Default|GetBP_Door)
    (Variables|/Game/Interaction_Objects/LeverObkect/BP_LeverDoor.BP_LeverDoor_C|SetNew%20Time _array_element (Variables|Default|GetReturnTime))))

(event EventTick
  (params (DeltaSeconds :type Float%20%28single-precision%29))
  (if (!= (Variables|Default|GetCustomTimeDilation) (Variables|Default|GetBy%20Costom%20Time))
    (for _array_element (Variables|Default|GetBP_Door)
      (Variables|/Script/Engine.Actor|SetCustomTimeDilation _array_element (Variables|Default|GetCustomTimeDilation)))
    (Variables|Default|SetBy%20Costom%20Time (Variables|Default|GetCustomTimeDilation))))

(event EventInteractive
  (if (not (Variables|Default|GetIs%20Operationing))
    (Variables|Default|SetIs%20Operationing true)
    (Development|SetHiddeninGame (Variables|Default|GetWidget) true false)
    (Actor|Tick|SetActorTickEnabled true)
    (Audio|PlaySoundatLocation "/Game/Sound/Plus_Sound/lever2.lever2" (Transformation|GetActorLocation) "0, 0, 0" 1.0 1.0 0.0 0 0 0 0)
    (for _array_element (Variables|Default|GetBP_Door)
      (Default|SwitchInteraction _array_element)
      (Variables|/Game/Interaction_Objects/LeverObkect/BP_LeverDoor.BP_LeverDoor_C|SetNoTime _array_element (Variables|Default|GetNoTime)))
    (bind _새_트랙_0 (Timeline|타임라인 PlayFromStart)
      (:Update
        (Transformation|SetWorldRotation (Variables|Default|GetSM_PROP_lever_handle_dungeon_02) (Math|Rotator|Lerp(Rotator) (Transformation|GetWorldRotation (Variables|Default|GetStart)) (Transformation|GetWorldRotation (Variables|Default|GetEnd)) _새_트랙_0) false false))
      (:Finished
        (if (not (Variables|Default|GetNoTime))
          (Utilities|FlowControl|Sequence
            (:then_0
              (bind _새_트랙_0_2 (Timeline|타임라인_0 SetNewTime)
                (:Update
                  (Transformation|SetWorldRotation (Variables|Default|GetSM_PROP_lever_handle_dungeon_02) (Math|Rotator|Lerp(Rotator) (Transformation|GetWorldRotation (Variables|Default|GetEnd)) (Transformation|GetWorldRotation (Variables|Default|GetStart)) (/ (- _새_트랙_0_2 (- 1e+02 (Variables|Default|GetReturnTime))) (Variables|Default|GetReturnTime))) false false))
                (:Finished
                  (Variables|Default|SetIs%20Operationing false)
                  (Actor|Tick|SetActorTickEnabled false)
                  (if (Variables|/Game/ThirdPerson/Blueprints/BP_ThirdPersonCharacter.BP_ThirdPersonCharacter_C|GetInteractionRanging (Variables|Default|GetBP%20Player))
                    (Development|SetHiddeninGame (Variables|Default|GetWidget) false false)))))
            (:then_1
              (Timeline|타임라인_0 Play))))))))

(fn ConstructionScript
  (|CallParentFunction))

(fn WidgetText
  (return (Utilities|Text|ToText(String) (Utilities|String|Append "[F] " "작동하기"))))