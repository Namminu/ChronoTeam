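; BP_LeverDoor1 is a trapdoor-style door that rotates between Start and End component orientations when it receives SwitchInteraction.
; A timeline lerps MoveStaticMesh from Start to End.
; Unless NoTime is set, a second timeline, seeked to 100 minus NewTime and normalized by NewTime, rotates it back, giving a configurable return duration.
; With NoTime set, it stays at End and disables the door mesh's collision.
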(event Custom|SwitchInteractionEnd)

(event Custom|SwitchInteraction
  (bind _새_트랙_0 (Timeline|타임라인 PlayFromStart)
    (:Update
      (Transformation|SetWorldRotation (Variables|Default|GetMove_StaticMesh) (Math|Rotator|Lerp(Rotator) (Transformation|GetWorldRotation (Variables|Default|GetStart)) (Transformation|GetWorldRotation (Variables|Default|GetEnd)) _새_트랙_0 true) false false))
    (:Finished
      (if (not (Variables|Default|GetNoTime))
        (Utilities|FlowControl|Sequence
          (:then_0
            (bind _새_트랙_0_2 (Timeline|타임라인_0 SetNewTime)
              (:Update
                (Transformation|SetWorldRotation (Variables|Default|GetMove_StaticMesh) (Math|Rotator|Lerp(Rotator) (Transformation|GetWorldRotation (Variables|Default|GetEnd)) (Transformation|GetWorldRotation (Variables|Default|GetStart)) (/ (- _새_트랙_0_2 (- 1e+02 (Variables|Default|GetNew%20Time))) (Variables|Default|GetNew%20Time)) true) false false))))
          (:then_1
            (Timeline|타임라인_0 Play)))
        (else
          (Collision|SetCollisionEnabled (Variables|Default|GetSM_PROP_trapdoor_door_dungeon_02) "NoCollision"))))))

(event EventBeginPlay
  (Transformation|SetWorldRotation (Variables|Default|GetMove_StaticMesh) (Transformation|GetWorldRotation (Variables|Default|GetStart)) false false))

(fn ConstructionScript)