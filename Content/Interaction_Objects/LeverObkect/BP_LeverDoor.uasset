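; BP_LeverDoor is a door that opens on a switch interaction and can close itself on a timer.
; It slides MoveStaticMesh from the Start to End component location through a timeline, with a cell door sound.
; Unless NoTime is set, a second timeline then returns it over NewTime, starting at 100 minus NewTime and rescaling the track into the lerp alpha.
; SwitchInteractionEnd is empty.
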(event Custom|SwitchInteractionEnd)

(event Custom|SwitchInteraction
  (Audio|PlaySoundatLocation "/Game/Sound/Plus_Sound/Open_Prison_Cell_Door.Open_Prison_Cell_Door" (Transformation|GetActorLocation) "0, 0, 0" 1.0 1.0 1.0 0 0 0 0)
  (bind _새_트랙_0 (Timeline|타임라인 PlayFromStart)
    (:Update
      (Transformation|SetWorldLocation (Variables|Default|GetMove_StaticMesh) (Math|Vector|Lerp(Vector) (Transformation|GetWorldLocation (Variables|Default|GetStart)) (Transformation|GetWorldLocation (Variables|Default|GetEnd)) _새_트랙_0) false false))
    (:Finished
      (if (not (Variables|Default|GetNoTime))
        (Audio|PlaySoundatLocation "/Game/Sound/Plus_Sound/Open_Prison_Cell_Door.Open_Prison_Cell_Door" (Transformation|GetActorLocation) "0, 0, 0" 1.0 1.0 1.0 0 0 0 0)
        (Utilities|FlowControl|Sequence
          (:then_0
            (bind _새_트랙_0_2 (Timeline|타임라인_0 SetNewTime)
              (:Update
                (Transformation|SetWorldLocation (Variables|Default|GetMove_StaticMesh) (Math|Vector|Lerp(Vector) (Transformation|GetWorldLocation (Variables|Default|GetEnd)) (Transformation|GetWorldLocation (Variables|Default|GetStart)) (/ (- _새_트랙_0_2 (- 1e+02 (Variables|Default|GetNew%20Time))) (Variables|Default|GetNew%20Time))) false false))))
          (:then_1
            (Timeline|타임라인_0 Play)))))))

(event EventBeginPlay
  (Transformation|SetWorldLocation (Variables|Default|GetMove_StaticMesh) (Transformation|GetWorldLocation (Variables|Default|GetStart)) false false))

(fn ConstructionScript)